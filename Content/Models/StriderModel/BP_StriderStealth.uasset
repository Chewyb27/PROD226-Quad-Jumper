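; Stealth dropship that, as a level ship, takes player possession and flies a spline to deliver the player.
; A timeline drives it along the track; near the spline point closest to SpawnLocation it spawns and possesses BP_Player, then cloaks and later destroys itself.
; Cloaking animates dynamic hull materials and a post-process distortion material that tracks the ship's location.
; Non-level ships instead toggle the cloak periodically on Tick.
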(event `Drop Sequence`
  (bind _spline (`/Game/LevelStart/BP_ShipSpline.Spline` (`self.Track Reference`)))
  (bind _returnvalue (`KismetMathLibrary.Lerp` 0.0 (`SplineComponent.GetSplineLength` _spline) (`self.Alpha`)))
  (bind _returnvalue_2 (`SplineComponent.GetLocationAtDistanceAlongSpline` _spline _returnvalue "World"))
  (`Controller.Possess` (`GameplayStatics.GetPlayerController` 0) self)
  (`TimelineComponent.SetPlayRate` (`self.ShipMovement`) (/ 1.0 (`self.StartDuration`)))
  (`TimelineComponent.SetNewTime` (`self.ShipMovement`) (`self.StartOffset`))
  (bind (_direction _alpha) (`Timeline|ShipMovement`)
    (:`Update`
      (set `self.Alpha` _alpha)
      (`self.K2_SetActorLocationAndRotation` _returnvalue_2 (`SplineComponent.GetRotationAtDistanceAlongSpline` _spline _returnvalue "World"))
      (if (<= (`KismetMathLibrary.Vector_Distance` _returnvalue_2 (`self.Closest Point`)) 1000.0)
        (`/Engine/EditorBlueprintResources/StandardMacros.DoOnce` false
          (:`Completed`
            (bind _returnvalue_3 (`|SpawnActorFromClass` "/Game/Blueprints/Player/BP_Player.BP_Player_C" (`self.GetTransform` (`self.Spawn Location`)) "Undefined" "OverrideRootScale" null self))
            (`Controller.Possess` (`GameplayStatics.GetPlayerController` 0) _returnvalue_3)
            (`KismetSystemLibrary.Delay` 1.0)
            (`self.Switch Cloaking`)
            (`KismetSystemLibrary.Delay` 10.0)
            (`self.K2_DestroyActor`)))))))

(event `self.ReceiveBeginPlay`
  (bind _main_body (`self.Main Body`))
  (bind _returnvalue (`PrimitiveComponent.CreateDynamicMaterialInstance` _main_body 0 "/Game/Materials/StealthMaterials/StealthShipBody.StealthShipBody" "None"))
  (set `self.Body Material` _returnvalue)
  (bind _returnvalue_2 (`PrimitiveComponent.CreateDynamicMaterialInstance` _main_body 1 "/Game/Materials/StealthMaterials/StealthshipEngine.StealthshipEngine" "None"))
  (set `self.Engine Material` _returnvalue_2)
  (bind _returnvalue_3 (`PrimitiveComponent.CreateDynamicMaterialInstance` _main_body 2 "/Game/Materials/StealthMaterials/StealthshipWindowInst.StealthshipWindowInst" "None"))
  (set `self.Window Material` _returnvalue_3)
  (bind _returnvalue_4 (`KismetMaterialLibrary.CreateDynamicMaterialInstance` "/Game/Materials/StealthMaterials/M_Distortion.M_Distortion"))
  (bind _output_get (set `self.Post Process Material` _returnvalue_4))
  (bind _outactors (`GameplayStatics.GetAllActorsOfClass` "/Script/Engine.PostProcessVolume"))
  (`KismetArrayLibrary.Array_Add` (`.Array` (break `WeightedBlendables` (`.WeightedBlendables` (break `PostProcessSettings` (`PostProcessVolume.Settings` (`KismetArrayLibrary.Array_Random` _outactors)))))) (make `WeightedBlendable` 1.0 _output_get))
  (if (`self.LevelShip`)
    (bind _closestpoint (`self.Closest Point in Spline` (`SceneComponent.K2_GetComponentLocation` (`Actor.RootComponent` (`self.Spawn Location`))) (`/Game/LevelStart/BP_ShipSpline.Spline` (`self.Track Reference`))))
    (set `self.Closest Point` _closestpoint)
    (`self.Drop Sequence`)))

(event `Switch Cloaking`
  (`/Engine/EditorBlueprintResources/StandardMacros.FlipFlop` :!label _label
    (:`A`
      (bind (_direction _cloaking_amount _distortion) (`Timeline|Timeline_0` :!label _label_2)
        (:`Update`
          (`MaterialInstanceDynamic.SetScalarParameterValue` (`self.Body Material`) "Amount" _cloaking_amount)
          (`MaterialInstanceDynamic.SetScalarParameterValue` (`self.Engine Material`) "Amount" _cloaking_amount)
          (`MaterialInstanceDynamic.SetScalarParameterValue` (`self.Window Material`) "Amount" _cloaking_amount)
          (`MaterialInstanceDynamic.SetScalarParameterValue` (`self.Post Process Material`) "Amount" _distortion))))
    (:`B`
      (goto _label_2 :!via `ReverseFromEnd`))))

(event `self.ReceiveTick`
  (params (DeltaSeconds :type "Float (single-precision)"))
  (bind _cloak_delay (`self.Cloak Delay`))
  (`MaterialInstanceDynamic.SetVectorParameterValue` (`self.Post Process Material`) "Location" (`KismetMathLibrary.Conv_VectorToLinearColor` (`self.K2_GetActorLocation`)))
  (if (not (`self.LevelShip`))
    (if (>= _cloak_delay 10.0)
      (set `self.Cloak Delay` 0.0)
      (goto _label)
      (else
        (set `self.Cloak Delay` (+ _cloak_delay DeltaSeconds))))))

(fn `Closest Point in Spline`
  (params (`Location To Check` :type "Vector Structure") (Spline :type "SplineComponent Object Reference"))
  (returns (ClosestPoint :type "Vector Structure") (`Spline Point` :type Integer))
  (bind _returnvalue (`SplineComponent.FindInputKeyClosestToWorldLocation` Spline `Location To Check`))
  (bind _returnvalue_2 (`KismetMathLibrary.FFloor` _returnvalue))
  (bind _returnvalue_3 (+ _returnvalue_2 1))
  (bind _returnvalue_4 (`SplineComponent.GetDistanceAlongSplineAtSplinePoint` Spline _returnvalue_3))
  (return (`SplineComponent.GetLocationAtDistanceAlongSpline` Spline (- _returnvalue_4 (* (- (`SplineComponent.GetDistanceAlongSplineAtSplinePoint` Spline _returnvalue_2) _returnvalue_4) (- _returnvalue (`KismetMathLibrary.Conv_IntToDouble` _returnvalue_3)))) "World") _returnvalue_2))

(fn `UserConstructionScript`)
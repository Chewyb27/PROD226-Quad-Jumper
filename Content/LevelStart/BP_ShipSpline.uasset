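; BP_ShipSpline is a spline helper Blueprint whose one working function, ClosestPointInSpline, finds the point on a given spline nearest a world location.
; It takes the closest input key, linearly interpolates distance between the two surrounding spline points, and returns that world-space position plus the floored point index.
; The event graph and construction script hold no logic.
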(fn `Closest Point in Spline`
  (params (`Location To Check` :type "Vector Structure") (Spline :type "SplineComponent Object Reference"))
  (returns (ClosestPoint :type "Vector Structure") (`Spline Point` :type Integer))
  (bind _returnvalue (`SplineComponent.FindInputKeyClosestToWorldLocation` Spline `Location To Check`))
  (bind _returnvalue_2 (`KismetMathLibrary.FFloor` _returnvalue))
  (bind _returnvalue_3 (+ _returnvalue_2 1))
  (bind _returnvalue_4 (`SplineComponent.GetDistanceAlongSplineAtSplinePoint` Spline _returnvalue_3))
  (return (`SplineComponent.GetLocationAtDistanceAlongSpline` Spline (- _returnvalue_4 (* (- (`SplineComponent.GetDistanceAlongSplineAtSplinePoint` Spline _returnvalue_2) _returnvalue_4) (- _returnvalue (`KismetMathLibrary.Conv_IntToDouble` _returnvalue_3)))) "World") _returnvalue_2))

(fn `UserConstructionScript`)
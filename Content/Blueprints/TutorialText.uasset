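; TutorialText is a trigger actor that shows a tutorial message on the player's HUD while BP_Player overlaps it.
; On overlap it copies its title and three combined text lines into the player's tutorial variables.
; The FadeOut timeline then drives the TutorialOverlay's render opacity, playing forward on entry and reversing on exit.
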(event `self.ReceiveActorBeginOverlap`
  (params (OtherActor :type "Actor Object Reference"))
  (if (== (`GameplayStatics.GetObjectClass` OtherActor) "/Game/Blueprints/Player/BP_Player.BP_Player_C")
    (bind _asbp_player (cast `/Game/Blueprints/Player/BP_Player` OtherActor))
    (set `/Game/Blueprints/Player/BP_Player.Tutorial Text` (`self.Title`) _asbp_player)
    (set `/Game/Blueprints/Player/BP_Player.Tutorial info` (`KismetTextLibrary.Conv_StringToText` (`KismetStringLibrary.Concat_StrStr` (`self.Text_Line_1`) " \n" (`self.Text_Line_2`) " \n" (`self.Text_Line_3`))) _asbp_player)
    (set `self.Player reference` _asbp_player)
    (bind (_direction _opacity) (`Timeline|Fade Out` :!via `PlayFromStart` :!label _label)
      (:`Update`
        (set `Widget.RenderOpacity` _opacity (`/Game/Widgets/WBP_PlayerHUD.TutorialOverlay` (`/Game/Blueprints/Player/BP_Player.HUD` (`self.Player reference`))))))))

(event `self.ReceiveActorEndOverlap`
  (params (OtherActor :type "Actor Object Reference"))
  (if (== (`GameplayStatics.GetObjectClass` OtherActor) "/Game/Blueprints/Player/BP_Player.BP_Player_C")
    (bind _asbp_player (cast `/Game/Blueprints/Player/BP_Player` OtherActor))
    (set `self.Player reference` _asbp_player)
    (goto _label :!via `ReverseFromEnd`)))

(fn `UserConstructionScript`)
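; VehiclePatrolRoute is a scene actor that holds a spline, evidently marking a patrol path for vehicles.
; The Construction Script parses the number after "VehiclePatrolRoute" in the actor's display name and uses it to select the unselected segment color, so numbered routes are distinguishable in the editor.
; It has no runtime logic, and its FlyingRoute variable is unused here.
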(fn `UserConstructionScript`
  (`SplineComponent.SetUnselectedSplineSegmentColor` (`self.Spline`) (select `int` (`KismetStringLibrary.Conv_StringToInt` (`.RightS` (`KismetStringLibrary.Split` (`KismetSystemLibrary.GetDisplayName` self) "VehiclePatrolRoute"))) :`0` (`KismetMathLibrary.MakeColor` 1.0) :`1` (struct) :`2` (`KismetMathLibrary.MakeColor` 1.0 1.0) :`3` (`KismetMathLibrary.MakeColor` 0.0 1.0) :`4` (`KismetMathLibrary.MakeColor` 0.0 1.0 1.0) :`5` (`KismetMathLibrary.MakeColor` 0.0 0.0 1.0) :`6` (`KismetMathLibrary.MakeColor` 1.0 0.0 1.0))))
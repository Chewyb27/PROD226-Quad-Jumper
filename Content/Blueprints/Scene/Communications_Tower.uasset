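; Communications Tower scene actor that can switch from a standing state to a weakened, physics-driven one.
; On BeginPlay the static mesh carries collision and the capsule has none.
; WeakenedState, not called by any live path here, swaps collision to the capsule, enables its physics simulation with heavy linear and angular damping, and flags Weakened.
; It also sets mesh and capsule to block the Visibility channel.
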(event `self.ReceiveBeginPlay`
  (`PrimitiveComponent.SetCollisionEnabled` (`self.Capsule`) "NoCollision")
  (`PrimitiveComponent.SetCollisionEnabled` (`self.StaticMesh`) "QueryAndPhysics"))

(event `Weakened State`
  (bind _capsule (`self.Capsule`))
  (bind _staticmesh (`self.StaticMesh`))
  (`PrimitiveComponent.SetCollisionEnabled` _capsule "QueryAndPhysics")
  (`PrimitiveComponent.SetCollisionEnabled` _staticmesh "NoCollision")
  (`PrimitiveComponent.SetSimulatePhysics` _capsule true)
  (set `self.Weakened` true)
  (`PrimitiveComponent.SetCollisionResponseToChannel` _staticmesh "ECC_Visibility" "ECR_Block")
  (`PrimitiveComponent.SetCollisionResponseToChannel` _capsule "ECC_Visibility" "ECR_Block")
  (`PrimitiveComponent.SetLinearDamping` _capsule 100.0)
  (`PrimitiveComponent.SetAngularDamping` _capsule 100.0))

(fn `UserConstructionScript`)
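; BP_Shield_Tower is a destructible tower that projects a charge beam and hit point onto the surface of its linked Shield.
; Tick weakens it once its guards are dead or, without guards, its support structure is dead or missing.
; SettoDynamic then lets a weakened tower simulate physics with a lowered center of mass.
; Up-vector tilt checks black out materials and cut the beam, then freeze the mesh once fallen flat.
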(event `self.ReceiveBeginPlay`
  (bind _shield (`/Game/Blueprints/Enemies/BP_Charged_Shield.Shield` (`self.Shield`)))
  (bind _returnvalue (`SceneComponent.K2_GetComponentLocation` _shield))
  (bind _x (`KismetMathLibrary.BreakVector3f` (`SceneComponent.RelativeScale3D` _shield)))
  (bind _returnvalue_2 (`KismetMathLibrary.Normal` (- (`SceneComponent.K2_GetComponentLocation` (`self.Charge Beam`)) _returnvalue)))
  (`FXSystemComponent.SetVectorParameter` (`self.Charge Beam`) "Beam End" (+ _returnvalue (* _returnvalue_2 50.0 _x)))
  (`SceneComponent.K2_SetWorldLocation` (`self.Hit Point`) (+ (* _returnvalue_2 48.0 _x) _returnvalue) false false))

(event `Set to Dynamic`
  (bind _staticmesh (`self.StaticMesh`))
  (if (`self.Weakened`)
    (if (not (`self.is Dynamic`))
      (`PrimitiveComponent.SetCenterOfMass` _staticmesh (0.0 0.0 -700.0) "None")
      (set `self.is Dynamic` true)
      (`PrimitiveComponent.SetCollisionObjectType` _staticmesh "ECC_WorldDynamic")
      (`PrimitiveComponent.SetSimulatePhysics` _staticmesh true)
      (`PrimitiveComponent.SetSimulatePhysics` (`self.StaticMesh`) true)
      (`PrimitiveComponent.SetLinearDamping` _staticmesh 1000.0)
      (`PrimitiveComponent.SetAngularDamping` _staticmesh 0.5))))

(event `Weakened State`
  (set `self.Weakened` true)
  (set `self.Fallen` false))

(event `self.ReceiveTick`
  (params (DeltaSeconds :type "Float (single-precision)"))
  (bind _guards (`self.Guards`))
  (bind _staticmesh (`self.StaticMesh`))
  (bind _childactor (`ChildActorComponent.ChildActor` (`self.Support`)))
  (bind _returnvalue (`KismetMathLibrary.Dot_VectorVector` (`KismetMathLibrary.Vector_Up`) (`SceneComponent.GetUpVector` (`self.StaticMesh`))))
  (if (`self.use guards`)
    (set `self.Valid Guards` false)
    (for _array_element _guards
      (if (`/Game/Blueprints/Enemies/Enemy.EnemyAlive` _array_element)
        (set `self.Valid Guards` true)))
    (if (`KismetArrayLibrary.Array_IsEmpty` _guards)
      (`|ExecutionSequence` :!label _label
        (:`then_0`
          (`/Engine/EditorBlueprintResources/StandardMacros.DoOnce` false
            (:`Completed`
              (`self.Weakened State`))))
        (:`then_1`
          (if (<= _returnvalue 0.9)
            (`/Engine/EditorBlueprintResources/StandardMacros.DoOnce` false
              (:`Completed`
                (`PrimitiveComponent.SetMaterial` (`self.StaticMesh`) 2 "/Game/Materials/GeneralMaterials/M_Black_Padding.M_Black_Padding")
                (`PrimitiveComponent.SetMaterial` (`self.radar`) 0 "/Game/Materials/GeneralMaterials/M_Black_Padding.M_Black_Padding")
                (`PrimitiveComponent.SetMaterial` (`self.radar2`) 0 "/Game/Materials/GeneralMaterials/M_Black_Padding.M_Black_Padding")
                (`PrimitiveComponent.SetMaterial` (`self.radar1`) 0 "/Game/Materials/GeneralMaterials/M_Black_Padding.M_Black_Padding")
                (set `self.Disabled` true)
                (`SceneComponent.SetVisibility` (`self.Charge Beam`) false false)
                (`ActorComponent.K2_DestroyComponent` (`self.Hit Point`))))))
        (:`then_2`
          (if (<= _returnvalue 0.03)
            (`PrimitiveComponent.SetCollisionObjectType` _staticmesh "ECC_WorldStatic")
            (`PrimitiveComponent.SetSimulatePhysics` _staticmesh false)
            (set `self.Fallen` true))))
      (elif (not (`self.Valid Guards`))
        (goto _label)))
    (else
      (`/Engine/EditorBlueprintResources/StandardMacros.IsValid` _childactor
        (:`Is Valid`
          (bind _asbp_support_structure (cast `/Game/Blueprints/Enemies/BP_Support_Structure` _childactor))
          (if (not (`/Game/Blueprints/Enemies/Enemy.EnemyAlive` _asbp_support_structure))
            (goto _label)))
        (:`Is Not Valid`
          (goto _label))))))

(fn `UserConstructionScript`
  (bind _charge_beam (`self.Charge Beam`))
  (`FXSystemComponent.SetVectorParameter` _charge_beam "Beam End" (`SceneComponent.K2_GetComponentLocation` _charge_beam)))
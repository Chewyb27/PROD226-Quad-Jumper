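; G_Zone is a gravity zone actor that pulls physics objects along its own down axis.
; Cube overlap events register a gravity vector in BP_Player's GravityDirection map, keyed by zone, and toggle world gravity off for other simulating components until they exit.
; Tick applies delta-scaled, mass-independent impulses to overlapping simulating components, skipping players and the zone's parent component.
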(event `self.ReceiveBeginPlay`)

(event `self.ReceiveTick`
  (params (DeltaSeconds :type "Float (single-precision)"))
  (for _array_element (`self.GetOverlappingComponents`)
    (if (and (`SceneComponent.IsSimulatingPhysics` _array_element "None") (not (`KismetMathLibrary.ClassIsChildOf` (`GameplayStatics.GetObjectClass` (`ActorComponent.GetOwner` _array_element)) "/Game/Blueprints/Player/BP_Player.BP_Player_C")) (not (== (`self.GetParentComponent`) _array_element)))
      (`PrimitiveComponent.AddImpulse` _array_element (* (`self.GetActorUpVector`) -9.81 DeltaSeconds 200.0) "None" true))))

(event `self.Cube.OnComponentBeginOverlap`
  (params (OverlappedComponent :type "PrimitiveComponent Object Reference") (OtherActor :type "Actor Object Reference") (OtherComp :type "PrimitiveComponent Object Reference") (OtherBodyIndex :type Integer) (bFromSweep :type Boolean) (SweepResult :type "HitResult Structure (by ref)"))
  (`/Engine/EditorBlueprintResources/StandardMacros.IsValid` OtherComp
    (:`Is Valid`
      (if (`SceneComponent.IsSimulatingPhysics` OtherComp "None")
        (if (`KismetMathLibrary.ClassIsChildOf` (`GameplayStatics.GetObjectClass` OtherActor) "/Game/Blueprints/Player/BP_Player.BP_Player_C")
          (bind _asbp_player (cast `/Game/Blueprints/Player/BP_Player` OtherActor))
          (`BlueprintMapLibrary.Map_Add` (`/Game/Blueprints/Player/BP_Player.Gravity Direction` _asbp_player) self (* (`self.GetActorUpVector`) -9.81))
          (else
            (`PrimitiveComponent.SetEnableGravity` OtherComp false)))))))

(event `self.Cube.OnComponentEndOverlap`
  (params (OverlappedComponent :type "PrimitiveComponent Object Reference") (OtherActor :type "Actor Object Reference") (OtherComp :type "PrimitiveComponent Object Reference") (OtherBodyIndex :type Integer))
  (`/Engine/EditorBlueprintResources/StandardMacros.IsValid` OtherComp
    (:`Is Valid`
      (if (`SceneComponent.IsSimulatingPhysics` OtherComp "None")
        (if (`KismetMathLibrary.ClassIsChildOf` (`GameplayStatics.GetObjectClass` OtherActor) "/Game/Blueprints/Player/BP_Player.BP_Player_C")
          (bind _asbp_player (cast `/Game/Blueprints/Player/BP_Player` OtherActor))
          (`BlueprintMapLibrary.Map_Remove` (`/Game/Blueprints/Player/BP_Player.Gravity Direction` _asbp_player) self)
          (else
            (`PrimitiveComponent.SetEnableGravity` OtherComp true)))))))

(fn `UserConstructionScript`)
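; Comms tower that becomes weakened once all its assigned guards are dead (or none are assigned) and can then be toppled.
; SettoDynamic, once weakened, enables physics with a lowered center of mass and very high linear damping.
; Tick polls the guards, then uses the up-vector dot product to black out a material slot as it tilts and freeze it as static, flagged Fallen, when nearly horizontal.
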(event `Set to Dynamic`
  (bind _staticmesh (`self.StaticMesh`))
  (if (`self.Weakened`)
    (if (not (`self.is Dynamic`))
      (`PrimitiveComponent.SetCenterOfMass` _staticmesh (0.0 0.0 -900.0) "None")
      (set `self.is Dynamic` true)
      (`PrimitiveComponent.SetCollisionObjectType` _staticmesh "ECC_WorldDynamic")
      (`PrimitiveComponent.SetSimulatePhysics` _staticmesh true)
      (`PrimitiveComponent.SetSimulatePhysics` (`self.StaticMesh`) true)
      (`PrimitiveComponent.SetLinearDamping` _staticmesh 1000.0)
      (`PrimitiveComponent.SetAngularDamping` _staticmesh 0.5))))

(event `self.ReceiveBeginPlay`)

(event `Weakened State`
  (set `self.Weakened` true)
  (set `self.Fallen` false))

(event `self.ReceiveTick`
  (params (DeltaSeconds :type "Float (single-precision)"))
  (bind _guards (`self.Guards`))
  (bind _staticmesh (`self.StaticMesh`))
  (bind _returnvalue (`KismetMathLibrary.Dot_VectorVector` (`KismetMathLibrary.Vector_Up`) (`SceneComponent.GetUpVector` (`self.StaticMesh`))))
  (set `self.Valid Guards` false)
  (for _array_element _guards
    (if (`/Game/Blueprints/Enemies/Enemy.EnemyAlive` _array_element)
      (set `self.Valid Guards` true)))
  (if (`KismetArrayLibrary.Array_IsEmpty` _guards)
    (`|ExecutionSequence` :!label _label
      (:`then_0`
        (`/Engine/EditorBlueprintResources/StandardMacros.DoOnce` false
          (:`Completed`
            (`self.Weakened State`))))
      (:`then_1`
        (if (<= _returnvalue 0.9)
          (`/Engine/EditorBlueprintResources/StandardMacros.DoOnce` false
            (:`Completed`
              (`PrimitiveComponent.SetMaterial` (`self.StaticMesh`) 2 "/Game/Materials/GeneralMaterials/M_Black_Padding.M_Black_Padding")))))
      (:`then_2`
        (if (<= _returnvalue 0.3)
          (`PrimitiveComponent.SetCollisionObjectType` _staticmesh "ECC_WorldStatic")
          (`PrimitiveComponent.SetSimulatePhysics` _staticmesh false)
          (set `self.Fallen` true))))
    (elif (not (`self.Valid Guards`))
      (goto _label))))

(fn `UserConstructionScript`)
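; BP_Australis is a friendly ship with laser turrets, a health display and a Niagara thrust plume sized at construction.
; A Hover timeline with randomized rate and start drifts it around its spawn point, while InitializeAustralis registers it on the player's HUD.
; At zero health it disables its turrets, cuts thrust and retreats toward the Australis_Waypoint on the MoveAway timeline, then destroys itself or, if last of its class, triggers game over.
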(event `Visible`
  (params (NewParam :type Boolean))
  (`SceneComponent.SetVisibility` (`self.Enemy Class Display`) NewParam false))

(event `self.ReceiveBeginPlay`
  (bind _returnvalue (`GameplayStatics.GetActorOfClass` "/Game/Blueprints/Scene/Australis_Waypoint.Australis_Waypoint_C"))
  (set `self.Waypoint` _returnvalue)
  (bind _aswbp_friendly_display (cast `/Game/Widgets/WBP_FriendlyDisplay` (`WidgetComponent.GetWidget` (`self.Enemy Class Display`))))
  (set `/Game/Widgets/WBP_FriendlyDisplay.Friendly_Name` (`KismetTextLibrary.Conv_StringToText` (`self.Name`)) _aswbp_friendly_display)
  (bind _output_get (set `/Game/Widgets/WBP_FriendlyDisplay.DisplayHealth` (`self.Health`) _aswbp_friendly_display))
  (set `/Game/Widgets/WBP_FriendlyDisplay.MaxHealth` _output_get _aswbp_friendly_display)
  (set `self.Display` _aswbp_friendly_display)
  (set `self.Starting Coordinate` (`self.K2_GetActorLocation`))
  (`TimelineComponent.SetPlayRate` (`self.Hover`) (`KismetMathLibrary.RandomFloatInRange` 0.2 0.6))
  (`|ExecutionSequence`
    (:`then_0`
      (bind (_direction _hover) (`Timeline|Hover` :`NewTime` (`KismetMathLibrary.RandomFloatInRange` 0.0 3.5) :!via `SetNewTime` :!label _label)
        (:`Update`
          (bind _returnvalue_2 (`KismetMathLibrary.Lerp` -300.0 300.0 _hover))
          (`self.K2_SetActorLocation` (`KismetMathLibrary.MakeVector` (+ (.x (`self.Starting Coordinate`)) _returnvalue_2) (+ (.y (`self.Starting Coordinate`)) _returnvalue_2) (+ (`KismetMathLibrary.Lerp` -1000.0 1000.0 _hover) (.z (`self.Starting Coordinate`))))))))
    (:`then_1`
      (goto _label))))

(event `Initialize Australis`
  (bind _returnvalue (`GameplayStatics.GetActorOfClass` "/Game/Blueprints/Player/BP_Player.BP_Player_C"))
  (set `self.Player` _returnvalue)
  (`/Game/Widgets/WBP_PlayerHUD.Add Enemy` (`/Game/Blueprints/Player/BP_Player.HUD` (`self.Player`)) self false))

(event `Damage`
  (params (`Health Change` :type "Float (double-precision)"))
  (bind _returnvalue (`self.K2_GetActorLocation`))
  (bind _player (`self.Player`))
  (bind _health (`self.Health`))
  (bind _returnvalue_2 (`self.K2_GetActorLocation` (`self.Waypoint`)))
  (bind _output_get (set `self.Health` (`KismetMathLibrary.FClamp` (- _health `Health Change`) 0.0 999999999999.0)))
  (set `/Game/Widgets/WBP_FriendlyDisplay.DisplayHealth` _output_get (`self.Display`))
  (if (<= _health 0.0)
    (`/Engine/EditorBlueprintResources/StandardMacros.DoOnce` false
      (:`Completed`
        (for _array_element (`|MakeArray` (`self.laser`) (`self.laser1`) (`self.laser2`))
          (bind _asbp_friendly_laser_turret (cast `/Game/Blueprints/Enemies/Faction_2/BP_FriendlyLaserTurret` (`ChildActorComponent.ChildActor` _array_element)))
          (set `/Game/Blueprints/Enemies/Faction_2/BP_FriendlyLaserTurret.Not Destroyed` false _asbp_friendly_laser_turret))
        (`TimelineComponent.SetPlayRate` (`self.Move Away`) 0.25)
        (bind (_direction _alpha _newtrack_1) (`Timeline|Move Away`)
          (:`Update`
            (`self.K2_SetActorLocation` (* (`KismetMathLibrary.VLerp` _returnvalue _returnvalue_2 (/ _newtrack_1 5.0)) (1.0 1.0 1.0)) false true)
            (`self.K2_SetActorRotation` (`KismetMathLibrary.RLerp` (`self.K2_GetActorRotation`) (`KismetMathLibrary.MakeRotator` (.roll (`KismetMathLibrary.FindLookAtRotation` _returnvalue_2 _returnvalue)) (* (.pitch (`KismetMathLibrary.FindLookAtRotation` _returnvalue_2 _returnvalue)) -1.5) (.yaw (`KismetMathLibrary.FindLookAtRotation` _returnvalue_2 _returnvalue))) _alpha))
            (`NiagaraComponent.SetVariableVec3` (`self.Thrust Plume`) "Beam End" (0.0 0.0 0.0)))
          (:`Finished`
            (bind _outactors (`GameplayStatics.GetAllActorsOfClass` "BP_Australis_C"))
            (if (> (`KismetArrayLibrary.Array_Length` _outactors) 1)
              (`self.K2_DestroyActor`)
              (else
                (set `/Game/Blueprints/Player/BP_Player.WinOrLose` false _player)
                (`/Game/Blueprints/Player/BP_Player.Game Over` _player)))))))))

(fn `UserConstructionScript`
  (bind _thrust_plume (`self.Thrust Plume`))
  (`NiagaraComponent.SetVariableVec3` _thrust_plume "Beam End" (`KismetMathLibrary.MakeVector` 0.0 0.0 (`self.Thrust Length`)))
  (`NiagaraComponent.SetVariableFloat` _thrust_plume "Scale Curve_Beam Width" (`self.Beam Width`)))
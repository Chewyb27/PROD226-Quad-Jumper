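; InWorldWidget is an actor that shows an information panel in the world with a title and body text.
; Its widget component hosts an InWorldInfo widget, whose TitleBlock and TextBlock are filled from the actor's Title and Text variables.
; The same assignment runs in both the construction script and BeginPlay, so the text is applied at construction and again when play starts.
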(event `self.ReceiveBeginPlay`
  (bind _asin_world_info (cast `/Game/Widgets/InWorldInfo` (`WidgetComponent.GetWidget` (`self.Widget`))))
  (`TextBlock.SetText` (`/Game/Widgets/InWorldInfo.TitleBlock` _asin_world_info) (`self.Title`))
  (`TextBlock.SetText` (`/Game/Widgets/InWorldInfo.TextBlock` _asin_world_info) (`self.Text`)))

(fn `UserConstructionScript`
  (bind _asin_world_info (cast `/Game/Widgets/InWorldInfo` (`WidgetComponent.GetWidget` (`self.Widget`))))
  (`TextBlock.SetText` (`/Game/Widgets/InWorldInfo.TitleBlock` _asin_world_info) (`self.Title`))
  (`TextBlock.SetText` (`/Game/Widgets/InWorldInfo.TextBlock` _asin_world_info) (`self.Text`)))
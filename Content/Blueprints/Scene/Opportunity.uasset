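; Opportunity vehicle actor with seven thruster effects, built to fly along a VehiclePatrolRoute spline.
; InitializeOpportunity stores the player and finds the route.
; A disconnected chain checks MissionTimer against StartTime, then uses a timeline to sweep the actor along the spline, adopting spline rotation after 10% and scaling thruster beams.
; Tick and BeginPlay are empty, so neither this launch nor the separate beam-zeroing loop runs.
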(event `self.ReceiveBeginPlay`)

(event `Initialize Opportunity`
  (params (Player :type "/Game/Blueprints/Player/BP_Player Object Reference"))
  (set `self.Player` Player)
  (bind _returnvalue (`GameplayStatics.GetActorOfClass` "/Game/Blueprints/Scene/VehiclePatrolRoute.VehiclePatrolRoute_C"))
  (set `self.Spline` _returnvalue))

(event `self.ReceiveTick`
  (params (DeltaSeconds :type "Float (single-precision)")))

(fn `UserConstructionScript`)
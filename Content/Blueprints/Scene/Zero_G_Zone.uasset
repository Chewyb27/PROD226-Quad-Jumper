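; Zero-gravity volume that removes gravity from physics-simulating components inside its Cube trigger.
; On BeginPlay it disables gravity on simulating components already overlapping it, then toggles gravity as others enter and leave.
; BP_Player is handled separately: the zone registers itself in the player's GravityDirection map on entry and removes itself on exit, provided the overlapping component simulates physics.
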(event `self.ReceiveBeginPlay`
  (for _array_element (`self.GetOverlappingComponents`)
    (if (`SceneComponent.IsSimulatingPhysics` _array_element "None")
      (`PrimitiveComponent.SetEnableGravity` _array_element false))))

(event `self.Cube.OnComponentBeginOverlap`
  (params (OverlappedComponent :type "PrimitiveComponent Object Reference") (OtherActor :type "Actor Object Reference") (OtherComp :type "PrimitiveComponent Object Reference") (OtherBodyIndex :type Integer) (bFromSweep :type Boolean) (SweepResult :type "HitResult Structure (by ref)"))
  (`/Engine/EditorBlueprintResources/StandardMacros.IsValid` OtherComp
    (:`Is Valid`
      (if (`SceneComponent.IsSimulatingPhysics` OtherComp "None")
        (if (`KismetMathLibrary.ClassIsChildOf` (`GameplayStatics.GetObjectClass` OtherActor) "/Game/Blueprints/Player/BP_Player.BP_Player_C")
          (bind _asbp_player (cast `/Game/Blueprints/Player/BP_Player` OtherActor))
          (`BlueprintMapLibrary.Map_Add` (`/Game/Blueprints/Player/BP_Player.Gravity Direction` _asbp_player) self)
          (else
            (`PrimitiveComponent.SetEnableGravity` OtherComp false)))))))

(event `self.Cube.OnComponentEndOverlap`
  (params (OverlappedComponent :type "PrimitiveComponent Object Reference") (OtherActor :type "Actor Object Reference") (OtherComp :type "PrimitiveComponent Object Reference") (OtherBodyIndex :type Integer))
  (if (`SceneComponent.IsSimulatingPhysics` OtherComp "None")
    (if (`KismetMathLibrary.ClassIsChildOf` (`GameplayStatics.GetObjectClass` OtherActor) "/Game/Blueprints/Player/BP_Player.BP_Player_C")
      (bind _asbp_player (cast `/Game/Blueprints/Player/BP_Player` OtherActor))
      (`BlueprintMapLibrary.Map_Remove` (`/Game/Blueprints/Player/BP_Player.Gravity Direction` _asbp_player) self)
      (else
        (`PrimitiveComponent.SetEnableGravity` OtherComp true)))))

(fn `UserConstructionScript`)
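; BP_Arrows is a scene actor that animates four arrows as a looping chase light.
; On BeginPlay the Animate timeline starts and replays itself whenever it finishes.
; Each Lights event resets all arrows to ArrowBase, then advances a wrapping index and applies ArrowBright to that arrow.
; The construction script calls Glow, which is an empty event.
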(event `Glow`)

(event `self.ReceiveBeginPlay`
  (bind _array (`|MakeArray` (`self.Arrow 1`) (`self.Arrow 2`) (`self.Arrow 3`) (`self.Arrow 4`)))
  (bind _returnvalue (+ (`self.Index`) 1))
  (`Timeline|Animate` :!via `PlayFromStart` :!label _label
    (:`Finished`
      (if true
        (goto _label :!via `PlayFromStart`)))
    (:`Lights`
      (for _array_element _array
        (`PrimitiveComponent.SetMaterial` _array_element 0 "/Game/Materials/Scene/ArrowBase.ArrowBase"))
      (set `self.Index` (`KismetMathLibrary.SelectInt` 0 _returnvalue (>= _returnvalue (- (`KismetArrayLibrary.Array_Length` _array) 0))))
      (`PrimitiveComponent.SetMaterial` (`|GetArrayItem` _array (`self.Index`)) 0 "/Game/Materials/Scene/ArrowBright.ArrowBright"))))

(fn `UserConstructionScript`
  (`self.Glow`))
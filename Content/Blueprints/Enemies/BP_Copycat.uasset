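; BP_Copycat is an enemy that trails a set number of points behind the end of a spline, carrying three child turrets that receive its player reference.
; A periodic box trace switches it between walking with animated legs along the spline's heading and flying with gimballed rotors while facing the player.
; It shows an aiming laser on clear line of sight.
; On death it updates HUD and win state, explodes twice and destroys itself.
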(event `Ground Check`
  (bind _groundcheck (`self.GroundCheck`))
  (bind _cube (`self.Cube`))
  (bind _returnvalue (`SceneComponent.K2_GetComponentLocation` _cube))
  (if (> _groundcheck 0.2)
    (set `self.GroundCheck` 0.0)
    (bind (_outhit _returnvalue_2) (`KismetSystemLibrary.BoxTraceSingle` _returnvalue (+ (* (`SceneComponent.GetUpVector` _cube) -200.0) _returnvalue) (450.0 550.0 150.0) (`self.K2_GetActorRotation`) "TraceTypeQuery1"))
    (bind _output_get (set `self.OnGround` _returnvalue_2))
    (set `self.Grounded_0` _returnvalue_2)
    (else
      (set `self.GroundCheck` (+ (`self.Delta Seconds`) _groundcheck))))
  (if _output_get
    _))

(event `Gimbal Thrust`
  (params (Delta :type "Float (double-precision)") (MoveAmount :type "Float (double-precision)"))
  (bind _returnvalue (* 0.0 1.0))
  (bind _roll (.roll (`SceneComponent.RelativeRotation` (`self.Main Body`))))
  (bind _pitch (.pitch (`SceneComponent.RelativeRotation` (`self.Main Body`))))
  (bind _returnvalue_2 (* _pitch -0.25))
  (`SceneComponent.K2_SetRelativeRotation` (`self.Rotor 1`) (`KismetMathLibrary.MakeRotator` _returnvalue (+ (`KismetMathLibrary.Lerp` (`KismetMathLibrary.ClampAngle` (+ (* _roll 3.0) 70.0 _returnvalue_2 0.0) -20.0 120.0) _pitch 0.025) 90.0)) false false)
  (`SceneComponent.K2_SetRelativeRotation` (`self.Rotor 2`) (`KismetMathLibrary.MakeRotator` _returnvalue (+ (`KismetMathLibrary.Lerp` (`KismetMathLibrary.ClampAngle` (+ (* _roll -3.0) 70.0 _returnvalue_2 0.0) -20.0 120.0) _pitch 0.01) 90.0)) false false))

(event `Aim laser`
  (bind _laser (`self.Laser`))
  (bind _playerreference (`self.PlayerReference`))
  (bind _returnvalue (`SceneComponent.K2_GetComponentLocation` (`self.Sphere`)))
  (bind _returnvalue_2 (`SceneComponent.K2_GetComponentLocation` (`/Game/Blueprints/Player/BP_Player.Main Body` _playerreference)))
  (`/Engine/EditorBlueprintResources/StandardMacros.IsValid` _playerreference
    (:`Is Valid`
      (bind (_outhit _returnvalue_3) (`KismetSystemLibrary.LineTraceSingle` _returnvalue _returnvalue_2 "TraceTypeQuery1" false (`|MakeArray` self _playerreference :!type "Actor Object Reference")))
      (`SceneComponent.SetVisibility` _laser (and (not _returnvalue_3) (< (`KismetMathLibrary.Dot_VectorVector` (`SceneComponent.GetUpVector` (`self.Sphere`)) (- _returnvalue_2 _returnvalue)) 0.0)) false)
      (`FXSystemComponent.SetVectorParameter` _laser "Beam End" _returnvalue_2))))

(event `self.ReceiveBeginPlay`
  (bind _sub_enemies (`self.Sub Enemies`))
  (set `self.Enemy Body` (`self.Main Body`))
  (`KismetArrayLibrary.Array_Add` _sub_enemies (`self.BP_Interior_Turret1`))
  (`KismetArrayLibrary.Array_Add` _sub_enemies (`self.BP_Interior_Missile_Turret`))
  (`KismetArrayLibrary.Array_Add` _sub_enemies (`self.BP_Interior_Turret`)))

(event `Follow Sequence`
  (bind _followspeed (`self.FollowSpeed`))
  (`TimelineComponent.SetPlayRate` _followspeed (/ 1.0 (`self.StartDuration`)))
  (`TimelineComponent.SetNewTime` _followspeed (`self.StartOffset`))
  (`Timeline|FollowSpeed`))

(event `Animate Legs`
  (`self.Animate BL`)
  (`self.Animate BR`)
  (`self.animate FL`)
  (`self.Animate FR`))

(event `Initialize Turrets`
  (for _array_element (`self.Sub Enemies`)
    (bind _asenemy (cast `/Game/Blueprints/Enemies/Enemy` (`ChildActorComponent.ChildActor` _array_element))
      (:`then`
        (set `/Game/Blueprints/Enemies/Enemy.PlayerReference` (`self.PlayerReference`) _asenemy)
        (`self.Initialize Enemy` _asenemy)
        (`KismetSystemLibrary.PrintString` "Initialized"))
      (:`CastFailed`
        (`KismetSystemLibrary.PrintString` "Failed to Cast Turret")))))

(event `self.ReceiveTick`
  (params (DeltaSeconds :type "Float (single-precision)"))
  (bind _returnvalue (`self.K2_GetActorLocation`))
  (bind _grounded_0 (`self.Grounded_0`))
  (bind _delta_seconds (`self.Delta Seconds`))
  (bind _returnvalue_2 (`KismetMathLibrary.DegSin` (`KismetSystemLibrary.GetGameTimeInSeconds`)))
  (bind _spline (`/Game/Blueprints/Player/BP_PlayerFollowSpline.Spline` (`self.Spline Instance`)))
  (bind _returnvalue_3 (`SplineComponent.GetNumberOfSplinePoints` _spline))
  (bind _returnvalue_4 (`KismetMathLibrary.Lerp` 0.0 (`SplineComponent.GetSplineLength` _spline) (`self.Alpha`)))
  (bind _returnvalue_5 (`SplineComponent.GetLocationAtDistanceAlongSpline` _spline _returnvalue_4 "World"))
  (bind _returnvalue_6 (`KismetMathLibrary.VInterpTo` _returnvalue (`KismetMathLibrary.SelectVector` _returnvalue_5 (+ _returnvalue_5 (* (`KismetMathLibrary.MakeVector` _returnvalue_2 _returnvalue_2 _returnvalue_2) 1.0)) (`self.Grounded_0`)) _delta_seconds 2.0))
  (bind _returnvalue_7 (- _returnvalue_6 _returnvalue))
  (`self.Enemy Health Visibility`)
  (set `self.Delta Seconds` DeltaSeconds)
  (`/Engine/EditorBlueprintResources/StandardMacros.IsValid` (`self.Spline Instance`)
    (:`Is Valid`
      (`|ExecutionSequence`
        (:`then_0`
          (`self.Death Check`)
          (set `self.Alpha` (/ (- _returnvalue_3 (`self.Lag`)) _returnvalue_3))
          (`self.K2_SetActorRotation` (`KismetMathLibrary.RInterpTo` (`self.K2_GetActorRotation`) (`KismetMathLibrary.SelectRotator` (`SplineComponent.GetRotationAtDistanceAlongSpline` _spline _returnvalue_4 "World") (`KismetMathLibrary.MakeRotator` 0.0 0.0 (.yaw (`KismetMathLibrary.FindLookAtRotation` _returnvalue (`SceneComponent.K2_GetComponentLocation` (`/Game/Blueprints/Player/BP_Player.Main Box Component` (`self.PlayerReference`)))))) _grounded_0) _delta_seconds (`KismetMathLibrary.SelectFloat` 8.0 0.5 _grounded_0)))
          (`self.K2_SetActorLocation` _returnvalue_6 true)
          (set `self.Forward Speed` (* (`KismetMathLibrary.VSize` (`KismetMathLibrary.ClampVectorSize` _returnvalue_7 -1.0 1.0)) 0.3))
          (if (`self.Grounded_0`)
            (`SceneComponent.K2_SetRelativeRotation` :`self` (`self.Rotor 2`))
            (`SceneComponent.K2_SetRelativeRotation` :`self` (`self.Rotor 1`))
            (`self.Animate Legs`)
            (else
              (`self.Gimbal Thrust` 0.0 (.y (`KismetMathLibrary.TransformLocation` (`self.GetTransform`) _returnvalue_7))))))
        (:`then_1`
          (`self.Ground Check`)
          (`self.Aim laser`))))))

(event `animate FL`
  (bind _asabp_leg (cast `/Game/Animations/ABP_Leg` (`SkeletalMeshComponent.GetAnimInstance` (`self.legFLSM`))))
  (`KismetSystemLibrary.Delay` 0.0)
  (set `/Game/Animations/ABP_Leg.ForwardSpeed` (* (`self.Forward Speed`) -1.0 (`KismetMathLibrary.SelectFloat` 1.8 0.0 (`self.Grounded_0`))) _asabp_leg))

(event `Animate FR`
  (bind _asabp_leg (cast `/Game/Animations/ABP_Leg` (`SkeletalMeshComponent.GetAnimInstance` (`self.legFRSM`))))
  (`KismetSystemLibrary.Delay` 0.2)
  (set `/Game/Animations/ABP_Leg.ForwardSpeed` (* (`self.Forward Speed`) (`KismetMathLibrary.SelectFloat` 1.8 0.0 (`self.Grounded_0`))) _asabp_leg))

(event `Animate BL`
  (bind _asabp_leg (cast `/Game/Animations/ABP_Leg` (`SkeletalMeshComponent.GetAnimInstance` (`self.legBLSM`))))
  (`KismetSystemLibrary.Delay` 0.2)
  (set `/Game/Animations/ABP_Leg.ForwardSpeed` (* (`self.Forward Speed`) (`KismetMathLibrary.SelectFloat` 1.8 0.0 (`self.Grounded_0`))) _asabp_leg))

(event `Animate BR`
  (bind _asabp_leg (cast `/Game/Animations/ABP_Leg` (`SkeletalMeshComponent.GetAnimInstance` (`self.legBRSM`))))
  (`KismetSystemLibrary.Delay` 0.0)
  (set `/Game/Animations/ABP_Leg.ForwardSpeed` (* (`self.Forward Speed`) (`KismetMathLibrary.SelectFloat` 1.8 0.0 (`self.Grounded_0`))) _asabp_leg))

(event `Death Check`
  (bind _returnvalue (`SceneComponent.K2_GetComponentLocation` (`self.Main Body`)))
  (if (not (`self.EnemyAlive`))
    (`/Engine/EditorBlueprintResources/StandardMacros.DoOnce` false
      (:`Completed`
        (`/Game/Widgets/WBP_PlayerHUD.Destroy Enemy` (`/Game/Blueprints/Player/BP_Player.HUD` (`self.PlayerReference`)) self)
        (`/Game/Blueprints/Player/BP_Player.Check Win State` (`self.PlayerReference`) false)
        (`GameplayStatics.SpawnEmitterAtLocation` "/Game/Particles/PS_Explosion.PS_Explosion" _returnvalue (struct) (10.0 10.0 10.0))
        (`KismetSystemLibrary.Delay` 2.0)
        (`GameplayStatics.SpawnEmitterAtLocation` "/Game/Particles/PS_Explosion.PS_Explosion" _returnvalue (struct) (10.0 10.0 10.0))
        (`/Engine/EditorBlueprintResources/StandardMacros.DoOnce` false
          (:`Completed`
            (`self.K2_DestroyActor`)))))))

(fn `UserConstructionScript`)
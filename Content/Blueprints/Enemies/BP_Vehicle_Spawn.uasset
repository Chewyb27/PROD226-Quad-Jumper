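; Enemy spawner actor that sends in a BP_DropShip high above its Sphere to deliver units, passing it patrol route, objective and player references.
; Tick either spawns once or, when using survival time, accumulates a timer to trigger repeat drops while the player is valid.
; Timed drops require no previous units, or clearance from both the last dropship and nearest unit; blocked attempts and successful spawns rewind the timer.
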(event `self.ReceiveBeginPlay`)

(event `self.ReceiveTick`
  (params (DeltaSeconds :type "Float (single-precision)"))
  (bind _previous_units (`self.Previous Units`))
  (bind _player (`self.Player`))
  (bind _location (.location (`SceneComponent.K2_GetComponentToWorld` (`self.Sphere`))))
  (bind _returnvalue (+ _location (* (`KismetMathLibrary.RandomUnitVector`) 1000.0) (0.0 0.0 25000.0)))
  (if (`self.SpawnOnce`)
    (`/Engine/EditorBlueprintResources/StandardMacros.DoOnce` false
      (:`Completed`
        (`/Engine/EditorBlueprintResources/StandardMacros.IsValid` _player :!label _label
          (:`Is Valid`
            (bind _returnvalue_2 (`|SpawnActorFromClass` "/Game/Blueprints/Enemies/Faction_1/BP_DropShip.BP_DropShip_C" (`KismetMathLibrary.MakeTransform` _returnvalue (`KismetMathLibrary.RandomRotator` false) (0.45 0.45 0.45)) "AdjustIfPossibleButAlwaysSpawn" "OverrideRootScale" null _location (`|MakeArray` 1 3) (`self.Dropped Enemy Patrol Route`) false (`self.Objective Trucks`) null true _player 1000.0 false false false (`self.Objective Dropship`) null false 1.0 0.0 true null))
            (set `self.Previous Dropship` _returnvalue_2)
            (set `self.time` (- (`self.time`) (`self.StepBackTime`)))))))
    (elif (`self.UsesSurvivalTime`)
      (set `self.time` (+ (`self.time`) DeltaSeconds))
      (if (< (`self.spawnontime`) (`self.time`))
        (if (or (`KismetArrayLibrary.Array_IsEmpty` _previous_units) (and (>= (`KismetMathLibrary.Vector_Distance` _returnvalue (`SceneComponent.K2_GetComponentLocation` (`/Game/Blueprints/Enemies/Faction_1/BP_DropShip.Main Body` (`self.Previous Dropship`)))) 2000.0) (>= (`GameplayStatics.FindNearestActor` (`SceneComponent.K2_GetComponentLocation` (`self.Sphere`)) _previous_units) 5000.0)))
          (goto _label)
          (else
            (set `self.time` (- (`self.time`) 10.0))))))))

(fn `UserConstructionScript`)
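; Segmented drill-worm enemy boss that wakes when the player comes near and carries mini laser turrets along its body.
; The construction script builds a drill head and alternating body meshes, and BeginPlay attaches a turret every fifth segment.
; Tick eases each segment toward a lag-offset spline point, using forward traces for ground-break effects.
; Death destroys the turrets, updates HUD and win state, then explodes.
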(event `Ground Check`)

(event `Gimbal Thrust`
  (params (Delta :type "Float (double-precision)") (MoveAmount :type "Float (double-precision)")))

(event `self.ReceiveBeginPlay`
  (for _index (range (+ (/ (`self.Total Segments`) 5) 1))
    (if (> _index 0)
      (bind _output (`|GetArrayItem` (`self.Sections`) (* _index 5)))
      (bind _returnvalue (`|SpawnActorFromClass` "/Game/Blueprints/Enemies/Faction_2/BP_Mini_Laser.BP_Mini_Laser_C" (`KismetMathLibrary.MakeTransform` (+ (`SceneComponent.K2_GetComponentLocation` _output) (0.0 0.0 1000.0)) (struct) (0.5 0.5 0.5)) "AlwaysSpawn" "OverrideRootScale" null 100.0 true 0.1 1.0 true (`self.PlayerReference`) 8000.0 false false false true null false 1.0 0.0 null))
      (`KismetArrayLibrary.Array_Add` (`self.Turrets`) _returnvalue)
      (`self.K2_AttachToComponent` _returnvalue _output "None" "KeepWorld" "KeepWorld" "KeepWorld" true)
      (`self.Initialize Enemy` _returnvalue))))

(event `Spawn Particles`
  (params (Location :type "Vector Structure"))
  (`/Engine/EditorBlueprintResources/StandardMacros.FlipFlop`
    (:`A`
      (`NiagaraFunctionLibrary.SpawnSystemAtLocation` "/Game/Particles/FXS_GroundBreakWorm.FXS_GroundBreakWorm" Location))))

(event `Aim laser`)

(event `Animate Legs`)

(event `Initialize Turrets`
  (for _array_element (`self.Sub Enemies`)
    (bind _asenemy (cast `/Game/Blueprints/Enemies/Enemy` (`ChildActorComponent.ChildActor` _array_element))
      (:`then`
        (set `/Game/Blueprints/Enemies/Enemy.PlayerReference` (`self.PlayerReference`) _asenemy)
        (`self.Initialize Enemy` _asenemy)
        (`KismetSystemLibrary.PrintString` "Initialized"))
      (:`CastFailed`
        (`KismetSystemLibrary.PrintString` "Failed to Cast Turret")))))

(event `Follow Sequence`
  (bind _followspeed (`self.FollowSpeed`))
  (`TimelineComponent.SetPlayRate` _followspeed (/ 1.0 (`self.StartDuration`)))
  (`TimelineComponent.SetNewTime` _followspeed (`self.StartOffset`))
  (`Timeline|FollowSpeed`))

(event `self.ReceiveTick`
  (params (DeltaSeconds :type "Float (single-precision)"))
  (bind _sections (`self.Sections`))
  (bind _enemy_class_display (`self.Enemy Class Display`))
  (bind _playerreference (`self.PlayerReference`))
  (bind _delta_seconds (`self.Delta Seconds`))
  (bind _spline (`/Game/Blueprints/Player/BP_PlayerFollowSpline.Spline` (`self.Spline Instance`)))
  (bind _returnvalue (`SplineComponent.GetNumberOfSplinePoints` _spline))
  (bind _returnvalue_2 (`KismetMathLibrary.Lerp` 0.0 (`SplineComponent.GetSplineLength` _spline) (`self.Alpha`)))
  (bind _returnvalue_3 (`SplineComponent.GetLocationAtDistanceAlongSpline` _spline _returnvalue_2 "World"))
  (`self.Enemy Health Visibility`)
  (set `self.Delta Seconds` DeltaSeconds)
  (`/Engine/EditorBlueprintResources/StandardMacros.IsValid` (`self.Spline Instance`)
    (:`Is Valid`
      (`|ExecutionSequence`
        (:`then_0`
          (`/Engine/EditorBlueprintResources/StandardMacros.IsValid` _playerreference
            (:`Is Valid`
              (if (<= (`KismetMathLibrary.Vector_Distance` (`SceneComponent.K2_GetComponentLocation` (`/Game/Blueprints/Player/BP_Player.Main Box Component` _playerreference)) (`SceneComponent.K2_GetComponentLocation` (`self.Enemy Body`))) 15000.0)
                (`/Engine/EditorBlueprintResources/StandardMacros.DoOnce` false
                  (:`Completed`
                    (set `self.Enemy Awake` true)))))))
        (:`then_1`
          (if (`self.Enemy Awake`)
            (`self.Death Check`)
            (if (`self.EnemyAlive`)
              (`SceneComponent.K2_AddRelativeRotation` (`self.Drill`) (* (struct :`Roll` 100.0) DeltaSeconds) false false)
              (for (_array_element _array_index) _sections
                (set `self.Alpha` (/ (- _returnvalue (+ (`self.Lag`) (* _array_index (`self.Segment Distance`)))) _returnvalue))
                (`/Engine/EditorBlueprintResources/StandardMacros.IsValid` _array_element
                  (:`Is Valid`
                    (bind _returnvalue_4 (`SceneComponent.K2_GetComponentLocation` _array_element))
                    (`SceneComponent.K2_SetWorldLocation` _array_element (`KismetMathLibrary.VInterpTo` _returnvalue_4 _returnvalue_3 _delta_seconds 1.0) false false)
                    (`SceneComponent.K2_SetWorldRotation` _array_element (`KismetMathLibrary.RInterpTo` (`SceneComponent.K2_GetComponentRotation` _array_element) (`SplineComponent.GetRotationAtDistanceAlongSpline` _spline _returnvalue_2 "World") _delta_seconds 1.0) false false)
                    (bind (_outhit _returnvalue_5) (`KismetSystemLibrary.LineTraceSingle` :`Start` _returnvalue_4 :`End` (+ (* (`SceneComponent.GetForwardVector` _array_element) 500.0) _returnvalue_4) :`TraceChannel` "TraceTypeQuery1" :`DrawDebugType` "ForOneFrame"))
                    (if _returnvalue_5
                      (`self.Spawn Particles` (`.ImpactPoint` (`GameplayStatics.BreakHitResult` _outhit)))))))
              (`/Engine/EditorBlueprintResources/StandardMacros.IsValid` _enemy_class_display
                (:`Is Valid`
                  (`SceneComponent.K2_SetWorldLocation` _enemy_class_display (`SceneComponent.K2_GetComponentLocation` (`|GetArrayItem` _sections)) false false)
                  (`SceneComponent.K2_SetWorldLocation` (`self.Targeted_Reticule`) (`SceneComponent.K2_GetComponentLocation` (`|GetArrayItem` _sections)) false false)
                  (set `self.Forward Speed` (* (`KismetMathLibrary.VSize` (`KismetMathLibrary.ClampVectorSize` (- (`KismetMathLibrary.VInterpTo_Constant` _returnvalue_4 _returnvalue_3) (`self.K2_GetActorLocation`)) -1.0 1.0)) 0.3)))))))))))

(event `animate FL`)

(event `Animate FR`)

(event `Animate BL`)

(event `Animate BR`)

(event `Death Check`
  (bind _returnvalue (`SceneComponent.K2_GetComponentLocation` (`self.Main Body`)))
  (if (not (`self.EnemyAlive`))
    (`/Engine/EditorBlueprintResources/StandardMacros.DoOnce` false
      (:`Completed`
        (for _array_element (`self.Turrets`)
          (`self.Take Damage` _array_element 10000.0 true)
          (`self.K2_DestroyActor` _array_element))
        (`/Game/Widgets/WBP_PlayerHUD.Destroy Enemy` (`/Game/Blueprints/Player/BP_Player.HUD` (`self.PlayerReference`)) self)
        (`/Game/Blueprints/Player/BP_Player.Check Win State` (`self.PlayerReference`) false)
        (`GameplayStatics.SpawnEmitterAtLocation` "/Game/Particles/PS_Explosion.PS_Explosion" _returnvalue (struct) (30.0 30.0 30.0))
        (`KismetSystemLibrary.Delay` 2.0)
        (`GameplayStatics.SpawnEmitterAtLocation` "/Game/Particles/PS_Explosion.PS_Explosion" _returnvalue (struct) (30.0 30.0 30.0))
        (`/Engine/EditorBlueprintResources/StandardMacros.DoOnce` false
          (:`Completed`
            (`self.K2_DestroyActor`)))))))

(fn `UserConstructionScript`
  (bind _sections (`self.Sections`))
  (for _index (range (+ (`self.Total Segments`) 1))
    (if (== _index 0)
      (bind _returnvalue (`KismetMathLibrary.MakeTransform` (+ (* _index (-500.0 0.0 0.0)) (-500.0 0.0 0.0))))
      (bind _returnvalue_2 (`AddComponent|NODE_AddStaticMeshComponent-3` :`RelativeTransform` _returnvalue))
      (`KismetArrayLibrary.Array_Add` _sections _returnvalue_2)
      (bind _returnvalue_3 (`AddComponent|NODE_AddStaticMeshComponent-2` :`RelativeTransform` _returnvalue))
      (`SceneComponent.K2_AttachToComponent` _returnvalue_3 _returnvalue_2 "None" "KeepWorld" "KeepWorld" "KeepWorld" true)
      (`StaticMeshComponent.SetStaticMesh` _returnvalue_3 "/Game/Models/Scene/Worm/Drill_Face_1_pTorusShape1.Drill_Face_1_pTorusShape1")
      (`SceneComponent.SetRelativeScale3D` _returnvalue_3 (2.0 2.0 2.0))
      (set `self.Drill` _returnvalue_3)
      (set `self.Enemy Body` _returnvalue_2)
      (else
        (bind _returnvalue_4 (`AddComponent|NODE_AddStaticMeshComponent-0` :`RelativeTransform` _returnvalue))
        (`KismetArrayLibrary.Array_Add` _sections _returnvalue_4)
        (`/Engine/EditorBlueprintResources/StandardMacros.FlipFlop`
          (:`A`
            (`StaticMeshComponent.SetStaticMesh` _returnvalue_4 "/Game/Models/Scene/Worm/Worm_Body_1.Worm_Body_1")
            (`SceneComponent.SetRelativeScale3D` _returnvalue_4 (2.0 2.0 2.0)))
          (:`B`
            (`StaticMeshComponent.SetStaticMesh` _returnvalue_4 "/Game/Models/Scene/Worm/Worm_Body_2.Worm_Body_2")
            (`SceneComponent.SetRelativeScale3D` _returnvalue_4 (2.0 2.0 2.0))))))))
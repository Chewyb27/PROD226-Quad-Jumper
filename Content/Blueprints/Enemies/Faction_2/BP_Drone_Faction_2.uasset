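; Faction 2 enemy drone that trails the player at a random offset and attacks with a periodic laser.
; Tick turns it toward the player and eases it to that player-relative point, using the line-trace hit when world geometry intervenes.
; After charging, a Niagara beam deals rising damage within range, with no line-of-sight check.
; Launch suspends following for a one-time forward push; death clears targeting, updates HUD and win state, then explodes.
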(event `self.ReceiveBeginPlay`
  (`parent.ReceiveBeginPlay`)
  (set `self.Enemy Body` (`self.Drone_Faction_2_pCylinder1`))
  (set `self.Orbit Location` (+ (* (`KismetMathLibrary.RandomUnitVectorInConeInDegrees` (`KismetMathLibrary.Normal` (+ (`KismetMathLibrary.Vector_Up`) (`KismetMathLibrary.Vector_Forward`))) 50.0) (`self.Maintain Distance`) (1.0 1.0 0.0)) (`KismetMathLibrary.MakeVector` 0.0 0.0 (`KismetMathLibrary.RandomFloatInRange` 1000.0 2000.0))))
  (set `self.Laser Delay` (`KismetMathLibrary.RandomFloatInRange` 0.0 0.4)))

(event `self.ReceiveTick`
  (params (DeltaSeconds :type "Float (single-precision)"))
  (bind _returnvalue (`self.K2_GetActorLocation`))
  (bind _laser_delay (`self.Laser Delay`))
  (bind _playerreference (`self.PlayerReference`))
  (bind _niagara (`self.Niagara`))
  (bind _playerreference_2 (`self.PlayerReference`))
  (bind _returnvalue_2 (+ DeltaSeconds _laser_delay))
  (bind _main_box_component (`/Game/Blueprints/Player/BP_Player.Main Box Component` (`self.PlayerReference`)))
  (bind _returnvalue_3 (`SceneComponent.K2_GetComponentLocation` (`/Game/Blueprints/Player/BP_Player.Main Body` _playerreference_2)))
  (bind _returnvalue_4 (`KismetMathLibrary.Vector_Distance` _returnvalue_3 _returnvalue))
  (bind _returnvalue_5 (+ (* (`KismetMathLibrary.TransformDirection` (`SceneComponent.K2_GetComponentToWorld` _main_box_component) (`self.Orbit Location`)) 1.0) _returnvalue_3))
  (`parent.ReceiveTick` DeltaSeconds)
  (`/Engine/EditorBlueprintResources/StandardMacros.IsValid` _playerreference_2
    (:`Is Valid`
      (if (`self.EnemyAlive`)
        (`|ExecutionSequence`
          (:`then_0`
            (if (>= _laser_delay 6.0)
              (if (<= _returnvalue_4 7000.0)
                (`FXSystemComponent.SetVectorParameter` _niagara "Beam End" _returnvalue_3)
                (`SceneComponent.SetVisibility` _niagara true false)
                (set `self.Laser Delay` _returnvalue_2)
                (`/Game/Blueprints/Player/BP_Player.Health Change` (`self.PlayerReference`) (* DeltaSeconds 1.0 (`self.Laser Delay`) -1.0) false)
                (if (>= _laser_delay 9.0)
                  (set `self.Laser Delay` 0.0)
                  (`SceneComponent.SetVisibility` _niagara false false))
                (else
                  (`SceneComponent.SetVisibility` _niagara false false)))
              (else
                (set `self.Laser Delay` (`KismetMathLibrary.FClamp` _returnvalue_2 0.0 6.0)))))
          (:`then_1`
            (if (not (`self.Launching`))
              (`self.K2_SetActorRotation` (`KismetMathLibrary.RInterpTo` (`self.K2_GetActorRotation`) (`KismetMathLibrary.FindLookAtRotation` _returnvalue _returnvalue_3) DeltaSeconds 1.5))
              (if (<= _returnvalue_4 15000.0)
                (bind (_outhit _returnvalue_6) (`KismetSystemLibrary.LineTraceSingleForObjects` (`SceneComponent.K2_GetComponentLocation` _main_box_component) _returnvalue_5 (`|MakeArray` "ObjectTypeQuery1" :!type "EObjectTypeQuery Enum")))
                (`self.K2_SetActorLocation` (`KismetMathLibrary.VInterpTo` _returnvalue (`KismetMathLibrary.SelectVector` (`.ImpactPoint` (`GameplayStatics.BreakHitResult` _outhit)) _returnvalue_5 _returnvalue_6) DeltaSeconds 0.5) true true)))))
        (else
          (`/Engine/EditorBlueprintResources/StandardMacros.DoOnce` false
            (:`Completed`
              (set `/Game/Blueprints/Player/BP_Player.Enemy Targeting` false _playerreference)
              (`KismetArrayLibrary.Array_RemoveItem` (`/Game/Blueprints/Player/BP_Player.Enemy Targeting Count` _playerreference) self)
              (`self.Death Animation`)
              (`self.Enemy Death`))))))))

(event `Death Animation`
  (`/Game/Widgets/WBP_PlayerHUD.Destroy Enemy` (`/Game/Blueprints/Player/BP_Player.HUD` (`self.PlayerReference`)) self)
  (`/Game/Blueprints/Player/BP_Player.Check Win State` (`self.PlayerReference`) false)
  (`GameplayStatics.SpawnEmitterAtLocation` "/Game/Particles/PS_Explosion.PS_Explosion" (`SceneComponent.K2_GetComponentLocation` (`self.Drone_Faction_2_pCylinder1`)) (struct) (10.0 10.0 10.0))
  (`self.K2_DestroyActor`))

(event `Launch`
  (bind _drone_faction_2_pcylinder1 (`self.Drone_Faction_2_pCylinder1`))
  (`/Engine/EditorBlueprintResources/StandardMacros.DoOnce` false
    (:`Completed`
      (set `self.Launching` true)
      (`Timeline|Launch Timeline` :!via `PlayFromStart`
        (:`Update`
          (`self.K2_SetActorLocation` (+ (* (`SceneComponent.GetForwardVector` _drone_faction_2_pcylinder1) (`GameplayStatics.GetWorldDeltaSeconds`) 1200.0) (`SceneComponent.K2_GetComponentLocation` _drone_faction_2_pcylinder1))))
        (:`Finished`
          (set `self.Launching` false))))))

(fn `UserConstructionScript`
  (`parent.UserConstructionScript`))
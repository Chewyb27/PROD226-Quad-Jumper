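; Inactive variant of the Faction 2 drone carrier enemy, with eight containers and no working drone-launch behavior.
; The construction script gives each container a random material and defect overlay for visual variety.
; At runtime it registers the Cube as the enemy body and keeps the class display on it while player references exist.
; Disconnected leftover nodes for registering, detaching and launching child drones never run.
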(event `self.ReceiveBeginPlay`
  (`parent.ReceiveBeginPlay`)
  (set `self.Enemy Body` (`self.Cube`)))

(event `self.ReceiveTick`
  (params (DeltaSeconds :type "Float (single-precision)"))
  (`parent.ReceiveTick` DeltaSeconds)
  (if (`KismetArrayLibrary.Array_IsNotEmpty` (`self.PlayerReference`))
    (`|ExecutionSequence`
      (:`then_1`
        (`SceneComponent.K2_SetWorldLocation` (`self.Enemy Class Display`) (`SceneComponent.K2_GetComponentLocation` (`self.Cube`)) false false)))))

(fn `UserConstructionScript`
  (`parent.UserConstructionScript`)
  (for _array_element (`|MakeArray` (`self.Container1`) (`self.Container2`) (`self.Container3`) (`self.Container4`) (`self.Container5`) (`self.Container6`) (`self.Container7`) (`self.Container8`))
    (`PrimitiveComponent.SetMaterial` _array_element 0 (`KismetArrayLibrary.Array_Random` (`self.Materials`)))
    (`MeshComponent.SetOverlayMaterial` _array_element (`KismetArrayLibrary.Array_Random` (`self.Defect Overlay`)))))
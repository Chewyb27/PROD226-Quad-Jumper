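; Allied laser turret that automatically attacks hostile BP_ShipTurret actors with a blue Niagara beam.
; SelectNewEnemy filters ship turrets by range, line of sight, life and allegiance to set ShipTarget, reselecting when the target is lost.
; Tick traces for a clear shot and counts down FiringDelay; the RecoilAbsorbtion timeline drives the beam while damage applies per second.
; DeathAnimation updates player HUD and win state, spawns explosions and powers the turret down.
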(event `Select New Enemy`
  (bind _allships (`self.Allships`))
  (bind _returnvalue (`SceneComponent.K2_GetComponentLocation` (`self.SM_Artillery_Base`)))
  (bind _outactors (`GameplayStatics.GetAllActorsOfClass` "/Game/Blueprints/Enemies/Faction_1/BP_ShipTurret.BP_ShipTurret_C"))
  (set `self.Allships` _outactors)
  (for _array_element _allships
    (bind _returnvalue_2 (`self.K2_GetActorLocation` _array_element))
    (bind (_outhit _returnvalue_3) (`KismetSystemLibrary.LineTraceSingle` _returnvalue _returnvalue_2 "TraceTypeQuery2" false _allships))
    (bind _asenemy (cast `/Game/Blueprints/Enemies/Enemy` _array_element))
    (if (or (>= (`KismetMathLibrary.Vector_Distance` _returnvalue_2 _returnvalue) 40000.0) (not (`/Game/Blueprints/Enemies/Enemy.EnemyAlive` _asenemy)) _returnvalue_3 (`/Game/Blueprints/Enemies/Enemy.Friendly` _asenemy))
      (`KismetArrayLibrary.Array_RemoveItem` _allships _array_element)
      (else
        (set `self.Ship Target` _array_element)
        (break))))
  (set `self.Ship Target` (`.ReturnValue` (`GameplayStatics.FindNearestActor` _returnvalue _allships))))

(event `self.ReceiveBeginPlay`
  (bind _out_actors (`self.Out Actors`))
  (bind _niagara (`self.Niagara`))
  (`parent.ReceiveBeginPlay`)
  (`GameplayStatics.GetAllActorsOfClass` "/Game/Blueprints/Scene/BP_Australis.BP_Australis_C")
  (set `self.Out Actors` (`|MakeArray` null :!type "Actor Object Reference"))
  (`FXSystemComponent.SetFloatParameter` _niagara "Beam Width" 100.0)
  (`SceneComponent.SetVisibility` _niagara false false)
  (`FXSystemComponent.SetColorParameter` _niagara "Color" (struct :`R` 0.027282 :`G` 0.298601 :`B` 1.0 :`A` 1.0))
  (set `self.Grounded` true)
  (set `self.Enemy Body` null)
  (set `self.Firing Delay` (`KismetMathLibrary.RandomFloatInRange` 0.0 5.0))
  (bind _returnvalue (`GameplayStatics.GetActorOfClass` "/Game/Blueprints/Scene/Large_Ship_Thing.Large_Ship_Thing_C"))
  (`KismetArrayLibrary.Array_Add` _out_actors _returnvalue)
  (bind _outactors (`GameplayStatics.GetAllActorsOfClass` "/Game/Blueprints/Enemies/Faction_1/BP_ShipTurret.BP_ShipTurret_C"))
  (set `self.Allships` _outactors)
  (`KismetArrayLibrary.Array_Append` _out_actors _outactors)
  (`self.Select New Enemy`))

(event `self.ReceiveTick`
  (params (DeltaSeconds :type "Float (single-precision)"))
  (bind _ship_target (`self.Ship Target`))
  (bind _ship_target_2 (`self.Ship Target`))
  (bind _niagara (`self.Niagara`))
  (bind _ship_target_3 (`self.Ship Target`))
  (`/Engine/EditorBlueprintResources/StandardMacros.IsValid` _ship_target_3
    (:`Is Valid`
      (bind _asenemy (cast `/Game/Blueprints/Enemies/Enemy` _ship_target_3)
        (:`then`
          (if (`/Game/Blueprints/Enemies/Enemy.EnemyAlive` _asenemy)
            (if (`self.Not Destroyed`)
              (bind _output_get (set `self.Delta Seconds` DeltaSeconds))
              (`/Engine/EditorBlueprintResources/StandardMacros.IsValid` _ship_target_2
                (:`Is Valid`
                  (bind _asenemy_2 (cast `/Game/Blueprints/Enemies/Enemy` _ship_target_2))
                  (if (not (`/Game/Blueprints/Enemies/Enemy.EnemyAlive` _asenemy_2))
                    (`self.Select New Enemy`))
                  (if (`self.Can Fire`)
                    (if (`self.Firing`)
                      (bind _asenemy_3 (cast `/Game/Blueprints/Enemies/Enemy` _ship_target_2))
                      (`self.Take Damage` _asenemy_3 (* _output_get 50.0) true null))
                    (else
                      (`self.Select New Enemy`))))
                (:`Is Not Valid`
                  (`self.Select New Enemy`)))
              (`/Engine/EditorBlueprintResources/StandardMacros.IsValid` (`self.Ship Target`)
                (:`Is Valid`
                  (if (not (`self.Targeting Player`))
                    (`self.Weapon Targeting` DeltaSeconds)
                    (if (<= (`self.Firing Delay`) 0.0)
                      (if (`self.Can Fire`)
                        (set `self.Firing Delay` 5.0)
                        (`SceneComponent.SetVisibility` _niagara true false)
                        (`Timeline|Recoil Absorbtion` :!via `PlayFromStart`
                          (:`Update`
                            (set `self.Firing` true)
                            (`SceneComponent.SetVisibility` _niagara true false)
                            (`/Engine/EditorBlueprintResources/StandardMacros.IsValid` _ship_target
                              (:`Is Valid`
                                (bind _asenemy_4 (cast `/Game/Blueprints/Enemies/Enemy` _ship_target))
                                (if (`/Game/Blueprints/Enemies/Enemy.EnemyAlive` _asenemy_4)
                                  (`FXSystemComponent.SetVectorParameter` _niagara "Beam End" (`self.K2_GetActorLocation` _ship_target))
                                  (else
                                    (`FXSystemComponent.SetVectorParameter` _niagara "Beam End" (`SceneComponent.K2_GetComponentLocation` (`self.BulletSpawn`)) :!label _label)
                                    (`self.Select New Enemy`))))
                              (:`Is Not Valid`
                                (goto _label))))
                          (:`Finished`
                            (`SceneComponent.SetVisibility` _niagara false false)
                            (set `self.Firing` false))))
                      (else
                        (set `self.Firing Delay` (`KismetMathLibrary.FClamp` (- (`self.Firing Delay`) DeltaSeconds) 0.0 100.0)))))))
              (else
                (`SceneComponent.SetVisibility` (`self.Niagara`) false false)))
            (else
              (`self.Select New Enemy` :!label _label_2))))
        (:`CastFailed`
          (goto _label_2))))
    (:`Is Not Valid`
      (goto _label_2))))

(event `Weapon Targeting`
  (params (Delta :type "Float (double-precision)"))
  (set `self.Targeting Player` false)
  (bind (_outhit _returnvalue) (`KismetSystemLibrary.LineTraceSingle` (`SceneComponent.K2_GetComponentLocation` (`self.BulletSpawn`)) (`self.K2_GetActorLocation` (`self.Ship Target`)) "TraceTypeQuery2" false (`self.Out Actors`)))
  (set `self.Can Fire` (not _returnvalue)))

(event `Death Animation`
  (bind _returnvalue (`SceneComponent.K2_GetComponentLocation` (`self.BulletSpawn`)))
  (for _array_element (`self.PlayerReference`)
    (`/Game/Widgets/WBP_PlayerHUD.Destroy Enemy` (`/Game/Blueprints/Player/BP_Player.HUD` _array_element) self)
    (`/Game/Blueprints/Player/BP_Player.Check Win State` _array_element false))
  (`GameplayStatics.SpawnEmitterAtLocation` "/Game/Particles/PS_Explosion.PS_Explosion" _returnvalue (struct) (10.0 10.0 10.0))
  (`KismetSystemLibrary.Delay` 0.1)
  (`GameplayStatics.SpawnEmitterAtLocation` "/Game/Particles/PS_Explosion.PS_Explosion" _returnvalue (struct) (10.0 10.0 10.0))
  (`/Engine/EditorBlueprintResources/StandardMacros.DoOnce` false
    (:`Completed`
      (set `self.EnemyAlive` false)
      (`PrimitiveComponent.SetMaterial` (`self.Glow Mesh1`) 0 "/Game/Materials/GeneralMaterials/M_Black_Padding.M_Black_Padding")
      (`self.Remove Lock`)
      (`Timeline|Power Down Turret`))))

(fn `UserConstructionScript`)
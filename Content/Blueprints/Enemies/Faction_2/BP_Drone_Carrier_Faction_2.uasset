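; Faction 2 drone carrier enemy that carries five child-actor drones and launches them when the player comes near.
; BeginPlay registers the child actor components in SubEnemies.
; Tick checks distance to the player's body; within range, it makes each valid drone HUD-visible, sets its body, enables its tick, calls Launch, removes it from SubEnemies and detaches it.
; No one-shot guard exists, so this repeats every in-range tick.
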(event `self.ReceiveBeginPlay`
  (for _array_element (`|MakeArray` (`self.ChildActor5`) (`self.ChildActor3`) (`self.ChildActor2`) (`self.ChildActor7`) (`self.ChildActor6`))
    (`KismetArrayLibrary.Array_Add` (`self.Sub Enemies`) _array_element)
    (bind _asbp_drone_faction_2 (cast `/Game/Blueprints/Enemies/Faction_2/BP_Drone_Faction_2` (`ChildActorComponent.ChildActor` _array_element)))))

(event `self.ReceiveTick`
  (params (DeltaSeconds :type "Float (single-precision)"))
  (bind _playerreference (`self.PlayerReference`))
  (`parent.ReceiveTick` DeltaSeconds)
  (`/Engine/EditorBlueprintResources/StandardMacros.IsValid` _playerreference
    (:`Is Valid`
      (if (<= (`KismetMathLibrary.Vector_Distance` (`SceneComponent.K2_GetComponentLocation` (`/Game/Blueprints/Player/BP_Player.Main Body` _playerreference)) (`self.K2_GetActorLocation`)) 15000.0)
        (for _array_element (`|MakeArray` (`self.ChildActor5`) (`self.ChildActor3`) (`self.ChildActor2`) (`self.ChildActor7`) (`self.ChildActor6`))
          (bind _childactor (`ChildActorComponent.ChildActor` _array_element))
          (`/Engine/EditorBlueprintResources/StandardMacros.IsValid` _childactor
            (:`Is Valid`
              (bind _asbp_drone_faction_2 (cast `/Game/Blueprints/Enemies/Faction_2/BP_Drone_Faction_2` _childactor))
              (set `/Game/Blueprints/Enemies/Enemy.Invisible On HUD` false _asbp_drone_faction_2)
              (set `/Game/Blueprints/Enemies/Enemy.Enemy Body` (`/Game/Blueprints/Enemies/Faction_2/BP_Drone_Faction_2.Drone_Faction_2_pCylinder1` _asbp_drone_faction_2) _asbp_drone_faction_2)
              (`self.SetActorTickEnabled` _asbp_drone_faction_2 true)
              (`self.SetActorTickEnabled` _childactor true)
              (`/Game/Blueprints/Enemies/Faction_2/BP_Drone_Faction_2.Launch` _asbp_drone_faction_2)
              (`KismetArrayLibrary.Array_RemoveItem` (`self.Sub Enemies`) _array_element)
              (`SceneComponent.K2_DetachFromComponent` _array_element "KeepWorld" "KeepWorld" "KeepWorld" true))))))))

(fn `UserConstructionScript`
  (`parent.UserConstructionScript`))
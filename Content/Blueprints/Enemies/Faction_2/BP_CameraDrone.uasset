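; Faction 2 camera drone enemy that can follow a patrol spline, watching for the player in a downward cone that turns red on detection.
; Once alerted, Tick turns it toward the player and eases it to a random orbit offset, while a timed Niagara laser deals ramping damage in range.
; Launch drives a one-time forward burst that suspends tracking; death clears targeting, updates HUD and win state, then explodes.
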(event `self.ReceiveBeginPlay`
  (`parent.ReceiveBeginPlay`)
  (set `self.Enemy Body` (`self.Drone_Faction_2_pCylinder1`))
  (set `self.Orbit Location` (* (`KismetMathLibrary.RandomUnitVectorInConeInDegrees` (`KismetMathLibrary.Vector_Up`) 70.0) (`self.Maintain Distance`) (1.0 1.0 0.25)))
  (`/Engine/EditorBlueprintResources/StandardMacros.IsValid` (`self.Patrol Route Spline`)
    (:`Is Valid`
      (`self.Follow Patrol Route` 0.0)
      (`FXSystemComponent.SetColorParameter` (`self.ConeShape`) "Color" (struct :`R` 0.027282 :`G` 0.2986 :`B` 1.0 :`A` 1.0)))))

(event `self.ReceiveTick`
  (params (DeltaSeconds :type "Float (single-precision)"))
  (bind _returnvalue (`self.K2_GetActorLocation`))
  (bind _laser_delay (`self.Laser Delay`))
  (bind _playerreference (`self.PlayerReference`))
  (bind _niagara (`self.Niagara`))
  (bind _playerreference_2 (`self.PlayerReference`))
  (bind _returnvalue_2 (`SceneComponent.K2_GetComponentLocation` (`self.Drone_Faction_2_pCylinder1`)))
  (bind _returnvalue_3 (+ DeltaSeconds _laser_delay))
  (bind _returnvalue_4 (`SceneComponent.K2_GetComponentLocation` (`/Game/Blueprints/Player/BP_Player.Main Box Component` (`self.PlayerReference`))))
  (bind _returnvalue_5 (`SceneComponent.K2_GetComponentLocation` (`/Game/Blueprints/Player/BP_Player.Main Body` _playerreference_2)))
  (bind _returnvalue_6 (`KismetMathLibrary.Vector_Distance` _returnvalue_5 _returnvalue))
  (`parent.ReceiveTick` DeltaSeconds)
  (`/Engine/EditorBlueprintResources/StandardMacros.IsValid` _playerreference_2
    (:`Is Valid`
      (if (`self.EnemyAlive`)
        (if (`self.Detected Player`)
          (`|ExecutionSequence`
            (:`then_0`
              (if (>= _laser_delay 6.0)
                (if (<= _returnvalue_6 7000.0)
                  (`FXSystemComponent.SetVectorParameter` _niagara "Beam End" _returnvalue_5)
                  (`SceneComponent.SetVisibility` _niagara true false)
                  (set `self.Laser Delay` _returnvalue_3)
                  (`/Game/Blueprints/Player/BP_Player.Health Change` (`self.PlayerReference`) (* DeltaSeconds 2.0 (`self.Laser Delay`) -1.0) false)
                  (if (>= _laser_delay 9.0)
                    (set `self.Laser Delay` 0.0)
                    (`SceneComponent.SetVisibility` _niagara false false))
                  (else
                    (`SceneComponent.SetVisibility` _niagara false false)))
                (else
                  (set `self.Laser Delay` (`KismetMathLibrary.FClamp` _returnvalue_3 0.0 6.0)))))
            (:`then_1`
              (if (not (`self.Launching`))
                (`self.K2_SetActorRotation` (`KismetMathLibrary.RInterpTo` (`self.K2_GetActorRotation`) (`KismetMathLibrary.FindLookAtRotation` _returnvalue _returnvalue_5) DeltaSeconds 1.5))
                (if (<= _returnvalue_6 15000.0)
                  (`self.K2_SetActorLocation` (`KismetMathLibrary.VInterpTo` _returnvalue (+ (* (`KismetMathLibrary.TransformDirection` (`SceneComponent.K2_GetComponentToWorld` (`/Game/Blueprints/Player/BP_Player.Main Box Component` (`self.PlayerReference`))) (`self.Orbit Location`)) 1.0) _returnvalue_5) DeltaSeconds 1.0) true true)))))
          (elif (< (`KismetMathLibrary.Vector_Distance` _returnvalue_4 _returnvalue_2) 10000.0)
            (if (>= (`KismetMathLibrary.Dot_VectorVector` (`KismetMathLibrary.Normal` (- _returnvalue_4 _returnvalue_2)) (`KismetMathLibrary.Vector_Down`)) 0.6)
              (set `self.Detected Player` true)
              (`FXSystemComponent.SetColorParameter` (`self.ConeShape`) "Color" (struct :`R` 1.0 :`A` 1.0)))))
        (else
          (`/Engine/EditorBlueprintResources/StandardMacros.DoOnce` false
            (:`Completed`
              (set `/Game/Blueprints/Player/BP_Player.Enemy Targeting` false _playerreference)
              (`KismetArrayLibrary.Array_RemoveItem` (`/Game/Blueprints/Player/BP_Player.Enemy Targeting Count` _playerreference) self)
              (`self.Death Animation`)
              (`self.Enemy Death`))))))))

(event `Death Animation`
  (`/Game/Widgets/WBP_PlayerHUD.Destroy Enemy` (`/Game/Blueprints/Player/BP_Player.HUD` (`self.PlayerReference`)) self)
  (`/Game/Blueprints/Player/BP_Player.Check Win State` (`self.PlayerReference`) false)
  (`GameplayStatics.SpawnEmitterAtLocation` "/Game/Particles/PS_Explosion.PS_Explosion" (`SceneComponent.K2_GetComponentLocation` (`self.Drone_Faction_2_pCylinder1`)) (struct) (10.0 10.0 10.0))
  (`self.K2_DestroyActor`))

(event `Launch`
  (`/Engine/EditorBlueprintResources/StandardMacros.DoOnce` false
    (:`Completed`
      (set `self.Launching` true)
      (`Timeline|Launch Timeline` :!via `PlayFromStart`
        (:`Update`
          (`self.K2_SetActorLocation` (+ (* (`SceneComponent.GetForwardVector` (`self.Drone_Faction_2_pCylinder1`)) (`GameplayStatics.GetWorldDeltaSeconds`) 1200.0) (`self.K2_GetActorLocation`))))
        (:`Finished`
          (set `self.Launching` false))))))

(fn `UserConstructionScript`
  (`parent.UserConstructionScript`))
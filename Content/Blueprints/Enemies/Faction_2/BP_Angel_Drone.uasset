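; Flying Angel Drone enemy that attacks the player with a periodic laser and a timed EMP charge.
; After line-of-sight detection, Tick orbits a random offset around the player, pushed off obstacles by capsule traces, and tilts the wings with movement.
; The Niagara beam deals rising damage; the charge swaps glow materials and rushes the player before a proximity-damage EMP.
; Launch drives forward movement by timeline; death notifies HUD and win check, then explodes.
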(event `Charge Attack`
  (bind _returnvalue (`self.K2_GetActorLocation`))
  (set `self.Charge Attack Timer` (+ (`KismetMathLibrary.RandomFloatInRange` 0.0 15.0) 12.0))
  (set `self.Running Charge Attack` true)
  (`self.Change Wing Materials` "/Game/Materials/SpecialEffects/M_Timer.M_Timer" "/Game/Materials/SpecialEffects/M_Timer.M_Timer")
  (`KismetSystemLibrary.Delay` 3.0)
  (`NiagaraFunctionLibrary.SpawnSystemAtLocation` "/Game/Particles/EMP.EMP" _returnvalue (struct) (1.0 1.0 1.0) true true "AutoRelease")
  (set `self.Running Charge Attack` false)
  (`self.Change Wing Materials` "/Game/Materials/GeneralMaterials/M_GlowDim.M_GlowDim" "/Game/Materials/GeneralMaterials/M_Glow.M_Glow")
  (if (< (`KismetMathLibrary.Vector_Distance` (`SceneComponent.K2_GetComponentLocation` (`/Game/Blueprints/Player/BP_Player.Main Body` (`self.PlayerReference`))) _returnvalue) 2000.0)
    (`/Game/Blueprints/Player/BP_Player.Health Change` (`self.PlayerReference`) -75.0 false)))

(event `self.ReceiveBeginPlay`
  (`parent.ReceiveBeginPlay`)
  (set `self.Enemy Body` (`self.Drone Body`))
  (set `self.Orbit Location` (* (`KismetMathLibrary.RandomUnitVectorInConeInDegrees` (`KismetMathLibrary.Vector_Up`) 70.0) (`self.Maintain Distance`) (1.0 1.0 0.25)))
  (set `self.Charge Attack Timer` (+ (`KismetMathLibrary.RandomFloatInRange` 0.0 20.0) 5.0)))

(event `self.ReceiveTick`
  (params (DeltaSeconds :type "Float (single-precision)"))
  (bind _returnvalue (`self.GetTransform`))
  (bind _returnvalue_2 (`self.K2_GetActorRotation`))
  (bind _returnvalue_3 (`self.K2_GetActorLocation`))
  (bind _returnvalue_4 (`self.K2_GetActorLocation`))
  (bind _laser_delay (`self.Laser Delay`))
  (bind _playerreference (`self.PlayerReference`))
  (bind _niagara (`self.Niagara`))
  (bind _playerreference_2 (`self.PlayerReference`))
  (bind _running_charge_attack (`self.Running Charge Attack`))
  (bind _charge_attack_timer (`self.Charge Attack Timer`))
  (bind _returnvalue_5 (+ DeltaSeconds _laser_delay))
  (bind _returnvalue_6 (`SceneComponent.K2_GetComponentLocation` (`/Game/Blueprints/Player/BP_Player.Main Body` _playerreference_2)))
  (bind _returnvalue_7 (`SceneComponent.K2_GetComponentLocation` (`/Game/Blueprints/Player/BP_Player.Main Body` (`self.PlayerReference`))))
  (bind _returnvalue_8 (`KismetMathLibrary.Vector_Distance` _returnvalue_6 _returnvalue_4))
  (bind _returnvalue_9 (`KismetMathLibrary.RInterpTo` _returnvalue_2 (`KismetMathLibrary.FindLookAtRotation` _returnvalue_4 _returnvalue_6) DeltaSeconds (`KismetMathLibrary.SelectFloat` 10.0 1.5 _running_charge_attack)))
  (`parent.ReceiveTick` DeltaSeconds)
  (`/Engine/EditorBlueprintResources/StandardMacros.IsValid` _playerreference_2
    (:`Is Valid`
      (if (`self.EnemyAlive`)
        (if (`self.FoundPlayer`)
          (`|ExecutionSequence`
            (:`then_0`
              (if (>= _laser_delay 6.0)
                (if (<= _returnvalue_8 7000.0)
                  (`FXSystemComponent.SetVectorParameter` _niagara "Beam End" _returnvalue_6)
                  (`SceneComponent.SetVisibility` _niagara true false)
                  (set `self.Laser Delay` _returnvalue_5)
                  (`/Game/Blueprints/Player/BP_Player.Health Change` (`self.PlayerReference`) (* DeltaSeconds 2.0 (`self.Laser Delay`) -1.0) false)
                  (if (>= _laser_delay 9.0)
                    (set `self.Laser Delay` 0.0)
                    (`SceneComponent.SetVisibility` _niagara false false))
                  (else
                    (`SceneComponent.SetVisibility` _niagara false false)))
                (else
                  (set `self.Laser Delay` (`KismetMathLibrary.FClamp` _returnvalue_5 0.0 6.0)))))
            (:`then_1`
              (if (`self.Launching`)
                _
                (elif (<= _returnvalue_8 15000.0)
                  (bind (_outhit _returnvalue_10) (`KismetSystemLibrary.CapsuleTraceSingle` _returnvalue_4 (+ _returnvalue_4 (* (`KismetMathLibrary.GetForwardVector` _returnvalue_2) 200.0)) 500.0 300.0 "TraceTypeQuery1" false (`|MakeArray` _playerreference_2 :!type "Actor Object Reference")))
                  (bind (_bblockinghit _binitialoverlap _time _distance _location _impactpoint _normal _impactnormal _physmat _hitactor) (`GameplayStatics.BreakHitResult` _outhit))
                  (bind _returnvalue_11 (* (+ _normal (0.0 0.0 0.0)) 7000.0))
                  (bind _returnvalue_12 (and (not (`KismetMathLibrary.ClassIsChildOf` (`GameplayStatics.GetObjectClass` _hitactor) "/Game/Blueprints/Enemies/Enemy.Enemy_C")) _returnvalue_10))
                  (bind _returnvalue_13 (`KismetMathLibrary.SelectVector` (`KismetMathLibrary.VInterpTo_Constant` _returnvalue_4 (+ _returnvalue_6 (0.0 0.0 500.0) (`KismetMathLibrary.SelectVector` _returnvalue_11 (0.0 0.0 0.0) (and _returnvalue_12 (<= 3000.0 _returnvalue_8)))) DeltaSeconds 5000.0) (`KismetMathLibrary.VInterpTo` _returnvalue_4 (+ (+ (* (`KismetMathLibrary.TransformDirection` (`SceneComponent.K2_GetComponentToWorld` (`/Game/Blueprints/Player/BP_Player.Main Box Component` (`self.PlayerReference`))) (`self.Orbit Location`)) 1.0) _returnvalue_6) (`KismetMathLibrary.SelectVector` _returnvalue_11 (0.0 0.0 0.0) _returnvalue_12)) DeltaSeconds 0.4) _running_charge_attack))
                  (`self.K2_SetActorLocation` _returnvalue_13 true true)
                  (`self.K2_SetActorRotation` _returnvalue_9)
                  (`self.Wing Movements` (`KismetMathLibrary.InverseTransformRotation` _returnvalue _returnvalue_9) (`KismetMathLibrary.InverseTransformLocation` _returnvalue _returnvalue_13) DeltaSeconds))))
            (:`then_2`
              (if (< (`KismetMathLibrary.Vector_Distance` _returnvalue_7 _returnvalue_3) 15000.0)
                (if (> _charge_attack_timer 0.0)
                  (set `self.Charge Attack Timer` (- _charge_attack_timer DeltaSeconds))
                  (else
                    (`self.Charge Attack`))))))
          (else
            (bind (_outhit_2 _returnvalue_14) (`KismetSystemLibrary.LineTraceSingle` _returnvalue_3 _returnvalue_7 "TraceTypeQuery1" false (`|MakeArray` (`self.PlayerReference`) :!type "Actor Object Reference")))
            (if (not _returnvalue_14)
              (set `self.FoundPlayer` true))))
        (else
          (`/Engine/EditorBlueprintResources/StandardMacros.DoOnce` false
            (:`Completed`
              (set `/Game/Blueprints/Player/BP_Player.Enemy Targeting` false _playerreference)
              (`KismetArrayLibrary.Array_RemoveItem` (`/Game/Blueprints/Player/BP_Player.Enemy Targeting Count` _playerreference) self)
              (`self.Death Animation`)
              (`self.Enemy Death`))))))))

(event `Death Animation`
  (`/Game/Widgets/WBP_PlayerHUD.Destroy Enemy` (`/Game/Blueprints/Player/BP_Player.HUD` (`self.PlayerReference`)) self)
  (`/Game/Blueprints/Player/BP_Player.Check Win State` (`self.PlayerReference`) false)
  (`GameplayStatics.SpawnEmitterAtLocation` "/Game/Particles/PS_Explosion.PS_Explosion" (`SceneComponent.K2_GetComponentLocation` (`self.Drone Body`)) (struct) (10.0 10.0 10.0))
  (`self.K2_DestroyActor`))

(event `Launch`
  (`/Engine/EditorBlueprintResources/StandardMacros.DoOnce` false
    (:`Completed`
      (set `self.Launching` true)
      (`Timeline|Launch Timeline` :!via `PlayFromStart`
        (:`Update`
          (`self.K2_SetActorLocation` (+ (* (`SceneComponent.GetForwardVector` (`self.Drone Body`)) (`GameplayStatics.GetWorldDeltaSeconds`) 1200.0) (`self.K2_GetActorLocation`))))
        (:`Finished`
          (set `self.Launching` false))))))

(fn `Change Wing Materials`
  (params (Dimmer :type "MaterialInterface Object Reference") (Brighter :type "MaterialInterface Object Reference"))
  (for _array_element (`|MakeArray` (`self.TopRightWingMesh`) (`self.BackRightWingMesh`) (`self.BottomRightWingMesh`) (`self.TopLeftWingMesh`) (`self.BackLeftWingMesh`) (`self.BottomLeftWingMesh`) :!type "PrimitiveComponent Object Reference")
    (`PrimitiveComponent.SetMaterial` _array_element 1 Dimmer))
  (for _array_element_2 (`|MakeArray` (`self.Drone Body`) (`self.DroneRightGun`) (`self.Drone Left Gun`) :!type "PrimitiveComponent Object Reference")
    (`PrimitiveComponent.SetMaterial` _array_element_2 2 Brighter)))

(fn `UserConstructionScript`
  (`parent.UserConstructionScript`))

(fn `Wing Movements`
  (params (`Rotation Value` :type "Rotator Structure") (`Translational Value` :type "Vector Structure") (Delta :type "Float (double-precision)"))
  (bind _bottomleftwing (`self.BottomLeftWing`))
  (bind _bottomrightwing (`self.BottomRightWing`))
  (bind _returnvalue (/ (.x `Translational Value`) 150.0))
  (bind _returnvalue_2 (`KismetMathLibrary.RInterpTo` (`SceneComponent.RelativeRotation` _bottomleftwing) (`KismetMathLibrary.MakeRotator` 0.0 0.0 (`KismetMathLibrary.ClampAngle` (* 1.0 -10.0 (* _returnvalue 10.0)) -40.0 10.0)) Delta 10.0))
  (bind _returnvalue_3 (`KismetMathLibrary.RInterpTo` (`SceneComponent.RelativeRotation` _bottomrightwing) (`KismetMathLibrary.MakeRotator` 0.0 0.0 (`KismetMathLibrary.ClampAngle` (* 1.0 -10.0 (* _returnvalue -10.0)) -10.0 40.0)) Delta 10.0))
  (`SceneComponent.K2_SetRelativeRotation` (`self.TopLeftWing`) _returnvalue_2 false false)
  (`SceneComponent.K2_SetRelativeRotation` (`self.BackLeftWing`) _returnvalue_2 false false)
  (`SceneComponent.K2_SetRelativeRotation` _bottomleftwing _returnvalue_2 false false)
  (`SceneComponent.K2_SetRelativeRotation` (`self.TopRightWing`) _returnvalue_3 false false)
  (`SceneComponent.K2_SetRelativeRotation` (`self.BackRightWing`) _returnvalue_3 false false)
  (`SceneComponent.K2_SetRelativeRotation` _bottomrightwing _returnvalue_3 false false))
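; Faction 2 variant of an enemy drop ship that deploys that faction's tanks.
; On initialization it runs the parent logic, then passes the player reference to the enemy in its child actor component and initializes it.
; Spawning a tank creates a Faction 2 tank with patrol spline and convoy offset, initializes it, and records it in the dropped units and any valid spawner's unit list.
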(fn `Initialize Enemy1`
  (`parent.Initialize Enemy1`)
  (for _array_element (`|MakeArray` (`self.ChildActor2`))
    (bind _asenemy (cast `/Game/Blueprints/Enemies/Enemy` (`ChildActorComponent.ChildActor` _array_element)))
    (set `/Game/Blueprints/Enemies/Enemy.PlayerReference` (`self.PlayerReference`) _asenemy)
    (`self.Initialize Enemy1` _asenemy)))

(fn `Spawn Enemy Tank`
  (params (SpawnTransform :type "Transform Structure") (PlayerReference :type "Array of /Game/Blueprints/Player/BP_Player Object Reference (by ref)") (`Patrol Route Spline` :type "/Game/Blueprints/Scene/VehiclePatrolRoute Object Reference") (`Convoy Offset` :type "Float (double-precision)"))
  (bind _spawner (`self.Spawner`))
  (bind _returnvalue (`|SpawnActorFromClass` "/Game/Blueprints/Enemies/Faction_2/BP_Tank_Faction_2.BP_Tank_Faction_2_C" SpawnTransform "AdjustIfPossibleButAlwaysSpawn" "OverrideRootScale" null true PlayerReference 800.0 false false false true false false `Patrol Route Spline` false 1.0 `Convoy Offset` false 15000.0 null))
  (`self.Initialize Enemy1` _returnvalue)
  (`KismetArrayLibrary.Array_Add` (`self.Dropped Units`) _returnvalue)
  (`/Engine/EditorBlueprintResources/StandardMacros.IsValid` _spawner
    (:`Is Valid`
      (`KismetArrayLibrary.Array_Add` (`/Game/Blueprints/Enemies/BP_Vehicle_Spawn.Previous Units` _spawner) _returnvalue))))

(fn `UserConstructionScript`
  (`parent.UserConstructionScript`))
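; EnemyRemains is an actor that bursts a destroyed enemy's mesh into fragments, then destroys itself after a few seconds.
; On BeginPlay it copies the static mesh into a procedural mesh and repeatedly slices it on random planes with capped cuts, pausing briefly between slices.
; It then attaches an explosion emitter, applies outward velocity impulses to the pieces and makes them ignore collision.
; The Niagara fragment, material-swap and construction-script slicing paths are disconnected.
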(event `self.ReceiveBeginPlay`
  (bind _returnvalue (`KismetMathLibrary.RandomUnitVector`))
  (bind _staticmesh (`self.StaticMesh`))
  (bind _proceduralmesh (`self.ProceduralMesh`))
  (bind _proceduralmesh_2 (`self.ProceduralMesh`))
  (bind _returnvalue_2 (`PrimitiveComponent.GetCenterOfMass` _proceduralmesh_2 "None"))
  (`StaticMeshComponent.SetStaticMesh` _staticmesh (`self.Static Mesh`))
  (`KismetProceduralMeshLibrary.CopyProceduralMeshFromStaticMeshComponent` _staticmesh 0 _proceduralmesh true)
  (`ProceduralMeshComponent.SetMeshSectionVisible` _proceduralmesh 0 true)
  (`PrimitiveComponent.SetCollisionResponseToAllChannels` _proceduralmesh "ECR_Ignore")
  (for _ (range 4)
    (`KismetSystemLibrary.Delay` 0.05)
    (bind _outotherhalfprocmesh (`KismetProceduralMeshLibrary.SliceProceduralMesh` _proceduralmesh (+ (`SceneComponent.K2_GetComponentLocation` (`self.ProceduralMesh`)) (* _returnvalue 1.0)) _returnvalue true "CreateNewSectionForCap" "/Game/Materials/GeneralMaterials/M_GeneralDestructable.M_GeneralDestructable"))
    (`PrimitiveComponent.SetSimulatePhysics` _outotherhalfprocmesh false)
    (`KismetArrayLibrary.Array_Add` (`self.Meshes`) _outotherhalfprocmesh))
  (`GameplayStatics.SpawnEmitterAttached` "/Game/Particles/PS_Explosion.PS_Explosion" (`self.ProceduralMesh`) "None" (0.0 0.0 0.0) (struct) (20.0 20.0 20.0) "SnapToTarget")
  (`KismetSystemLibrary.Delay` 0.1)
  (for _array_element (`self.Meshes`)
    (bind _returnvalue_3 (`PrimitiveComponent.GetCenterOfMass` _array_element "None"))
    (`PrimitiveComponent.AddVelocityChangeImpulseAtLocation` _array_element (* (`KismetMathLibrary.Normal` (- _returnvalue_3 (`SceneComponent.K2_GetComponentLocation` _proceduralmesh_2))) 3000.0) _returnvalue_3 "None")
    (`PrimitiveComponent.SetCollisionResponseToAllChannels` _array_element "ECR_Ignore"))
  (`PrimitiveComponent.AddVelocityChangeImpulseAtLocation` _proceduralmesh_2 (* (`KismetMathLibrary.Normal` (- _returnvalue_2 (`SceneComponent.K2_GetComponentLocation` _proceduralmesh_2))) 3000.0) _returnvalue_2 "None")
  (`PrimitiveComponent.SetCollisionResponseToAllChannels` _proceduralmesh_2 "ECR_Ignore")
  (`KismetSystemLibrary.Delay` 3.0)
  (`self.K2_DestroyActor`))

(event `self.ProceduralMesh.OnComponentHit`
  (params (HitComponent :type "PrimitiveComponent Object Reference") (OtherActor :type "Actor Object Reference") (OtherComp :type "PrimitiveComponent Object Reference") (NormalImpulse :type "Vector Structure") (Hit :type "HitResult Structure (by ref)")))

(fn `UserConstructionScript`)
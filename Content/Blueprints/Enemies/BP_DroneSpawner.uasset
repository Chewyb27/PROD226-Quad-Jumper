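; Drone spawner that creates a leader-led swarm of BP_Drone actors on waves enabled in SpawnOnWaves, checking wave 0 at BeginPlay.
; The first drone spawns at the spawner as leader, with followers at random offsets around it.
; Each receives the patrol spline, player, convoy offset and formation location, then links to the leader and swarm.
; MinGroupSize is effectively unused, as the random-size node is disconnected and MaxGroupSize bounds the loop.
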(event `self.ReceiveBeginPlay`
  (if (`|GetArrayItem` (`self.Spawn on waves`))
    (`self.Spawn Drones` 2 4)))

(event `Spawn Drones`
  (params (`Min Group Size` :type Integer) (`Max Group Size` :type Integer) (Wave :type Integer))
  (bind _drones_of_group (`self.Drones Of Group`))
  (bind _location (.location (`self.GetTransform`)))
  (bind _returnvalue (* (`KismetMathLibrary.RandomUnitVector`) 1000.0))
  (if (`|GetArrayItem` (`self.Spawn on waves`) Wave)
    (`KismetArrayLibrary.Array_Clear` _drones_of_group)
    (for _index (range (+ `Max Group Size` 1))
      (bind _returnvalue_2 (< _index 1))
      (bind _returnvalue_3 (`|SpawnActorFromClass` "/Game/Blueprints/Enemies/BP_Drone.BP_Drone_C" (`KismetMathLibrary.MakeTransform` (`KismetMathLibrary.SelectVector` _location (+ _location _returnvalue) _returnvalue_2) (.rotation (`self.GetTransform`)) (1.25 1.25 1.25)) "AdjustIfPossibleButAlwaysSpawn" "OverrideRootScale" self _returnvalue_2 _returnvalue self true (`self.Player`) 200.0 false false false false (`self.Patrol Route Spline`) true 1.5 (`KismetMathLibrary.Conv_IntToDouble` _index) null))
      (`/Engine/EditorBlueprintResources/StandardMacros.IsValid` (`self.Player`)
        (:`Is Valid`
          _)
        (:`Is Not Valid`
          _))
      (`KismetArrayLibrary.Array_Add` _drones_of_group _returnvalue_3)
      (set `/Game/Blueprints/Enemies/BP_Drone.Leader` (`|GetArrayItem` (`self.Drones Of Group`)) _returnvalue_3))
    (for _array_element (`self.Drones Of Group`)
      (set `/Game/Blueprints/Enemies/BP_Drone.Others in Swarm` (`self.Drones Of Group`) _array_element))))

(fn `UserConstructionScript`)
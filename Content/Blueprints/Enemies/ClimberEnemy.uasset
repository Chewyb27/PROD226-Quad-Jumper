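; Climber enemy that keeps itself oriented to and attached to surfaces such as walls; no forward movement is implemented here.
; Each Tick, Alignment sums normals from forward-down and downward traces, and CalculateAlignment turns them into stepped local pitch and roll.
; Without a usable normal, the root pitches steadily to find a surface.
; StickToWall then snaps the root above the downward hit; debug drawing is active and disconnected experiments remain.
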(event `self.ReceiveTick`
  (params (DeltaSeconds :type "Float (single-precision)"))
  (`parent.ReceiveTick` DeltaSeconds)
  (bind _on_wall (`self.Alignment` DeltaSeconds))
  (set `self.On Wall` _on_wall)
  (`self.Stick To Wall` DeltaSeconds))

(fn `Alignment`
  (params (DeltaTime :type "Float (single-precision)"))
  (returns (`On Wall` :type Boolean))
  (locals (Normal :type "Vector Structure"))
  (bind _normal (`local.Normal`))
  (bind _defaultsceneroot (`self.DefaultSceneRoot`))
  (bind _defaultsceneroot_2 (`self.DefaultSceneRoot`))
  (bind _returnvalue (`SceneComponent.GetUpVector` _defaultsceneroot_2))
  (bind _returnvalue_2 (`KismetMathLibrary.Normal` _normal))
  (bind _returnvalue_3 (!= _normal (0.0 0.0 0.0)))
  (bind _returnvalue_4 (* _returnvalue -1.0))
  (bind _returnvalue_5 (+ (`SceneComponent.K2_GetComponentLocation` _defaultsceneroot_2) (* _returnvalue 300.0)))
  (set `local.Normal` (0.0 0.0 0.0))
  (`|ExecutionSequence`
    (:`then_0`
      (bind (_outhit _returnvalue_6) (`KismetSystemLibrary.LineTraceSingle` :`Start` _returnvalue_5 :`End` (+ _returnvalue_5 (* (+ (* (`SceneComponent.GetForwardVector` _defaultsceneroot_2) 2.0) _returnvalue_4) 699.0)) :`TraceChannel` "TraceTypeQuery1" :`DrawDebugType` "ForOneFrame"))
      (if _returnvalue_6
        (set `local.Normal` (+ (`local.Normal`) (`.ImpactNormal` (`GameplayStatics.BreakHitResult` _outhit))))))
    (:`then_1`
      (bind (_outhit_2 _returnvalue_7) (`KismetSystemLibrary.LineTraceSingle` :`Start` _returnvalue_5 :`End` (+ _returnvalue_5 (* _returnvalue_4 2000.0)) :`TraceChannel` "TraceTypeQuery1" :`DrawDebugType` "ForOneFrame"))
      (if _returnvalue_7
        (set `local.Normal` (+ (`local.Normal`) (`.ImpactNormal` (`GameplayStatics.BreakHitResult` _outhit_2))))
        (else
          (set `local.Normal` (0.0 0.0 0.0)))))
    (:`then_2`
      (`KismetSystemLibrary.DrawDebugArrow` _returnvalue_5 (+ _returnvalue_5 (* _returnvalue_2 1000.0)) 100.0 (struct :`R` 1.0 :`G` 0.350361 :`A` 1.0) DeltaTime 100.0)
      (bind _returnvalue_8 (`self.Calculate Alignment` DeltaTime _returnvalue_2))
      (if _returnvalue_3
        (`SceneComponent.K2_SetWorldRotation` _defaultsceneroot _returnvalue_8 true false)
        (else
          (`SceneComponent.K2_AddLocalRotation` _defaultsceneroot (`KismetMathLibrary.MakeRotator` 0.0 (* DeltaTime -200.0)) true false)))
      (return _returnvalue_3))))

(fn `Calculate Alignment`
  (params (DeltaTime :type "Float (single-precision)") (Normal :type "Vector Structure"))
  (returns (ReturnValue :type "Rotator Structure"))
  (bind _adjustmentscalar (`self.AdjustmentScalar`))
  (bind _defaultsceneroot (`self.DefaultSceneRoot`))
  (bind _returnvalue (`SceneComponent.K2_GetComponentToWorld` _defaultsceneroot))
  (bind (_returnvalue_roll _returnvalue_pitch _returnvalue_yaw) (`KismetMathLibrary.BreakRotator` (`KismetMathLibrary.InverseTransformRotation` _returnvalue (`SceneComponent.K2_GetComponentRotation` _defaultsceneroot))))
  (bind _returnvalue_2 (`KismetMathLibrary.Normal` (`KismetMathLibrary.InverseTransformDirection` _returnvalue (`KismetMathLibrary.SelectVector` (`SceneComponent.GetForwardVector` _defaultsceneroot) Normal (== Normal (0.0 0.0 0.0))))))
  (bind _returnvalue_3 (`KismetMathLibrary.Dot_VectorVector` _returnvalue_2 (`KismetMathLibrary.InverseTransformDirection` _returnvalue (`SceneComponent.GetForwardVector` _defaultsceneroot))))
  (return (`KismetMathLibrary.TransformRotation` _returnvalue (`KismetMathLibrary.MakeRotator` (* (- 0.0 (.y _returnvalue_2)) -5.0 1.5) (`KismetMathLibrary.SelectFloat` 0.0 (* (/ (* 1.0 _returnvalue_3) (`KismetMathLibrary.Abs` _returnvalue_3)) -5.0 1.5) (and (> _returnvalue_3 (* _adjustmentscalar -1.0)) (< 0.0 _adjustmentscalar))) _returnvalue_yaw))))

(fn `Stick To Wall`
  (params (DeltaTime :type "Float (single-precision)"))
  (bind _defaultsceneroot (`self.DefaultSceneRoot`))
  (bind (_outhit _returnvalue) (`KismetSystemLibrary.LineTraceSingle` :`Start` (`SceneComponent.K2_GetComponentLocation` _defaultsceneroot) :`End` (+ (`SceneComponent.K2_GetComponentLocation` _defaultsceneroot) (* (`SceneComponent.GetUpVector` _defaultsceneroot) -2050.0)) :`TraceChannel` "TraceTypeQuery1" :`DrawDebugType` "ForOneFrame"))
  (if _returnvalue
    (bind (_bblockinghit _binitialoverlap _time _distance _location _impactpoint _normal _impactnormal) (`GameplayStatics.BreakHitResult` _outhit))
    (`SceneComponent.K2_SetWorldLocation` _defaultsceneroot (+ _location (* _impactnormal 100.0 1.0)) true false)))

(fn `UserConstructionScript`
  (`parent.UserConstructionScript`))
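; Super Heavy Tank enemy that targets a random NewWalker player and explodes when its health runs out.
; While active, Tick slowly turns the body and pitches the clamped gun pivot toward the player within range.
; An Enemy_Health widget shows name and health, visible only when active and near the player.
; FireMinigun is called but empty; its rate-limited Tank_GunFire spawning logic is disconnected, so the tank never fires.
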(event `Health Visibility`
  (bind _player (`self.Player`))
  (bind _display (`self.Display`))
  (`/Engine/EditorBlueprintResources/StandardMacros.IsValid` _player
    (:`Is Valid`
      (`SceneComponent.SetVisibility` _display (and (<= (`KismetMathLibrary.Vector_Distance` (`SceneComponent.K2_GetComponentLocation` (`/Game/Blueprints/Player/NewWalker.Main Body` _player)) (`SceneComponent.K2_GetComponentLocation` (`self.Tank Body`))) 15000.0) (`self.Active`)) false))
    (:`Is Not Valid`
      (`SceneComponent.SetVisibility` _display false false))))

(event `self.ReceiveBeginPlay`
  (bind _health (`self.Health`))
  (`self.SetActorTickEnabled` (`self.Active`))
  (bind _outactors (`GameplayStatics.GetAllActorsOfClass` "/Game/Blueprints/Player/NewWalker.NewWalker_C"))
  (set `self.All Players` _outactors)
  (set `self.Player` (`KismetArrayLibrary.Array_Random` _outactors))
  (bind _asenemy_health (cast `/Game/Widgets/Enemy_Health` (`WidgetComponent.GetUserWidgetObject` (`self.Display`))))
  (bind _output_get (set `self.Health Bar` _asenemy_health))
  (set `/Game/Widgets/Enemy_Health.MaxHealth` _health _output_get)
  (set `/Game/Widgets/Enemy_Health.DisplayHealth` _health _output_get)
  (set `/Game/Widgets/Enemy_Health.Enemy_Name` "Super Heavy Tank" _output_get)
  (`self.Health Visibility`))

(event `Fire Minigun`
  (params (delta :type "Float (double-precision)")))

(event `self.ReceiveTick`
  (params (DeltaSeconds :type "Float (single-precision)"))
  (bind _returnvalue (`self.K2_GetActorRotation`))
  (bind _gun_pivot (`self.Gun Pivot`))
  (bind _returnvalue_2 (`SceneComponent.K2_GetComponentLocation` (`/Game/Blueprints/Player/NewWalker.Box` (`self.Player`))))
  (bind (_returnvalue_roll _returnvalue_pitch) (`KismetMathLibrary.BreakRotator` (`KismetMathLibrary.FindLookAtRotation` (`SceneComponent.K2_GetComponentLocation` _gun_pivot) _returnvalue_2)))
  (`/Engine/EditorBlueprintResources/StandardMacros.IsValid` (`self.Player`)
    (:`Is Valid`
      (`self.Health Visibility`)
      (if (<= (`KismetMathLibrary.Vector_Distance` _returnvalue_2 (`self.K2_GetActorLocation`)) 15000.0)
        (`SceneComponent.K2_SetRelativeRotation` (`self.Tank Body`) (`KismetMathLibrary.RLerp` _returnvalue (`KismetMathLibrary.MakeRotator` (.roll _returnvalue) (.pitch _returnvalue) (`KismetMathLibrary.SelectFloat` (.yaw (`KismetMathLibrary.FindLookAtRotation` (`SceneComponent.K2_GetComponentLocation` (`self.Tank Body`)) (`SceneComponent.K2_GetComponentLocation` (`/Game/Blueprints/Player/NewWalker.Box` (`self.Player`))))) 0.0 true)) 0.001 true) false false)
        (`SceneComponent.K2_SetRelativeRotation` _gun_pivot (`KismetMathLibrary.MakeRotator` (.roll (`SceneComponent.RelativeRotation` _gun_pivot)) (`KismetMathLibrary.ClampAngle` (`KismetMathLibrary.Lerp` (.pitch (`SceneComponent.RelativeRotation` _gun_pivot)) (* _returnvalue_pitch -1.0) 0.005) -50.0 5.0) (.yaw (`SceneComponent.RelativeRotation` _gun_pivot))) false false)
        (`self.Fire Minigun` DeltaSeconds)))))

(event `Take Damage`
  (params (Damage :type "Float (double-precision)"))
  (bind _health (`self.Health`))
  (bind _output_get (set `self.Health` (- _health Damage)))
  (set `/Game/Widgets/Enemy_Health.DisplayHealth` _output_get (`self.Health Bar`))
  (if (<= _health 0.0)
    (`GameplayStatics.SpawnEmitterAtLocation` "/Game/Particles/P_Explosion.P_Explosion" (`SceneComponent.K2_GetComponentLocation` (`self.Tank Body`)) (struct) (20.0 20.0 20.0))
    (`KismetSystemLibrary.Delay` 0.5)
    (`self.K2_DestroyActor`)))

(fn `UserConstructionScript`)
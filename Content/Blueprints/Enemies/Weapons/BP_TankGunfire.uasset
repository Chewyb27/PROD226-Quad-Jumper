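; Enemy tank projectile that homes on a player and explodes on contact.
; BeginPlay points the projectile movement's homing target at the BP_Player nearest the world origin, while Tick tracks time since launch.
; Sphere overlaps count only after three seconds and ignore BP_Missile.
; Drop ships take damage without destroying the projectile; other hits destroy it, with player hits only printing a message, and the SpawnExpired flag goes unread.
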(event `self.ReceiveBeginPlay`
  (bind _outactors (`GameplayStatics.GetAllActorsOfClass` "/Game/Blueprints/Player/BP_Player.BP_Player_C"))
  (bind _asbp_player (cast `/Game/Blueprints/Player/BP_Player` (`.ReturnValue` (`GameplayStatics.FindNearestActor` (0.0 0.0 0.0) _outactors))))
  (set `ProjectileMovementComponent.HomingTargetComponent` (`/Game/Blueprints/Player/BP_Player.Main Component` _asbp_player) (`self.ProjectileMovement`))
  (`KismetSystemLibrary.Delay` 2.0)
  (set `self.Spawn Expired` true))

(event `self.ReceiveTick`
  (params (DeltaSeconds :type "Float (single-precision)"))
  (set `self.Time since launch` (+ (`self.Time since launch`) DeltaSeconds)))

(event `self.Sphere.OnComponentBeginOverlap`
  (params (OverlappedComponent :type "PrimitiveComponent Object Reference") (OtherActor :type "Actor Object Reference") (OtherComp :type "PrimitiveComponent Object Reference") (OtherBodyIndex :type Integer) (bFromSweep :type Boolean) (SweepResult :type "HitResult Structure (by ref)"))
  (bind _returnvalue (`GameplayStatics.GetObjectClass` OtherActor))
  (bind _returnvalue_2 (`SceneComponent.K2_GetComponentLocation` (`self.Sphere`)))
  (if (>= (`self.Time since launch`) 3.0)
    (if (== _returnvalue "/Game/Blueprints/Enemies/Weapons/BP_Missile.BP_Missile_C")
      _
      (elif (== _returnvalue "/Game/Blueprints/Player/BP_Player.BP_Player_C")
        (`GameplayStatics.SpawnEmitterAtLocation` "/Game/Particles/PS_Explosion.PS_Explosion" (`SceneComponent.K2_GetComponentLocation` (`self.Sphere`)) (struct) (5.0 5.0 5.0))
        (`KismetSystemLibrary.PrintString` "Hit Player")
        (`self.K2_DestroyActor`)
        (elif (== _returnvalue "/Game/Blueprints/Enemies/BP_DropShip.BP_DropShip_C")
          (`GameplayStatics.SpawnEmitterAtLocation` "/Game/Particles/PS_Explosion.PS_Explosion" _returnvalue_2 (struct) (5.0 5.0 5.0))
          (bind _asbp_drop_ship (cast `/Game/Blueprints/Enemies/BP_DropShip` OtherActor))
          (`/Game/Blueprints/Enemies/BP_DropShip.Take Damage` _asbp_drop_ship 75.0)
          (else
            (`GameplayStatics.SpawnEmitterAtLocation` "/Game/Particles/PS_Explosion.PS_Explosion" _returnvalue_2 (struct) (5.0 5.0 5.0))
            (`self.K2_DestroyActor`)))))))

(fn `UserConstructionScript`)
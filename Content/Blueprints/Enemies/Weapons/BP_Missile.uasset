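; Enemy homing missile that locks onto a player's box component and shows on the HUD as an enemy with a reticule.
; It registers itself in every Friend's missile list on spawn.
; A sphere overlap and short forward trace feed CheckCollide, which ignores other missiles and a brief launch window, explodes, and damages only players.
; Impact unregisters it, strips its components and delays destruction; drop-ship damage is disconnected.
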(event `self.ReceiveBeginPlay`
  (`SceneComponent.SetVisibility` (`self.Targeted_Reticule`) true false)
  (`/Game/Widgets/WBP_PlayerHUD.Add Enemy` (`/Game/Blueprints/Player/BP_Player.HUD` (`self.Player`)) self false)
  (bind _outactors (`GameplayStatics.GetAllActorsOfClass` "/Game/Blueprints/Player/Weapons/Friend.Friend_C"))
  (set `self.Friends` _outactors)
  (for _array_element _outactors
    (`KismetArrayLibrary.Array_Add` (`/Game/Blueprints/Player/Weapons/Friend.missiles` _array_element) self))
  (bind _outactors_2 (`GameplayStatics.GetAllActorsOfClass` "/Game/Blueprints/Player/BP_Player.BP_Player_C"))
  (bind _asbp_player (cast `/Game/Blueprints/Player/BP_Player` (`.ReturnValue` (`GameplayStatics.FindNearestActor` (0.0 0.0 0.0) _outactors_2))))
  (set `ProjectileMovementComponent.HomingTargetComponent` (`/Game/Blueprints/Player/BP_Player.Main Box Component` _asbp_player) (`self.ProjectileMovement`))
  (`KismetSystemLibrary.Delay` 2.0)
  (set `self.Spawn Expired` true))

(event `self.ReceiveTick`
  (params (DeltaSeconds :type "Float (single-precision)"))
  (bind _missile_v1 (`self.Missile_v1`))
  (bind _returnvalue (`SceneComponent.K2_GetComponentLocation` _missile_v1))
  (set `self.Time since launch` (+ (`self.Time since launch`) DeltaSeconds))
  (if (not (`self.Dead`))
    (bind (_outhit _returnvalue_2) (`KismetSystemLibrary.LineTraceSingle` _returnvalue (+ _returnvalue (* (`SceneComponent.GetForwardVector` _missile_v1) 100.0)) "TraceTypeQuery1" false (`|MakeArray` (`self.Creator`))))
    (if _returnvalue_2
      (`self.CheckCollide` (`.HitActor` (`GameplayStatics.BreakHitResult` _outhit))))))

(event `Impact`
  (set `self.Dead` true)
  (`SceneComponent.SetVisibility` (`self.Targeted_Reticule`) false false)
  (for _array_element (`self.Friends`)
    (`KismetArrayLibrary.Array_RemoveItem` (`/Game/Blueprints/Player/Weapons/Friend.missiles` _array_element) self))
  (`/Engine/EditorBlueprintResources/StandardMacros.DoOnce` false
    (:`Completed`
      (`ActorComponent.Deactivate` (`self.CloudParticle`))
      (`ActorComponent.K2_DestroyComponent` (`self.Sphere`))
      (`ActorComponent.K2_DestroyComponent` (`self.Missile_v1`))
      (`ActorComponent.K2_DestroyComponent` (`self.ProjectileMovement`))
      (`/Game/Widgets/WBP_PlayerHUD.Destroy Enemy` (`/Game/Blueprints/Player/BP_Player.HUD` (`self.Player`)) self)
      (`KismetSystemLibrary.Delay` 10.0)
      (`self.K2_DestroyActor`))))

(event `self.Sphere.OnComponentBeginOverlap`
  (params (OverlappedComponent :type "PrimitiveComponent Object Reference") (OtherActor :type "Actor Object Reference") (OtherComp :type "PrimitiveComponent Object Reference") (OtherBodyIndex :type Integer) (bFromSweep :type Boolean) (SweepResult :type "HitResult Structure (by ref)"))
  (`self.CheckCollide` OtherActor))

(event `CheckCollide`
  (params (Actor :type "Actor Object Reference"))
  (bind _returnvalue (`GameplayStatics.GetObjectClass` Actor))
  (bind _returnvalue_2 (`SceneComponent.K2_GetComponentLocation` (`self.Sphere`)))
  (if (>= (`self.Time since launch`) 0.25)
    (if (== _returnvalue "BP_Missile_C")
      _
      (elif (`KismetMathLibrary.ClassIsChildOf` _returnvalue "/Game/Blueprints/Player/BP_Player.BP_Player_C")
        (`GameplayStatics.SpawnEmitterAtLocation` "/Game/Particles/PS_Explosion.PS_Explosion" (`SceneComponent.K2_GetComponentLocation` (`self.Sphere`)) (struct) (5.0 5.0 5.0))
        (bind _asbp_player (cast `/Game/Blueprints/Player/BP_Player` Actor))
        (`/Game/Blueprints/Player/BP_Player.Health Change` _asbp_player -150.0 true)
        (`self.Impact`)
        (elif (== _returnvalue "/Game/Blueprints/Enemies/BP_DropShip.BP_DropShip_C")
          (`GameplayStatics.SpawnEmitterAtLocation` "/Game/Particles/PS_Explosion.PS_Explosion" _returnvalue_2 (struct) (5.0 5.0 5.0))
          (`self.Impact`)
          (else
            (`GameplayStatics.SpawnEmitterAtLocation` "/Game/Particles/PS_Explosion.PS_Explosion" _returnvalue_2 (struct) (5.0 5.0 5.0))
            (`self.Impact`)))))))

(fn `UserConstructionScript`)
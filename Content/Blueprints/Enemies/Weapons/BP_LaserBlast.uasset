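; Enemy laser projectile with configurable colour, size, speed and damage that sets a player as homing target.
; Tick moves it with swept offsets and line-traces ahead; traces and sphere overlaps feed Hit, which damages players, BP_Australis or ship turrets.
; Australis and scenery hits can add half-damage splash to the nearest player.
; Impact, also triggered after a timeout, spawns an explosion and optional black hole, strips components, then destroys the actor later.
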(event `self.ReceiveBeginPlay`
  (bind _fxs_enemy_blast (`self.FXS_Enemy_Blast`))
  (bind _colour (`self.Colour`))
  (bind _projectilemovement (`self.ProjectileMovement`))
  (bind _speed (`self.Speed`))
  (`SceneComponent.SetVisibility` (`self.FXS_Black_Hole`) (`self.Black Hole Spawner`) false)
  (`FXSystemComponent.SetColorParameter` (`self.FXS_Black_Hole`) "Color" _colour)
  (`FXSystemComponent.SetColorParameter` _fxs_enemy_blast "Color" _colour)
  (`FXSystemComponent.SetVectorParameter` _fxs_enemy_blast "Beam End" (`KismetMathLibrary.MakeVector` (`self.Length`)))
  (`SphereComponent.SetSphereRadius` (`self.Sphere`) (`self.Size`) true)
  (if (`self.Muzzle Flash`)
    (`GameplayStatics.SpawnEmitterAtLocation` (select `bool` (!= (`self.Colour`) (struct :`R` 500.294128 :`G` 164.759048 :`A` 1.0)) :`false` "/Game/Particles/PS_Explosion.PS_Explosion" :`true` "/Game/Particles/PS_Explosion2.PS_Explosion2" :!type "ParticleSystem Object Reference") (`self.K2_GetActorLocation`) (struct) (* (1.0 1.0 1.0) (/ (`self.Size`) 10.0))))
  (`FXSystemComponent.SetFloatParameter` (`self.FXS_Enemy_Blast`) "Scale Curve_Beam Width" (`self.Size`))
  (set `ProjectileMovementComponent.InitialSpeed` _speed _projectilemovement)
  (set `ProjectileMovementComponent.MaxSpeed` _speed _projectilemovement)
  (bind _outactors (`GameplayStatics.GetAllActorsOfClass` "/Game/Blueprints/Player/BP_Player.BP_Player_C"))
  (bind _asbp_player (cast `/Game/Blueprints/Player/BP_Player` (`.ReturnValue` (`GameplayStatics.FindNearestActor` (0.0 0.0 0.0) _outactors))))
  (set `ProjectileMovementComponent.HomingTargetComponent` (`/Game/Blueprints/Player/BP_Player.Main Box Component` _asbp_player) (`self.ProjectileMovement`))
  (`KismetSystemLibrary.Delay` 2.0)
  (set `self.Spawn Expired` true))

(event `self.ReceiveTick`
  (params (DeltaSeconds :type "Float (single-precision)"))
  (bind _time_since_launch (`self.Time since launch`))
  (bind _tick_reducer (`self.Tick Reducer`))
  (bind _time_since_launch_2 (`self.Time since launch`))
  (bind _sphere (`self.Sphere`))
  (bind _returnvalue (`SceneComponent.K2_GetComponentLocation` _sphere))
  (if (>= _tick_reducer 0.0)
    (`self.K2_AddActorLocalOffset` (* (1.0 0.0 0.0) (`self.Speed`) DeltaSeconds) true true)
    (set `self.Time since launch` (+ _time_since_launch_2 DeltaSeconds))
    (set `self.Tick Reducer` 0.0)
    (if (and (>= _time_since_launch_2 0.0) (not (`self.Dead`)))
      (bind (_outhit _returnvalue_2) (`KismetSystemLibrary.LineTraceSingle` _returnvalue (+ _returnvalue (* (`SceneComponent.GetForwardVector` _sphere) 50.0)) "TraceTypeQuery1" true))
      (if _returnvalue_2
        (if (>= _time_since_launch 0.1)
          (`self.Hit` null (`.HitComponent` (`GameplayStatics.BreakHitResult` _outhit))))
        (elif (>= _time_since_launch 10.0)
          (`self.Impact`))))
    (else
      (set `self.Tick Reducer` (+ _tick_reducer DeltaSeconds)))))

(event `Hit`
  (params (Actor :type "Actor Object Reference") (Comp :type "PrimitiveComponent Object Reference"))
  (bind _returnvalue (`GameplayStatics.GetObjectClass` Actor))
  (bind _returnvalue_2 (`PrimitiveComponent.GetCollisionObjectType` Comp))
  (bind _area_of_effect (`self.Area of Effect`))
  (bind _sphere (`self.Sphere`))
  (bind _returnvalue_3 (`SceneComponent.K2_GetComponentLocation` (`self.Sphere`)))
  (bind _returnvalue_4 (* (1.0 1.0 1.0) (/ (`self.Size`) 10.0)))
  (bind _returnvalue_5 (select `bool` (!= (`self.Colour`) (struct :`R` 500.294128 :`G` 164.759048 :`A` 1.0)) :`false` "/Game/Particles/PS_Explosion.PS_Explosion" :`true` "/Game/Particles/PS_Explosion2.PS_Explosion2" :!type "ParticleSystem Object Reference"))
  (bind _returnvalue_6 (+ (`SceneComponent.K2_GetComponentLocation` _sphere) (* (`SceneComponent.GetForwardVector` _sphere) -100.0)))
  (if (>= (`self.Time since launch`) 0.001)
    (if (not (== _returnvalue "/Game/Blueprints/Enemies/Weapons/BP_Missile.BP_Missile_C"))
      (`ActorComponent.Deactivate` (`self.ProjectileMovement`))
      (if (`KismetMathLibrary.ClassIsChildOf` _returnvalue "/Game/Blueprints/Player/BP_Player.BP_Player_C")
        (`GameplayStatics.SpawnEmitterAtLocation` _returnvalue_5 _returnvalue_6 (struct) _returnvalue_4)
        (bind _asbp_player (cast `/Game/Blueprints/Player/BP_Player` Actor))
        (`/Engine/EditorBlueprintResources/StandardMacros.DoOnce` false
          (:`Completed`
            (`/Game/Blueprints/Player/BP_Player.Health Change` _asbp_player (* (`self.Damage`) -1.0) true)
            (`self.Impact`)))
        (elif (== _returnvalue "/Game/Blueprints/Scene/BP_Australis.BP_Australis_C")
          (bind _asbp_australis (cast `/Game/Blueprints/Scene/BP_Australis` Actor))
          (`/Engine/EditorBlueprintResources/StandardMacros.DoOnce` false
            (:`Completed`
              (`/Game/Blueprints/Scene/BP_Australis.Damage` _asbp_australis (`self.Damage`))
              (`GameplayStatics.SpawnEmitterAtLocation` _returnvalue_5 _returnvalue_6 (struct) _returnvalue_4 :!label _label)
              (if (> _area_of_effect 0.0)
                (bind _asbp_player_2 (cast `/Game/Blueprints/Player/BP_Player` (`.ReturnValue` (`GameplayStatics.FindNearestActor` _returnvalue_3 (`self.Player Reference`)))))
                (`/Engine/EditorBlueprintResources/StandardMacros.IsValid` _asbp_player_2
                  (:`Is Valid`
                    (`GameplayStatics.SpawnEmitterAtLocation` _returnvalue_5 _returnvalue_3 (struct) (`KismetMathLibrary.Conv_DoubleToVector` (* _area_of_effect 0.01)) true "AutoRelease")
                    (if (< (`KismetMathLibrary.Vector_Distance` (`SceneComponent.K2_GetComponentLocation` (`/Game/Blueprints/Player/BP_Player.Main Box Component` _asbp_player_2)) _returnvalue_3) _area_of_effect)
                      (`/Game/Blueprints/Player/BP_Player.Health Change` _asbp_player_2 (* (`self.Damage`) -0.5) true)))
                  (:`Is Not Valid`
                    _)))
              (`self.Impact`)))
          (elif (== _returnvalue "/Game/Blueprints/Enemies/Faction_1/BP_DropShip.BP_DropShip_C")
            (if (or (`|EnumEquality` _returnvalue_2 "ECC_WorldDynamic") (`|EnumEquality` _returnvalue_2 "ECC_WorldStatic")) :!label _label_2
              (goto _label)
              (else
                (`KismetSystemLibrary.PrintString` "Hello")))
            (elif (== _returnvalue "/Game/Blueprints/Enemies/Faction_1/BP_ShipTurret.BP_ShipTurret_C")
              (bind _asenemy (cast `/Game/Blueprints/Enemies/Enemy` Actor))
              (`/Game/Blueprints/Enemies/Enemy.Take Damage` _asenemy (* (`self.Damage`) 10.0) false null)
              (else
                (goto _label_2)))))))))

(event `Impact`
  (bind _sphere (`self.Sphere`))
  (`/Engine/EditorBlueprintResources/StandardMacros.IsValid` (`self.Sphere`)
    (:`Is Valid`
      (`GameplayStatics.SpawnEmitterAtLocation` (select `bool` (!= (`self.Colour`) (struct :`R` 500.294128 :`G` 164.759048 :`A` 1.0)) :`false` "/Game/Particles/PS_Explosion.PS_Explosion" :`true` "/Game/Particles/PS_Explosion2.PS_Explosion2" :!type "ParticleSystem Object Reference") (+ (`SceneComponent.K2_GetComponentLocation` _sphere) (* (`SceneComponent.GetForwardVector` _sphere) -100.0)) (struct) (* (1.0 1.0 1.0) (/ (`self.Size`) 10.0))))
    (:`Is Not Valid`
      _))
  (set `self.Dead` true)
  (if (`self.Black Hole Spawner`)
    (`|SpawnActorFromClass` "/Game/Blueprints/Enemies/Weapons/Black_Hole_enemy.Black_Hole_enemy_C" (`KismetMathLibrary.MakeTransform` (.location (`SceneComponent.K2_GetComponentToWorld` (`self.Sphere`))) (.rotation (`SceneComponent.K2_GetComponentToWorld` (`self.Sphere`)))) "Undefined" "OverrideRootScale" null (`self.Player Reference`) (`self.Colour`) 10.0 null))
  (`ActorComponent.K2_DestroyComponent` (`self.Sphere`))
  (`ActorComponent.K2_DestroyComponent` (`self.FXS_Enemy_Blast`))
  (`ActorComponent.K2_DestroyComponent` (`self.ProjectileMovement`))
  (`ActorComponent.K2_DestroyComponent` (`self.FXS_Black_Hole`))
  (`KismetSystemLibrary.Delay` 10.0)
  (`self.K2_DestroyActor`))

(event `self.Sphere.OnComponentBeginOverlap`
  (params (OverlappedComponent :type "PrimitiveComponent Object Reference") (OtherActor :type "Actor Object Reference") (OtherComp :type "PrimitiveComponent Object Reference") (OtherBodyIndex :type Integer) (bFromSweep :type Boolean) (SweepResult :type "HitResult Structure (by ref)"))
  (`self.Hit` OtherActor OtherComp))

(fn `UserConstructionScript`)
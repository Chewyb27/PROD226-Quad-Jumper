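; Fighter is an enemy ship built on a parent enemy Blueprint, with a body mesh and four ship turrets registered as sub-enemies on BeginPlay.
; Tick runs the parent logic and, once the enemy is no longer alive, fires a one-time death sequence that clears the player's targeting of it.
; The death sequence updates the HUD, checks the win state, spawns two staggered large explosions at the body, then destroys the actor.
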(event `self.ReceiveBeginPlay`
  (bind _sub_enemies (`self.Sub Enemies`))
  (set `self.Enemy Body` (`self.Body`))
  (`KismetArrayLibrary.Array_Add` _sub_enemies (`self.BP_ShipTurret`))
  (`KismetArrayLibrary.Array_Add` _sub_enemies (`self.BP_ShipTurret1`))
  (`KismetArrayLibrary.Array_Add` _sub_enemies (`self.BP_ShipTurret3`))
  (`KismetArrayLibrary.Array_Add` _sub_enemies (`self.BP_ShipTurret2`)))

(event `self.ReceiveTick`
  (params (DeltaSeconds :type "Float (single-precision)"))
  (bind _playerreference (`self.PlayerReference`))
  (`parent.ReceiveTick` DeltaSeconds)
  (if (not (`self.EnemyAlive`))
    (`/Engine/EditorBlueprintResources/StandardMacros.DoOnce` false
      (:`Completed`
        (set `/Game/Blueprints/Player/BP_Player.Enemy Targeting` false _playerreference)
        (`KismetArrayLibrary.Array_RemoveItem` (`/Game/Blueprints/Player/BP_Player.Enemy Targeting Count` _playerreference) self)
        (`self.Death Animation`)))))

(event `Death Animation`
  (bind _returnvalue (`SceneComponent.K2_GetComponentLocation` (`self.Body`)))
  (`/Game/Widgets/WBP_PlayerHUD.Destroy Enemy` (`/Game/Blueprints/Player/BP_Player.HUD` (`self.PlayerReference`)) self)
  (`/Game/Blueprints/Player/BP_Player.Check Win State` (`self.PlayerReference`) false)
  (`GameplayStatics.SpawnEmitterAtLocation` "/Game/Particles/PS_Explosion.PS_Explosion" _returnvalue (struct) (10.0 10.0 10.0))
  (`KismetSystemLibrary.Delay` 0.1)
  (`GameplayStatics.SpawnEmitterAtLocation` "/Game/Particles/PS_Explosion.PS_Explosion" _returnvalue (struct) (10.0 10.0 10.0))
  (`/Engine/EditorBlueprintResources/StandardMacros.DoOnce` false
    (:`Completed`
      (`self.K2_DestroyActor`))))

(fn `UserConstructionScript`
  (`parent.UserConstructionScript`))
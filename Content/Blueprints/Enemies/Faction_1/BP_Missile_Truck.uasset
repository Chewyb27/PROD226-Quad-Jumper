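; Missile truck enemy that tracks the nearest player with a rotating pod and fires missiles at them.
; While alive with a player nearby, Tick smoothly turns the pod's yaw and pitch, skipping stealthed or distant players.
; A visibility trace sets the player's targeted flag and gates spawning BP_Missile on a cooldown.
; On death it clears targeting, updates each player's HUD and win state, then explodes and destroys itself.
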(event `self.ReceiveBeginPlay`
  (set `self.Grounded` true)
  (set `self.Enemy Body` (`self.Truck Body`)))

(event `Pod Aiming`
  (params (Delta :type "Float (double-precision)"))
  (bind _pod_rotator (`self.Pod Rotator`))
  (bind _asbp_player (cast `/Game/Blueprints/Player/BP_Player` (`.ReturnValue` (`GameplayStatics.FindNearestActor` (0.0 0.0 0.0) (`self.PlayerReference`)))))
  (bind _returnvalue (`SceneComponent.K2_GetComponentLocation` (`/Game/Blueprints/Player/BP_Player.Main Box Component` _asbp_player)))
  (if (and (<= (`/Game/Blueprints/Player/BP_Player.Stealth Time` _asbp_player) 2.0) (<= (`KismetMathLibrary.Vector_Distance` _returnvalue (`SceneComponent.K2_GetComponentLocation` (`self.Truck Body`))) 20000.0))
    (bind _returnvalue_2 (`KismetMathLibrary.FindLookAtRotation` (`SceneComponent.K2_GetComponentLocation` _pod_rotator) _returnvalue))
    (bind _yaw (.yaw (`KismetMathLibrary.RInterpTo` (`SceneComponent.K2_GetComponentRotation` _pod_rotator) _returnvalue_2 Delta 1.0)))
    (`SceneComponent.K2_SetWorldRotation` _pod_rotator (`KismetMathLibrary.MakeRotator` 0.0 0.0 _yaw) false false)
    (`SceneComponent.K2_SetWorldRotation` (`self.Pod Pitcher`) (`KismetMathLibrary.MakeRotator` 0.0 (.pitch (`KismetMathLibrary.RInterpTo` (`SceneComponent.K2_GetComponentRotation` (`self.Pod Pitcher`)) _returnvalue_2 Delta 1.0)) _yaw) false false)))

(event `self.ReceiveTick`
  (params (DeltaSeconds :type "Float (single-precision)"))
  (bind _playerreference (`self.PlayerReference`))
  (set `self.Timeline Tick` (+ DeltaSeconds (`self.Timeline Tick`)))
  (if (`KismetArrayLibrary.Array_IsNotEmpty` _playerreference)
    (if (`self.EnemyAlive`)
      (if (<= (`GameplayStatics.FindNearestActor` (`SceneComponent.K2_GetComponentLocation` (`self.Enemy Body`)) _playerreference) 35000.0)
        (`self.Enemy Health Visibility`)
        (if (`KismetArrayLibrary.Array_IsNotEmpty` (`self.PlayerReference`))
          (`self.Pod Aiming` DeltaSeconds)
          (`self.Pod Targeting` DeltaSeconds)
          (if (<= (`self.Firing Delay`) 0.0)
            (if (and (`self.Can Fire`) (<= (`GameplayStatics.FindNearestActor` (`SceneComponent.K2_GetComponentLocation` (`self.Truck Body`)) (`self.PlayerReference`)) 15000.0) (<= (`/Game/Blueprints/Player/BP_Player.Stealth Time` (stale `Pod Targeting` _asbp_player)) 2.0))
              (set `self.Firing Delay` 10.0)
              (`|SpawnActorFromClass` "/Game/Blueprints/Enemies/Weapons/BP_Missile.BP_Missile_C" (`KismetMathLibrary.MakeTransform` (.location (`SceneComponent.K2_GetComponentToWorld` (`self.Launcher`))) (.rotation (`SceneComponent.K2_GetComponentToWorld` (`self.Launcher`))) (0.3 0.3 0.3)) "AlwaysSpawn" "OverrideRootScale" null (stale `Pod Targeting` _asbp_player) self null))
            (else
              (set `self.Firing Delay` (`KismetMathLibrary.FClamp` (- (`self.Firing Delay`) DeltaSeconds) 0.0 100.0))))))
      (else
        (`/Engine/EditorBlueprintResources/StandardMacros.DoOnce` false
          (:`Completed`
            (for _array_element (`self.PlayerReference`)
              (bind _enemy_targeting_count (`/Game/Blueprints/Player/BP_Player.Enemy Targeting Count` _array_element))
              (`KismetArrayLibrary.Array_RemoveItem` _enemy_targeting_count self)
              (if (`KismetArrayLibrary.Array_IsEmpty` _enemy_targeting_count)
                (set `/Game/Blueprints/Player/BP_Player.Enemy Targeting` false _array_element)))
            (`self.Death Animation`)))))))

(event `Pod Targeting`
  (params (Delta :type "Float (double-precision)"))
  (bind _returnvalue (`SceneComponent.K2_GetComponentLocation` (`self.Truck Body`)))
  (bind _asbp_player (cast `/Game/Blueprints/Player/BP_Player` (`.ReturnValue` (`GameplayStatics.FindNearestActor` (`SceneComponent.K2_GetComponentLocation` (`self.Truck Body`)) (`self.PlayerReference`)))))
  (bind _returnvalue_2 (`SceneComponent.K2_GetComponentLocation` (`/Game/Blueprints/Player/BP_Player.Main Box Component` _asbp_player)))
  (if (and (<= (`KismetMathLibrary.Vector_Distance` _returnvalue_2 _returnvalue) 20000.0) (<= (`/Game/Blueprints/Player/BP_Player.Stealth Time` _asbp_player) 2.0))
    (bind (_outhit _returnvalue_3) (`KismetSystemLibrary.LineTraceSingle` _returnvalue _returnvalue_2 "TraceTypeQuery1" false (`|MakeArray` _asbp_player :!type "Actor Object Reference")))
    (bind _returnvalue_4 (not _returnvalue_3))
    (set `self.Can Fire` _returnvalue_4)
    (if _returnvalue_4
      (set `/Game/Blueprints/Player/BP_Player.Enemy Targeting` true _asbp_player)
      (`KismetArrayLibrary.Array_Add` (`/Game/Blueprints/Player/BP_Player.Enemy Targeting Count` _asbp_player) self)
      (else
        (set `/Game/Blueprints/Player/BP_Player.Enemy Targeting` false _asbp_player :!label _label)
        (`KismetArrayLibrary.Array_RemoveItem` (`/Game/Blueprints/Player/BP_Player.Enemy Targeting Count` _asbp_player) self)))
    (else
      (goto _label))))

(event `Death Animation`
  (bind _returnvalue (`SceneComponent.K2_GetComponentLocation` (`self.Truck Body`)))
  (for _array_element (`self.PlayerReference`)
    (`/Game/Widgets/WBP_PlayerHUD.Destroy Enemy` (`/Game/Blueprints/Player/BP_Player.HUD` _array_element) self)
    (`/Game/Blueprints/Player/BP_Player.Check Win State` _array_element false))
  (`GameplayStatics.SpawnEmitterAtLocation` "/Game/Particles/PS_Explosion.PS_Explosion" _returnvalue (struct) (10.0 10.0 10.0))
  (`KismetSystemLibrary.Delay` 0.1)
  (`GameplayStatics.SpawnEmitterAtLocation` "/Game/Particles/PS_Explosion.PS_Explosion" _returnvalue (struct) (10.0 10.0 10.0))
  (`/Engine/EditorBlueprintResources/StandardMacros.DoOnce` false
    (:`Completed`
      (`self.K2_DestroyActor`))))

(fn `UserConstructionScript`)
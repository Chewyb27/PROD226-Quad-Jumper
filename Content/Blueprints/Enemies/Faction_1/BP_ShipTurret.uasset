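; Enemy ship turret that tracks the nearest BP_Australis ship, or the player once no ships remain.
; Tick drives interpolated yaw/pitch aiming and targeting, which gates fire on range, stealth, line of sight and barrel alignment.
; It cycles barrels to fire missiles, laser blasts or a timed capsule-traced beam that damages players.
; On death it notifies players, then destroys itself if a child actor, otherwise explodes and powers down.
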(event `Weapon Aiming`
  (params (Delta :type "Float (double-precision)"))
  (bind _returnvalue (`self.GetTransform`))
  (bind _returnvalue_2 (`self.GetTransform`))
  (bind _playerreference (`self.PlayerReference`))
  (bind _gun_pivot (`self.Gun Pivot`))
  (bind _turret_body (`self.Turret Body`))
  (bind _rotation_speed (`self.Rotation Speed`))
  (bind (_distance _returnvalue_3) (`GameplayStatics.FindNearestActor` (0.0 0.0 0.0) _playerreference))
  (bind _returnvalue_4 (`self.K2_GetActorLocation` (`self.Ship Target`)))
  (bind _relativerotation (`SceneComponent.RelativeRotation` _turret_body))
  (bind _relativerotation_2 (`SceneComponent.RelativeRotation` (`self.Gun Pivot`)))
  (if (`KismetArrayLibrary.Array_IsNotEmpty` _playerreference)
    (bind _asbp_player (cast `/Game/Blueprints/Player/BP_Player` _returnvalue_3))
    (bind _main_box_component (`/Game/Blueprints/Player/BP_Player.Main Box Component` _asbp_player))
    (bind _returnvalue_5 (`PrimitiveComponent.GetPhysicsLinearVelocity` _main_box_component "None"))
    (if (`self.No Ships Remaining`)
      (if (<= _distance 35000.0)
        (if (`self.Can Fire`)
          _
          (else
            _))
        (bind _returnvalue_6 (+ (`SceneComponent.K2_GetComponentLocation` _main_box_component) (0.0 0.0 0.0)))
        (`SceneComponent.K2_SetRelativeRotation` _turret_body (`KismetMathLibrary.MakeRotator` 0.0 0.0 (.yaw (`KismetMathLibrary.RInterpTo` _relativerotation (`KismetMathLibrary.FindLookAtRotation` (`KismetMathLibrary.InverseTransformDirection` _returnvalue_2 (`SceneComponent.K2_GetComponentLocation` _turret_body)) (`KismetMathLibrary.InverseTransformDirection` _returnvalue_2 (+ _returnvalue_6 (/ _returnvalue_5 (`self.Projectile Speed`))))) Delta _rotation_speed))) false false)
        (`SceneComponent.K2_SetRelativeRotation` _gun_pivot (`KismetMathLibrary.MakeRotator` 0.0 (`KismetMathLibrary.ClampAngle` (.pitch (`KismetMathLibrary.RInterpTo` _relativerotation_2 (`KismetMathLibrary.FindLookAtRotation` (`KismetMathLibrary.InverseTransformDirection` _returnvalue_2 (`SceneComponent.K2_GetComponentLocation` (`self.Gun Pivot`))) (`KismetMathLibrary.InverseTransformDirection` _returnvalue_2 _returnvalue_6)) Delta _rotation_speed)) -20.0 100.0)) false false))
      (elif (not (`self.Targeting Player`))
        (if (<= (`KismetMathLibrary.Vector_Distance` _returnvalue_6 (`SceneComponent.K2_GetComponentLocation` (`self.Turret Body`))) 20000.0)
          _
          (else
            _))
        (if (`self.Can Fire`) :!label _label
          _
          (else
            _))
        (`SceneComponent.K2_SetRelativeRotation` _turret_body (`KismetMathLibrary.MakeRotator` 0.0 0.0 (.yaw (`KismetMathLibrary.RInterpTo` _relativerotation (`KismetMathLibrary.FindLookAtRotation` (`KismetMathLibrary.InverseTransformDirection` _returnvalue (`SceneComponent.K2_GetComponentLocation` (`self.Turret Body`))) (`KismetMathLibrary.InverseTransformDirection` _returnvalue _returnvalue_4)) Delta 2.0))) false false)
        (`SceneComponent.K2_SetRelativeRotation` _gun_pivot (`KismetMathLibrary.MakeRotator` 0.0 (`KismetMathLibrary.ClampAngle` (.pitch (`KismetMathLibrary.RInterpTo` _relativerotation_2 (`KismetMathLibrary.FindLookAtRotation` (`KismetMathLibrary.InverseTransformDirection` _returnvalue (`SceneComponent.K2_GetComponentLocation` (`self.Gun Pivot`))) (`KismetMathLibrary.InverseTransformDirection` _returnvalue _returnvalue_4)) Delta (`self.Rotation Speed`))) (`self.Min Angle Degrees`) (`self.Max Angle Degrees`))) false false)))
    (else
      (goto _label))))

(event `self.ReceiveBeginPlay`
  (bind _bulletspawn (`self.BulletSpawn`))
  (`parent.ReceiveBeginPlay`)
  (`KismetArrayLibrary.Array_Add` (`self.Bullet Spawn Pos`) _bulletspawn)
  (set `self.Selected Barrel` _bulletspawn)
  (set `self.Grounded` true)
  (set `self.Enemy Body` (`self.Turret Body`))
  (set `self.Firing Delay` (`KismetMathLibrary.RandomFloatInRange` 0.0 5.0))
  (`self.Find Enemy`)
  (`self.SetActorEnableCollision` (or (not (`self.IsChildActor`)) (`self.Targetable Sub Enemy`))))

(event `Find Enemy`
  (bind _allships (`self.Allships`))
  (bind _returnvalue (`SceneComponent.K2_GetComponentLocation` (`self.SM_Artillery_Base`)))
  (bind (_distance _returnvalue_2) (`GameplayStatics.FindNearestActor` _returnvalue _allships))
  (bind _outactors (`GameplayStatics.GetAllActorsOfClass` "/Game/Blueprints/Scene/BP_Australis.BP_Australis_C"))
  (bind _output_get (set `self.Allships` _outactors))
  (if (`KismetArrayLibrary.Array_IsEmpty` _output_get)
    (set `self.No Ships Remaining` true)
    (else
      (for _ _output_get
        (bind (_outhit _returnvalue_3) (`KismetSystemLibrary.LineTraceSingle` _returnvalue (`self.K2_GetActorLocation` _returnvalue_2) "TraceTypeQuery2" false _allships))
        (if _returnvalue_3
          (`KismetArrayLibrary.Array_RemoveItem` _allships _returnvalue_2)
          (else
            (set `self.Ship Target` _returnvalue_2))))
      (set `self.Ship Target` _returnvalue_2))))

(event `self.ReceiveTick`
  (params (DeltaSeconds :type "Float (single-precision)"))
  (bind _returnvalue (`self.GetActorScale3D`))
  (bind _selected_barrel (`self.Selected Barrel`))
  (bind _selected_barrel_2 (`self.Selected Barrel`))
  (bind _projectile_type (`self.Projectile Type`))
  (bind _laserparticle (`self.LaserParticle`))
  (bind _firing_laser (`self.Firing Laser`))
  (bind _playerreference (`self.PlayerReference`))
  (bind _returnvalue_2 (`SceneComponent.K2_GetComponentLocation` (`self.LaserParticle`)))
  (bind _location (.location (`SceneComponent.K2_GetComponentToWorld` _selected_barrel)))
  (bind _rotation (.rotation (`SceneComponent.K2_GetComponentToWorld` _selected_barrel)))
  (bind _returnvalue_3 (+ (* (`SceneComponent.GetForwardVector` _laserparticle) (`self.Laser Range`)) _returnvalue_2))
  (if (`KismetArrayLibrary.Array_IsNotEmpty` _playerreference)
    (`|ExecutionSequence`
      (:`then_0`
        (`self.Enemy Health Visibility`)
        (if (`self.EnemyAlive`)
          (if (`self.Active Turret`)
            (if (<= (`GameplayStatics.FindNearestActor` (`SceneComponent.K2_GetComponentLocation` (`self.Enemy Body`)) _playerreference) 25000.0)
              (`|ExecutionSequence`
                (:`then_0`
                  (`self.Enemy Health Visibility` :!label _label_2))
                (:`then_1`
                  (if (`KismetArrayLibrary.Array_IsNotEmpty` (`self.PlayerReference`))
                    (`/Engine/EditorBlueprintResources/StandardMacros.IsValid` (`self.Ship Target`)
                      (:`Is Valid`
                        (`self.Weapon Aiming` DeltaSeconds :!label _label_3)
                        (`self.Weapon Targeting` DeltaSeconds)
                        (if (<= (`self.Firing Delay`) 0.0)
                          (if (`self.Can Fire`)
                            (set `self.Firing Delay` (`self.Seconds Per Shot`))
                            (set `self.Selected Barrel` (`|GetArrayItem` (`self.Bullet Spawn Pos`) (`self.Barrel Index`)))
                            (if (== _projectile_type "/Game/Blueprints/Player/Weapons/BP_Laser_Arc.BP_Laser_Arc_C")
                              (if true
                                (`SceneComponent.SetVisibility` (`self.LaserParticle`) true false)
                                (set `self.Firing Laser` (`self.Laser Firing Period`))
                                (else
                                  (`self.Spawn Laser Bounce` _location (`SceneComponent.GetForwardVector` _selected_barrel))))
                              (else
                                (bind _asbp_player (cast `/Game/Blueprints/Player/BP_Player` (`.ReturnValue` (`GameplayStatics.FindNearestActor` (`SceneComponent.K2_GetComponentLocation` (`self.Selected Barrel`)) (`self.PlayerReference`)))))
                                (if (== _projectile_type "/Game/Blueprints/Enemies/Weapons/BP_Missile.BP_Missile_C")
                                  (`|SpawnActorFromClass` "/Game/Blueprints/Enemies/Weapons/BP_Missile.BP_Missile_C" (`KismetMathLibrary.MakeTransform` _location _rotation (* _returnvalue 0.3)) "AlwaysSpawn" "OverrideRootScale" null _asbp_player self null)
                                  (bind (_direction _newtrack_0) (`Timeline|Recoil Absorbtion` :!via `PlayFromStart` :!label _label_4)
                                    (:`Update`
                                      (`SceneComponent.K2_SetRelativeLocation` _selected_barrel_2 (+ (* (1.0 0.0 0.0) _newtrack_0 -50.0) (`KismetMathLibrary.MakeVector` 20.0 (.y (`SceneComponent.RelativeLocation` _selected_barrel_2)) (.z (`SceneComponent.RelativeLocation` _selected_barrel_2)))) false false)))
                                  (else
                                    (bind _returnvalue_4 (`|SpawnActorFromClass` "/Game/Blueprints/Enemies/Weapons/BP_LaserBlast.BP_LaserBlast_C" (`KismetMathLibrary.MakeTransform` _location _rotation (* _returnvalue 100.0)) "AlwaysSpawn" "OverrideRootScale" null (`self.Damage`) (`self.Projectile Speed`) (`self.Projectile Size`) (`self.Projectile Length`) (`self.Area Of Effect`) (`self.PlayerReference`) (`self.Colour`) (`self.Muzzle Flash`) (`self.Spawns Black Holes`) null null))
                                    (`GameplayStatics.PlaySoundAtLocation` "/Game/Sounds/EnemyWeapon.EnemyWeapon" _location (struct) (`self.Weapon Volume`) (`self.Weapon Pitch`) 0.0 null null null null)
                                    (goto _label_4 :!via `PlayFromStart`))))))
                          (else
                            (set `self.Firing Delay` (`KismetMathLibrary.FClamp` (- (`self.Firing Delay`) DeltaSeconds) 0.0 100.0)))))
                      (:`Is Not Valid`
                        (if (`self.No Ships Remaining`)
                          (goto _label_3)
                          (else
                            (`self.Find Enemy` :!label _label_5))))))))
              (else
                (`/Engine/EditorBlueprintResources/StandardMacros.IsValid` (`self.Ship Target`) :!label _label_6
                  (:`Is Valid`
                    (if (not (`self.Targeting Player`))
                      (if (>= (`self.time failed tracking`) 5.0)
                        (`self.Find Enemy`)
                        (set `self.time failed tracking` 0.0)
                        (else
                          (goto _label_3)))))
                  (:`Is Not Valid`
                    (if (`self.No Ships Remaining`)
                      (goto _label_2)
                      (else
                        (goto _label_5))))))))
          (else
            (`/Engine/EditorBlueprintResources/StandardMacros.DoOnce` false
              (:`Completed`
                (`self.Death Animation`))))))
      (:`then_1`
        (if (>= _firing_laser 0.0)
          (`|ExecutionSequence`
            (:`then_0`
              (goto _label_7 :!via `Reset`))
            (:`then_1`
              (bind _outhit (`KismetSystemLibrary.CapsuleTraceSingle` _returnvalue_2 _returnvalue_3 100.0 50.0 "TraceTypeQuery1"))
              (bind (_bblockinghit _binitialoverlap _time _distance _location_2 _impactpoint _normal _impactnormal _physmat _hitactor) (`GameplayStatics.BreakHitResult` _outhit))
              (`FXSystemComponent.SetVectorParameter` _laserparticle "Beam End" (`KismetMathLibrary.SelectVector` _returnvalue_3 _location_2 (== _location_2 (0.0 0.0 0.0))))
              (set `self.Firing Laser` (- _firing_laser DeltaSeconds))
              (bind _asbp_player_2 (cast `/Game/Blueprints/Player/BP_Player` _hitactor))
              (`/Game/Blueprints/Player/BP_Player.Health Change` _asbp_player_2 (* -1.0 DeltaSeconds (`self.Laser Damage`)) false)))
          (else
            (`/Engine/EditorBlueprintResources/StandardMacros.DoOnce` false :!label _label_7
              (:`Completed`
                (`/Engine/EditorBlueprintResources/StandardMacros.IsValid` _laserparticle
                  (:`Is Valid`
                    (`SceneComponent.SetVisibility` _laserparticle false false)))))))))
    (else
      (goto _label_6))))

(event `Weapon Targeting`
  (params (Delta :type "Float (double-precision)"))
  (bind _ship_target (`self.Ship Target`))
  (bind _selected_barrel (`self.Selected Barrel`))
  (bind _barrel_index (`self.Barrel Index`))
  (bind _returnvalue (`SceneComponent.K2_GetComponentLocation` (`self.BulletSpawn`)))
  (bind _asbp_player (cast `/Game/Blueprints/Player/BP_Player` (`.ReturnValue` (`GameplayStatics.FindNearestActor` _returnvalue (`self.PlayerReference`)))))
  (`/Engine/EditorBlueprintResources/StandardMacros.IsValid` _asbp_player
    (:`Is Valid`
      (bind _returnvalue_2 (`SceneComponent.K2_GetComponentLocation` (`/Game/Blueprints/Player/BP_Player.Main Box Component` _asbp_player)))
      (bind _returnvalue_3 (and (<= (`/Game/Blueprints/Player/BP_Player.Stealth Time` _asbp_player) 2.0) (<= (`KismetMathLibrary.Vector_Distance` _returnvalue_2 _returnvalue) (`self.Tracking Distance`))))
      (set `self.Targeting Player` _returnvalue_3)
      (if _returnvalue_3
        (set `self.Barrel Index` (`KismetMathLibrary.SelectInt` 0 (+ _barrel_index 1) (== _barrel_index (- (`KismetArrayLibrary.Array_Length` (`self.Bullet Spawn Pos`)) 1))))
        (bind (_outhit _returnvalue_4) (`KismetSystemLibrary.LineTraceSingle` _returnvalue _returnvalue_2 "TraceTypeQuery1" false (`|MakeArray` _asbp_player :!type "Actor Object Reference")))
        (bind _returnvalue_5 (not _returnvalue_4))
        (set `self.Can Fire` (and _returnvalue_5 (>= (`KismetMathLibrary.Dot_VectorVector` (`SceneComponent.GetForwardVector` _selected_barrel) (`KismetMathLibrary.Normal` (- _returnvalue_2 (`SceneComponent.K2_GetComponentLocation` _selected_barrel)))) 0.98)))
        (if (not _returnvalue_5)
          (set `self.Targeting Player` _returnvalue_5))
        (else
          (if (not (`self.No Ships Remaining`)) :!label _label_8
            (`/Engine/EditorBlueprintResources/StandardMacros.IsValid` _ship_target
              (:`Is Valid`
                (bind (_outhit_2 _returnvalue_6) (`KismetSystemLibrary.LineTraceSingle` _returnvalue (`self.K2_GetActorLocation` _ship_target) "TraceTypeQuery2" false (`|MakeArray` _ship_target)))
                (set `self.Can Fire` (not _returnvalue_6))
                (set `self.time failed tracking` (`KismetMathLibrary.SelectFloat` (+ (`self.time failed tracking`) Delta) 0.0 _returnvalue_6)))
              (:`Is Not Valid`
                (set `self.Can Fire` false)))))))
    (:`Is Not Valid`
      (set `self.Targeting Player` false)
      (goto _label_8))))

(event `Death Animation`
  (bind _returnvalue (`SceneComponent.K2_GetComponentLocation` (`self.Turret Body`)))
  (for _array_element (`self.PlayerReference`)
    (`/Game/Widgets/WBP_PlayerHUD.Destroy Enemy` (`/Game/Blueprints/Player/BP_Player.HUD` _array_element) self)
    (`/Game/Blueprints/Player/BP_Player.Check Win State` _array_element false))
  (if (`self.IsChildActor`)
    (`self.K2_DestroyActor`)
    (else
      (`GameplayStatics.SpawnEmitterAtLocation` "/Game/Particles/PS_Explosion.PS_Explosion" _returnvalue (struct) (40.0 40.0 40.0))
      (`KismetSystemLibrary.Delay` 0.1)
      (`GameplayStatics.SpawnEmitterAtLocation` "/Game/Particles/PS_Explosion.PS_Explosion" _returnvalue (struct) (25.0 25.0 25.0))
      (`/Engine/EditorBlueprintResources/StandardMacros.DoOnce` false
        (:`Completed`
          (set `self.EnemyAlive` false)
          (`PrimitiveComponent.SetMaterial` (`self.SM_Artillery_Energy`) 0 "/Game/Materials/GeneralMaterials/M_Black_Padding.M_Black_Padding")
          (`PrimitiveComponent.SetMaterial` (`self.Turret Body`) 0 "/Game/Materials/GeneralMaterials/M_Black_Padding.M_Black_Padding")
          (`self.Remove Lock`)
          (bind (_direction _newtrack_0) (`Timeline|Power Down Turret`)
            (:`Update`
              (`SceneComponent.K2_SetRelativeRotation` (`self.Gun Pivot`) (`KismetMathLibrary.MakeRotator` 0.0 (.pitch (`KismetMathLibrary.RInterpTo` (`SceneComponent.RelativeRotation` (`self.Gun Pivot`)) (struct :`Yaw` -50.0) 1.0 _newtrack_0))) false false))))))))

(event `Spawn Laser Bounce`
  (params (Start :type "Vector Structure") (Direction :type "Vector Structure") (Bounces :type "Float (double-precision)"))
  (if (<= Bounces (`self.Laser Bounces`))
    (bind _outhit (`KismetSystemLibrary.LineTraceSingle` :`Start` Start :`End` (+ (* Direction 80000.0) Start) :`TraceChannel` "TraceTypeQuery1" :`DrawTime` 1.0))
    (bind (_bblockinghit _binitialoverlap _time _distance _location _impactpoint _normal _impactnormal _physmat _hitactor) (`GameplayStatics.BreakHitResult` _outhit))
    (cast `/Game/Blueprints/Player/BP_Player` _hitactor
      (:`then`
        _)
      (:`CastFailed`
        _))
    (bind _returnvalue (`NiagaraFunctionLibrary.SpawnSystemAtLocation` "/Game/Particles/FXS_NewLaser.FXS_NewLaser" Start (struct) (1.0 1.0 1.0) true true "AutoRelease"))
    (`FXSystemComponent.SetColorParameter` _returnvalue "Color" (`self.Colour`))
    (`FXSystemComponent.SetFloatParameter` _returnvalue "Beam Width" 150.0)
    (`FXSystemComponent.SetVectorParameter` _returnvalue "Beam End" _location)
    (`KismetArrayLibrary.Array_Add` (`self.Lasers`) _returnvalue)
    (`self.Spawn Laser Bounce` _location (`KismetMathLibrary.GetReflectionVector` Direction _impactnormal) (+ Bounces 1.0))))

(fn `UserConstructionScript`)
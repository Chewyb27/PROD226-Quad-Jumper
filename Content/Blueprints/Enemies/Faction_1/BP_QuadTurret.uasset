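; BP_QuadTurret is an enemy turret Blueprint for Faction 1 that extends a parent class, to which it leaves its core behavior.
; On BeginPlay it adds three bullet spawn components to the BulletSpawnPos array after the parent's setup.
; Each tick while EnemyAlive is false, it sets the Cylinder mesh's material to black padding, then calls the parent tick.
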(event `self.ReceiveBeginPlay`
  (bind _bullet_spawn_pos (`self.Bullet Spawn Pos`))
  (`parent.ReceiveBeginPlay`)
  (`KismetArrayLibrary.Array_Add` _bullet_spawn_pos (`self.BulletSpawn3`))
  (`KismetArrayLibrary.Array_Add` _bullet_spawn_pos (`self.BulletSpawn1`))
  (`KismetArrayLibrary.Array_Add` _bullet_spawn_pos (`self.BulletSpawn2`)))

(event `self.ReceiveTick`
  (params (DeltaSeconds :type "Float (single-precision)"))
  (if (not (`self.EnemyAlive`))
    (`PrimitiveComponent.SetMaterial` (`self.Cylinder`) 0 "/Game/Materials/GeneralMaterials/M_Black_Padding.M_Black_Padding"))
  (`parent.ReceiveTick` DeltaSeconds))

(fn `UserConstructionScript`
  (`parent.UserConstructionScript`))
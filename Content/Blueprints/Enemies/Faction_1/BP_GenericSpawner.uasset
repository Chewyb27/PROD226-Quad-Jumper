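; BP_GenericSpawner is an enemy spawner that creates drone groups on patrol routes.
; It spawns at BeginPlay if the first wave is enabled, or repeatedly in survival-time mode, sizing groups from its stepped-back timer.
; The first drone appears at the spawner and the rest at random offsets around it, receiving route, convoy offset and player references.
; Each drone then gets the group array as its swarm.
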(event `self.ReceiveBeginPlay`
  (if (`|GetArrayItem` (`self.Spawn on waves`))
    (`self.Spawn Drones` 2 4)))

(event `Spawn Drones`
  (params (`Min Group Size` :type Integer) (`Max Group Size` :type Integer) (Wave :type Integer))
  (bind _drones_of_group (`self.Drones Of Group`))
  (bind _location (.location (`self.GetTransform`)))
  (if (`|GetArrayItem` (`self.Spawn on waves`) Wave)
    _
    (else
      _))
  (`KismetArrayLibrary.Array_Clear` _drones_of_group)
  (bind _outactors (`GameplayStatics.GetAllActorsOfClass` "/Game/Blueprints/Player/BP_Player.BP_Player_C"))
  (for _index (range (+ `Max Group Size` 1))
    (bind _asenemy (castclass `/Game/Blueprints/Enemies/Enemy` (`self.Enemy Class`)))
    (bind _returnvalue (`|SpawnActorFromClass` :`Class` _asenemy :`SpawnTransform` (`KismetMathLibrary.MakeTransform` (`KismetMathLibrary.SelectVector` _location (+ _location (* (`KismetMathLibrary.RandomUnitVector`) 1000.0)) (< _index 1)) (.rotation (`self.GetTransform`)) (1.25 1.25 1.25)) :`CollisionHandlingOverride` "AdjustIfPossibleButAlwaysSpawn" :`TransformScaleMethod` "OverrideRootScale" :`Owner` self :`PlayerReference` _outactors :`Patrol Route Spline` (`self.Patrol Route Spline`) :`Flying Route` (`self.Flying Route`) :`Patrol Speed` 1.5 :`Convoy Offset` (`KismetMathLibrary.Conv_IntToDouble` _index) :`Instigator` (`self.Player`)))
    (`/Game/Blueprints/Enemies/Enemy.Initialize Enemy1` _returnvalue)
    (`/Engine/EditorBlueprintResources/StandardMacros.IsValid` (`self.Player`)
      (:`Is Valid`
        _)
      (:`Is Not Valid`
        _))
    (`KismetArrayLibrary.Array_Add` _drones_of_group))
  (for _array_element (`self.Drones Of Group`)
    (set `/Game/Blueprints/Enemies/Faction_1/BP_Drone.Others in Swarm` (`self.Drones Of Group`) _array_element)))

(event `self.ReceiveTick`
  (params (DeltaSeconds :type "Float (single-precision)"))
  (bind _time (`self.time`))
  (bind _returnvalue (/ _time 60))
  (if (`self.UsesSurvivalTime`)
    (set `self.time` (+ (`self.time`) DeltaSeconds))
    (if (< (`self.TimeForSpawn`) _time)
      (`self.Spawn Drones` (+ _returnvalue 1) (+ _returnvalue 1))
      (set `self.time` (- (`self.time`) (`self.StepBackTime`))))))

(fn `UserConstructionScript`)
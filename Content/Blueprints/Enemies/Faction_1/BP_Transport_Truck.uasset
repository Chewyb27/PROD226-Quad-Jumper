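; Grounded transport truck enemy for Faction 1, built on a parent enemy class that receives the truck body as its EnemyBody.
; Tick updates health visibility while the player is within range and, once the truck dies, clears player targeting and dissolves it.
; DeathAnimation notifies the HUD and win check, spawns explosions and destroys the actor.
; Missile firing and line-of-sight targeting logic is left unconnected, so the truck never attacks.
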(event `self.ReceiveBeginPlay`
  (`parent.ReceiveBeginPlay`)
  (set `self.Grounded` true)
  (set `self.Enemy Body` (`self.Truck Body`)))

(event `self.ReceiveTick`
  (params (DeltaSeconds :type "Float (single-precision)"))
  (bind _playerreference (`self.PlayerReference`))
  (bind _playerreference_2 (`self.PlayerReference`))
  (set `self.Timeline Tick` (+ DeltaSeconds (`self.Timeline Tick`)))
  (`/Engine/EditorBlueprintResources/StandardMacros.IsValid` _playerreference_2
    (:`Is Valid`
      (if (`self.EnemyAlive`)
        (if (<= (`KismetMathLibrary.Vector_Distance` (`SceneComponent.K2_GetComponentLocation` (`self.Enemy Body`)) (`SceneComponent.K2_GetComponentLocation` (`/Game/Blueprints/Player/BP_Player.Main Body` _playerreference_2))) 35000.0)
          (`self.Enemy Health Visibility`)
          (`/Engine/EditorBlueprintResources/StandardMacros.IsValid` (`self.PlayerReference`)))
        (else
          (`/Engine/EditorBlueprintResources/StandardMacros.DoOnce` false
            (:`Completed`
              (set `/Game/Blueprints/Player/BP_Player.Enemy Targeting` false _playerreference)
              (`KismetArrayLibrary.Array_RemoveItem` (`/Game/Blueprints/Player/BP_Player.Enemy Targeting Count` _playerreference) self)
              (`self.Dissolve`))))))))

(event `Pod Targeting`
  (params (Delta :type "Float (double-precision)")))

(event `Death Animation`
  (bind _returnvalue (`SceneComponent.K2_GetComponentLocation` (`self.Truck Body`)))
  (`/Game/Widgets/WBP_PlayerHUD.Destroy Enemy` (`/Game/Blueprints/Player/BP_Player.HUD` (`self.PlayerReference`)) self)
  (`/Game/Blueprints/Player/BP_Player.Check Win State` (`self.PlayerReference`) false)
  (`GameplayStatics.SpawnEmitterAtLocation` "/Game/Particles/PS_Explosion.PS_Explosion" _returnvalue (struct) (10.0 10.0 10.0))
  (`KismetSystemLibrary.Delay` 0.1)
  (`GameplayStatics.SpawnEmitterAtLocation` "/Game/Particles/PS_Explosion.PS_Explosion" _returnvalue (struct) (10.0 10.0 10.0))
  (`/Engine/EditorBlueprintResources/StandardMacros.DoOnce` false
    (:`Completed`
      (`self.K2_DestroyActor`))))

(fn `UserConstructionScript`)
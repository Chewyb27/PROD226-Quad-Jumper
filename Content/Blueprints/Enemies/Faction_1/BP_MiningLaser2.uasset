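; Faction 1 enemy mining laser weapon that alternates between an aiming beam and a damaging beam.
; FireWeapon starts a self-restarting timeline whose value sets beam opacity and selects off, aiming or firing.
; FireLaser traces along a vector that lags behind BulletSpawn's forward direction, sets the active Niagara beam's end, and drains player health only while firing.
; The passed target does not steer the beam.
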(event `Fire Self Event`
  (bind (_direction _newtrack_0) (`Timeline|Timeline_0` :`NewTime` (`KismetMathLibrary.RandomFloatInRange` 0.0 7.0) :!via `PlayFromStart`)
    (:`Update`
      (if (> _newtrack_0 0.0)
        (`self.Fire Laser` (`GameplayStatics.GetWorldDeltaSeconds`) (<= _newtrack_0 0.5) _newtrack_0 (`self.Main Target`))
        (else
          (`self.Stop Firing Laser`))))
    (:`Finished`
      (`self.Fire Self Event`))))

(fn `Fire Laser`
  (params (Delta :type "Float (double-precision)") (`Aiming Mode` :type Boolean) (Opacity :type "Float (double-precision)") (Target :type "Actor Object Reference"))
  (bind _bulletspawn (`self.BulletSpawn`))
  (bind _niagara1 (`self.Niagara1`))
  (bind _returnvalue (`SceneComponent.K2_GetComponentLocation` _bulletspawn))
  (bind _returnvalue_2 (select `bool` `Aiming Mode` :`false` _niagara1 :`true` (`self.Aiming Laser`)))
  (bind _returnvalue_3 (`KismetMathLibrary.VInterpTo_Constant` (`self.Laser Vector`) (`SceneComponent.GetForwardVector` _bulletspawn) Delta 1.0))
  (bind _returnvalue_4 (+ (* _returnvalue_3 15000.0) _returnvalue))
  (set `self.Laser Vector` _returnvalue_3)
  (bind (_outhit _returnvalue_5) (`KismetSystemLibrary.LineTraceSingle` _returnvalue _returnvalue_4 "TraceTypeQuery1"))
  (`SceneComponent.SetVisibility` _niagara1 (not `Aiming Mode`) false)
  (`SceneComponent.SetVisibility` (`self.Aiming Laser`) `Aiming Mode` false)
  (if _returnvalue_5
    (bind (_bblockinghit _binitialoverlap _time _distance _location _impactpoint _normal _impactnormal _physmat _hitactor) (`GameplayStatics.BreakHitResult` _outhit))
    (`NiagaraComponent.SetVariableVec3` _returnvalue_2 "Beam End" _location)
    (bind _asbp_player (cast `/Game/Blueprints/Player/BP_Player` _hitactor)
      (:`then`
        (if (not `Aiming Mode`)
          (`/Game/Blueprints/Player/BP_Player.Health Change` _asbp_player (* -10.0 Delta) false)))
      (:`CastFailed`
        _))
    (else
      (`NiagaraComponent.SetVariableVec3` _returnvalue_2 "Beam End" _returnvalue_4)))
  (`NiagaraComponent.SetVariableFloat` _returnvalue_2 "Opacity" Opacity))

(fn `Fire Weapon`
  (`self.Fire Self Event`))

(fn `Stop Firing Laser`
  (`SceneComponent.SetVisibility` (`self.Aiming Laser`) false false)
  (`SceneComponent.SetVisibility` (`self.Niagara1`) false false))

(fn `UserConstructionScript`
  (`parent.UserConstructionScript`))
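; Grounded laser turret enemy that fires a timed Niagara beam at the player or at its ShipTarget.
; Tick handles range and cooldown, while WeaponTargeting line-traces to prefer a visible, nearby player, falling back to the ship.
; A timeline keeps the beam end on the target; death updates HUD and win state, explodes and powers down.
; Nearest-ship search and projectile spawn are disconnected, so the live graph applies no damage.
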(event `self.ReceiveBeginPlay`
  (bind _niagara (`self.Niagara`))
  (`FXSystemComponent.SetFloatParameter` _niagara "Beam Width" 150.0)
  (`SceneComponent.SetVisibility` _niagara false false)
  (`FXSystemComponent.SetColorParameter` _niagara "Color" (struct :`R` 10.0 :`G` 2.925588 :`A` 1.0))
  (set `self.Grounded` true)
  (set `self.Enemy Body` null)
  (set `self.EnemyName` "Laser Turret")
  (set `self.Firing Delay` (`KismetMathLibrary.RandomFloatInRange` 0.0 5.0)))

(event `self.ReceiveTick`
  (params (DeltaSeconds :type "Float (single-precision)"))
  (bind _playerreference (`self.PlayerReference`))
  (bind _playerreference_2 (`self.PlayerReference`))
  (bind _playerreference_3 (`self.PlayerReference`))
  (bind _niagara (`self.Niagara`))
  (bind _glow_mesh1 (`self.Glow Mesh1`))
  (bind _returnvalue (`self.K2_GetActorLocation` (`self.Ship Target`)))
  (`/Engine/EditorBlueprintResources/StandardMacros.IsValid` _playerreference_3
    (:`Is Valid`
      (`self.Enemy Health Visibility`)
      (if (`self.EnemyAlive`)
        (if (<= (`KismetMathLibrary.Vector_Distance` (`SceneComponent.K2_GetComponentLocation` (`self.SM_Artillery_Base`)) (`SceneComponent.K2_GetComponentLocation` (`/Game/Blueprints/Player/BP_Player.Main Body` _playerreference_3))) 25000.0)
          (`|ExecutionSequence`
            (:`then_0`
              (`/Engine/EditorBlueprintResources/StandardMacros.DoOnce` false :!label _label
                (:`Completed`
                  (set `self.Can Fire` false)
                  (`PrimitiveComponent.SetMaterial` _glow_mesh1 0 "/Game/Materials/GeneralMaterials/M_GeneralBase.M_GeneralBase")
                  (`KismetSystemLibrary.Delay` 2.0)
                  (set `self.Can Fire` true)
                  (`PrimitiveComponent.SetMaterial` _glow_mesh1 0 "/Game/Materials/GeneralMaterials/M_GeneralGlow.M_GeneralGlow"))))
            (:`then_1`
              _))
          (`self.Enemy Health Visibility`)
          (`/Engine/EditorBlueprintResources/StandardMacros.IsValid` (`self.PlayerReference`)
            (:`Is Valid`
              (`/Engine/EditorBlueprintResources/StandardMacros.IsValid` (`self.Ship Target`)
                (:`Is Valid`
                  (`self.Weapon Targeting` DeltaSeconds :!label _label_2)
                  (if (<= (`self.Firing Delay`) 0.0)
                    (if (`self.Can Fire`)
                      (set `self.Firing Delay` 5.0)
                      (`SceneComponent.SetVisibility` _niagara true false)
                      (bind (_direction _newtrack_0) (`Timeline|Recoil Absorbtion` :!via `PlayFromStart`)
                        (:`Update`
                          (`/Engine/EditorBlueprintResources/StandardMacros.IsValid` _playerreference
                            (:`Is Valid`
                              (`FXSystemComponent.SetVectorParameter` _niagara "Beam End" (`KismetMathLibrary.SelectVector` (`SceneComponent.K2_GetComponentLocation` (`/Game/Blueprints/Player/BP_Player.Main Box Component` _playerreference)) _returnvalue (`self.Targeting Player`))))
                            (:`Is Not Valid`
                              (`FXSystemComponent.SetVectorParameter` _niagara "Beam End" _returnvalue))))
                        (:`Finished`
                          (`SceneComponent.SetVisibility` _niagara false false))))
                    (else
                      (set `self.Firing Delay` (`KismetMathLibrary.FClamp` (- (`self.Firing Delay`) DeltaSeconds) 0.0 100.0))))))))
          (else
            (`|ExecutionSequence`
              (:`then_0`
                (goto _label :!via `Reset`))
              (:`then_1`
                (`/Engine/EditorBlueprintResources/StandardMacros.IsValid` (`self.Ship Target`) :!label _label_3
                  (:`Is Valid`
                    (if (not (`self.Targeting Player`))
                      (goto _label_2))))))))
        (else
          (`/Engine/EditorBlueprintResources/StandardMacros.DoOnce` false
            (:`Completed`
              (set `/Game/Blueprints/Player/BP_Player.Enemy Targeting` false _playerreference_2)
              (`KismetArrayLibrary.Array_RemoveItem` (`/Game/Blueprints/Player/BP_Player.Enemy Targeting Count` _playerreference_2) self)
              (`self.Death Animation`))))))
    (:`Is Not Valid`
      (goto _label_3))))

(event `Weapon Targeting`
  (params (Delta :type "Float (double-precision)"))
  (bind _ship_target (`self.Ship Target`))
  (bind _playerreference (`self.PlayerReference`))
  (bind _returnvalue (`SceneComponent.K2_GetComponentLocation` (`self.BulletSpawn`)))
  (bind _returnvalue_2 (`SceneComponent.K2_GetComponentLocation` (`/Game/Blueprints/Player/BP_Player.Main Box Component` _playerreference)))
  (bind _returnvalue_3 (<= (`KismetMathLibrary.Vector_Distance` _returnvalue_2 _returnvalue) 25000.0))
  (`/Engine/EditorBlueprintResources/StandardMacros.IsValid` _playerreference
    (:`Is Valid`
      (set `self.Targeting Player` _returnvalue_3)
      (if _returnvalue_3
        (bind (_outhit _returnvalue_4) (`KismetSystemLibrary.LineTraceSingle` _returnvalue _returnvalue_2 "TraceTypeQuery1" false (`|MakeArray` _playerreference :!type "Actor Object Reference")))
        (bind _returnvalue_5 (not _returnvalue_4))
        (set `self.Can Fire` _returnvalue_5)
        (if (not _returnvalue_5)
          (set `self.Targeting Player` _returnvalue_5)
          (bind (_outhit_2 _returnvalue_6) (`KismetSystemLibrary.LineTraceSingle` _returnvalue (`self.K2_GetActorLocation` _ship_target) "TraceTypeQuery1" false (`|MakeArray` _ship_target) :!label _label_4))
          (set `self.Can Fire` (not _returnvalue_6)))
        (else
          (goto _label_4))))
    (:`Is Not Valid`
      (set `self.Targeting Player` false)
      (goto _label_4))))

(event `Death Animation`
  (bind _returnvalue (`SceneComponent.K2_GetComponentLocation` (`self.BulletSpawn`)))
  (`/Game/Widgets/WBP_PlayerHUD.Destroy Enemy` (`/Game/Blueprints/Player/BP_Player.HUD` (`self.PlayerReference`)) self)
  (`/Game/Blueprints/Player/BP_Player.Check Win State` (`self.PlayerReference`) false)
  (`GameplayStatics.SpawnEmitterAtLocation` "/Game/Particles/PS_Explosion.PS_Explosion" _returnvalue (struct) (10.0 10.0 10.0))
  (`KismetSystemLibrary.Delay` 0.1)
  (`GameplayStatics.SpawnEmitterAtLocation` "/Game/Particles/PS_Explosion.PS_Explosion" _returnvalue (struct) (10.0 10.0 10.0))
  (`/Engine/EditorBlueprintResources/StandardMacros.DoOnce` false
    (:`Completed`
      (set `self.EnemyAlive` false)
      (`PrimitiveComponent.SetMaterial` (`self.Glow Mesh1`) 0 "/Game/Materials/GeneralMaterials/M_Black_Padding.M_Black_Padding")
      (`self.Remove Lock`)
      (`Timeline|Power Down Turret`))))

(fn `UserConstructionScript`)
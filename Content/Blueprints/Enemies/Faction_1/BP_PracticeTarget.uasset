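; Practice target enemy in Faction_1, set up as a grounded target.
; BeginPlay sets the Grounded flag and registers Body as EnemyBody; Tick and DeathAnimation are empty.
; Disconnected logic remains for distance-gated health visibility, targeting cleanup on death, and an explosion sequence with HUD removal and win-state check, but none of it runs.
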(event `self.ReceiveBeginPlay`
  (set `self.Grounded` true)
  (set `self.Enemy Body` (`self.Body`)))

(event `self.ReceiveTick`
  (params (DeltaSeconds :type "Float (single-precision)")))

(event `Death Animation`)

(fn `UserConstructionScript`)
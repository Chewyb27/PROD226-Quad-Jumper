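; Grounded enemy tank that tracks the player with its turret and fires laser blasts.
; Tick drives range-gated aiming and targeting, leading turret yaw by the player's velocity while the gun pitches at their current position.
; A close-range visibility trace sets CanFire and registers the tank as targeting the player, with shots spaced by a cooldown.
; On death it clears targeting, updates HUD and win state, explodes and destroys itself.
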(event `self.ReceiveBeginPlay`
  (set `self.Grounded` true)
  (set `self.Enemy Body` (`self.Tank Body`)))

(event `Weapon Aiming`
  (params (Delta :type "Float (double-precision)"))
  (bind _sm_turret_base1 (`self.SM_Turret_Base1`))
  (bind _main_box_component (`/Game/Blueprints/Player/BP_Player.Main Box Component` (`self.PlayerReference`)))
  (bind _returnvalue (`SceneComponent.K2_GetComponentLocation` _main_box_component))
  (set `self.Timeline Tick` (+ Delta (`self.Timeline Tick`)))
  (if (<= (`KismetMathLibrary.Vector_Distance` _returnvalue (`SceneComponent.K2_GetComponentLocation` (`self.Tank Body`))) 20000.0)
    (bind _returnvalue_2 (`PrimitiveComponent.GetPhysicsLinearVelocity` _main_box_component "None"))
    (bind _yaw (.yaw (`KismetMathLibrary.RInterpTo` (`SceneComponent.K2_GetComponentRotation` _sm_turret_base1) (`KismetMathLibrary.FindLookAtRotation` (`SceneComponent.K2_GetComponentLocation` (`self.Tank Body`)) (+ _returnvalue_2 _returnvalue)) Delta (`self.Interp Speed`))))
    (`SceneComponent.K2_SetWorldRotation` _sm_turret_base1 (`KismetMathLibrary.MakeRotator` 0.0 0.0 _yaw) false false)
    (`SceneComponent.K2_SetWorldRotation` (`self.Gun Pivot`) (`KismetMathLibrary.MakeRotator` 0.0 (.pitch (`KismetMathLibrary.RInterpTo` (`SceneComponent.K2_GetComponentRotation` (`self.Gun Pivot`)) (`KismetMathLibrary.FindLookAtRotation` (`SceneComponent.K2_GetComponentLocation` (`self.Gun Pivot`)) _returnvalue) Delta 3.0)) _yaw) false false)))

(event `self.ReceiveTick`
  (params (DeltaSeconds :type "Float (single-precision)"))
  (bind _playerreference (`self.PlayerReference`))
  (bind _playerreference_2 (`self.PlayerReference`))
  (set `self.Timeline Tick` (+ DeltaSeconds (`self.Timeline Tick`)))
  (`/Engine/EditorBlueprintResources/StandardMacros.IsValid` _playerreference_2
    (:`Is Valid`
      (if (`self.EnemyAlive`)
        (if (<= (`KismetMathLibrary.Vector_Distance` (`SceneComponent.K2_GetComponentLocation` (`self.Enemy Body`)) (`SceneComponent.K2_GetComponentLocation` (`/Game/Blueprints/Player/BP_Player.Main Body` _playerreference_2))) 35000.0)
          (`self.Enemy Health Visibility`)
          (`/Engine/EditorBlueprintResources/StandardMacros.IsValid` (`self.PlayerReference`)
            (:`Is Valid`
              (`self.Weapon Aiming` DeltaSeconds)
              (`self.Weapon Targeting` DeltaSeconds)
              (if (<= (`self.Firing Delay`) 0.0)
                (if (`self.Can Fire`)
                  (set `self.Firing Delay` 2.0)
                  (`|SpawnActorFromClass` "/Game/Blueprints/Enemies/Weapons/BP_LaserBlast.BP_LaserBlast_C" (`KismetMathLibrary.MakeTransform` (.location (`SceneComponent.K2_GetComponentToWorld` (`self.BulletSpawn`))) (.rotation (`SceneComponent.K2_GetComponentToWorld` (`self.BulletSpawn`))) (1.5 1.5 1.5)) "AlwaysSpawn" "OverrideRootScale" null 20.0 25000.0 10.0 200.0 300.0 (`self.PlayerReference`) null))
                (else
                  (set `self.Firing Delay` (`KismetMathLibrary.FClamp` (- (`self.Firing Delay`) DeltaSeconds) 0.0 100.0)))))))
        (else
          (`/Engine/EditorBlueprintResources/StandardMacros.DoOnce` false
            (:`Completed`
              (set `/Game/Blueprints/Player/BP_Player.Enemy Targeting` false _playerreference)
              (`KismetArrayLibrary.Array_RemoveItem` (`/Game/Blueprints/Player/BP_Player.Enemy Targeting Count` _playerreference) self)
              (`self.Death Animation`))))))))

(event `Weapon Targeting`
  (params (Delta :type "Float (double-precision)"))
  (bind _playerreference (`self.PlayerReference`))
  (bind _playerreference_2 (`self.PlayerReference`))
  (bind _playerreference_3 (`self.PlayerReference`))
  (bind _returnvalue (`SceneComponent.K2_GetComponentLocation` (`self.Tank Body`)))
  (bind _returnvalue_2 (`SceneComponent.K2_GetComponentLocation` (`/Game/Blueprints/Player/BP_Player.Main Box Component` _playerreference_3)))
  (if (<= (`KismetMathLibrary.Vector_Distance` _returnvalue_2 _returnvalue) 10000.0)
    (bind (_outhit _returnvalue_3) (`KismetSystemLibrary.LineTraceSingle` _returnvalue _returnvalue_2 "TraceTypeQuery1" false (`|MakeArray` _playerreference_3 :!type "Actor Object Reference")))
    (bind _returnvalue_4 (not _returnvalue_3))
    (set `self.Can Fire` _returnvalue_4)
    (if _returnvalue_4
      (set `/Game/Blueprints/Player/BP_Player.Enemy Targeting` true _playerreference)
      (`KismetArrayLibrary.Array_Add` (`/Game/Blueprints/Player/BP_Player.Enemy Targeting Count` _playerreference) self)
      (else
        (set `/Game/Blueprints/Player/BP_Player.Enemy Targeting` false _playerreference_2 :!label _label)
        (`KismetArrayLibrary.Array_RemoveItem` (`/Game/Blueprints/Player/BP_Player.Enemy Targeting Count` _playerreference_2) self)))
    (else
      (goto _label))))

(event `Death Animation`
  (bind _returnvalue (`SceneComponent.K2_GetComponentLocation` (`self.Tank Body`)))
  (`/Game/Widgets/WBP_PlayerHUD.Destroy Enemy` (`/Game/Blueprints/Player/BP_Player.HUD` (`self.PlayerReference`)) self)
  (`/Game/Blueprints/Player/BP_Player.Check Win State` (`self.PlayerReference`) false)
  (`GameplayStatics.SpawnEmitterAtLocation` "/Game/Particles/PS_Explosion.PS_Explosion" _returnvalue (struct) (10.0 10.0 10.0))
  (`KismetSystemLibrary.Delay` 0.1)
  (`GameplayStatics.SpawnEmitterAtLocation` "/Game/Particles/PS_Explosion.PS_Explosion" _returnvalue (struct) (10.0 10.0 10.0))
  (`/Engine/EditorBlueprintResources/StandardMacros.DoOnce` false
    (:`Completed`
      (`self.K2_DestroyActor`))))

(fn `UserConstructionScript`)
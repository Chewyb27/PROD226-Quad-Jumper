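; Enemy dropship that hovers high above the ground and fires missiles at the player's NewWalker.
; Tick eases it to a traced altitude, yaws and banks it toward the nearby player or a cached tank location, and gimbals the thrusters.
; Five seconds of unbroken line-of-sight targeting launches a missile from alternating pods.
; Damage and collisions drain a distance-shown health bar; death makes it fall, explode and leave the HUD.
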(event `Gimbal Thrust`
  (params (Delta :type "Float (double-precision)"))
  (bind _roll (.roll (`SceneComponent.RelativeRotation` (`self.Main Body`))))
  (bind _pitch (.pitch (`SceneComponent.RelativeRotation` (`self.Main Body`))))
  (bind _returnvalue (* _pitch -0.25))
  (`SceneComponent.K2_SetRelativeRotation` (`self.Right Thruster`) (`KismetMathLibrary.MakeRotator` 0.0 (`KismetMathLibrary.Lerp` (`KismetMathLibrary.ClampAngle` (+ (* _roll 3.0) 70.0 _returnvalue 0.0) -20.0 120.0) _pitch 0.025)) false false)
  (`SceneComponent.K2_SetRelativeRotation` (`self.Left Thruster`) (`KismetMathLibrary.MakeRotator` 0.0 (`KismetMathLibrary.Lerp` (`KismetMathLibrary.ClampAngle` (+ (* _roll -3.0) 70.0 _returnvalue 0.0) -20.0 120.0) _pitch 0.01)) false false))

(event `self.ReceiveBeginPlay`
  (bind _returnvalue (`self.K2_GetActorLocation`))
  (bind _health (`self.Health`))
  (`self.SetActorTickEnabled` (`self.Active`))
  (bind _outactors (`GameplayStatics.GetAllActorsOfClass` "/Game/Blueprints/Player/NewWalker.NewWalker_C"))
  (set `self.All Players` _outactors)
  (set `self.Player` (`KismetArrayLibrary.Array_Random` _outactors))
  (bind _outhit (`KismetSystemLibrary.LineTraceSingle` _returnvalue (+ _returnvalue (* (`KismetMathLibrary.Vector_Down`) 10000.0)) "TraceTypeQuery1"))
  (set `self.Height` (+ (.z (`.Location` (`GameplayStatics.BreakHitResult` _outhit))) (`KismetMathLibrary.RandomFloatInRange` 6000.0 6500.0)))
  (bind _outactors_2 (`GameplayStatics.GetAllActorsOfClass` "/Game/Blueprints/Scene/BuildingV3.BuildingV3_C"))
  (`KismetArrayLibrary.Array_Append` (`self.Nearby Actors`) _outactors_2)
  (bind _outactors_3 (`GameplayStatics.GetAllActorsOfClass` "/Game/Blueprints/Enemies/EnemyTank.EnemyTank_C"))
  (set `self.Nearby Tanks` _outactors_3)
  (bind _asenemy_health (cast `/Game/Widgets/Enemy_Health` (`WidgetComponent.GetUserWidgetObject` (`self.Display`))))
  (bind _output_get (set `self.Health Bar` _asenemy_health))
  (set `/Game/Widgets/Enemy_Health.MaxHealth` _health _output_get)
  (set `/Game/Widgets/Enemy_Health.DisplayHealth` _health _output_get)
  (set `self.Look Location` (`SceneComponent.K2_GetComponentLocation` (`Actor.RootComponent` (`.ReturnValue` (`GameplayStatics.FindNearestActor` (`self.K2_GetActorLocation`) (`self.Nearby Tanks`))))))
  (`self.Health Visibility`)
  (`PrimitiveComponent.SetEnableGravity` (`self.Main Body`) (not (`self.Active`))))

(event `Health Visibility`
  (bind _player (`self.Player`))
  (bind _display (`self.Display`))
  (`/Engine/EditorBlueprintResources/StandardMacros.IsValid` _player
    (:`Is Valid`
      (`SceneComponent.SetVisibility` _display (and (<= (`KismetMathLibrary.Vector_Distance` (`SceneComponent.K2_GetComponentLocation` (`/Game/Blueprints/Player/NewWalker.Main Body` _player)) (`SceneComponent.K2_GetComponentLocation` (`self.Main Body`))) 15000.0) (`self.Active`)) false)
      (`/Engine/EditorBlueprintResources/StandardMacros.DoOnce` false
        (:`Completed`
          (`/Game/Widgets/WalkerHUD.Add Enemy` (`/Game/Blueprints/Player/NewWalker.HUD` _player) self))))
    (:`Is Not Valid`
      (`SceneComponent.SetVisibility` _display false false))))

(event `self.ReceiveTick`
  (params (DeltaSeconds :type "Float (single-precision)"))
  (bind _returnvalue (`KismetMathLibrary.Vector_Up`))
  (bind _targeting_time (`self.Targeting Time`))
  (bind _player (`self.Player`))
  (bind (_returnvalue_roll _returnvalue_pitch _returnvalue_yaw) (`KismetMathLibrary.BreakRotator` (`SceneComponent.K2_GetComponentRotation` (`self.Main Body`))))
  (bind _yaw (.yaw (`KismetMathLibrary.FindLookAtRotation` (`self.K2_GetActorLocation`) (`KismetMathLibrary.SelectVector` (`SceneComponent.K2_GetComponentLocation` (`/Game/Blueprints/Player/NewWalker.Box` (`self.Player`))) (`self.Look Location`) (`self.Player Found`)))))
  (if (`self.Dying`)
    (`PrimitiveComponent.AddVelocityChangeImpulseAtLocation` (`self.Main Body`) (* (`KismetMathLibrary.Vector_Up`) -3.0) (`self.K2_GetActorLocation`) "None")
    (set `/Game/Blueprints/Player/NewWalker.Enemy Targeting` false (`self.Player`) :!label _label)
    (set `self.Targeting Time` 0.0)
    (`KismetArrayLibrary.Array_RemoveItem` (`/Game/Blueprints/Player/NewWalker.Enemy Targeting Count` (`self.Player`)) self)
    (else
      (`/Engine/EditorBlueprintResources/StandardMacros.IsValid` _player
        (:`Is Valid`
          (set `self.Player Found` (and (`KismetSystemLibrary.IsValid` _player) (<= (`KismetMathLibrary.Vector_Distance` (`SceneComponent.K2_GetComponentLocation` (`/Game/Blueprints/Player/NewWalker.Box` _player)) (`SceneComponent.K2_GetComponentLocation` (`self.Main Body`))) 25000.0)))
          (set `self.ChangeInYaw` _yaw)
          (`self.Gimbal Thrust` DeltaSeconds)
          (`self.Health Visibility`)
          (`SceneComponent.K2_SetRelativeRotation` (`self.Main Body`) (`KismetMathLibrary.RInterpTo` (`self.K2_GetActorRotation`) (`KismetMathLibrary.MakeRotator` (`KismetMathLibrary.ClampAngle` (* (- _returnvalue_yaw _yaw) -6.0) -20.0 20.0) 0.0 _yaw) DeltaSeconds 1.0) false false)
          (`self.K2_SetActorLocation` (`KismetMathLibrary.MakeVector` (.x (`self.K2_GetActorLocation`)) (.y (`self.K2_GetActorLocation`)) (`KismetMathLibrary.Lerp` (.z (`self.K2_GetActorLocation`)) (`KismetMathLibrary.SelectFloat` (`self.Height`) 0.0 true) 0.002)) false true)
          (`self.K2_AddActorWorldOffset` (* (+ (* _returnvalue (`KismetMathLibrary.Abs` (.roll (`SceneComponent.RelativeRotation` (`self.Main Body`)))) -1.0) (* _returnvalue (`KismetMathLibrary.Abs` (.pitch (`SceneComponent.RelativeRotation` (`self.Main Body`)))) -1.0)) 0.1))
          (if (`self.Player Found`)
            (`self.Target Player`)
            (if (`self.Player Targeting`)
              (set `self.Targeting Time` (+ _targeting_time DeltaSeconds))
              (if (>= _targeting_time 5.0)
                (set `self.Targeting Time` 0.0)
                (`/Engine/EditorBlueprintResources/StandardMacros.FlipFlop`
                  (:`A`
                    (`|SpawnActorFromClass` "/Game/Blueprints/Enemies/Weapons/Missile.Missile_C" (`SceneComponent.K2_GetComponentToWorld` (`self.Left Missile Pod`)) "AlwaysSpawn" "OverrideRootScale" self null))
                  (:`B`
                    (`|SpawnActorFromClass` "/Game/Blueprints/Enemies/Weapons/Missile.Missile_C" (`SceneComponent.K2_GetComponentToWorld` (`self.Right Missile Pod`)) "AlwaysSpawn" "OverrideRootScale" self null))))
              (else
                (set `self.Targeting Time` 0.0)))
            (else
              (goto _label))))))))

(event `Take Damage`
  (params (Damage :type "Float (double-precision)"))
  (bind _health (`self.Health`))
  (bind _output_get (set `self.Health` (- _health Damage)))
  (set `/Game/Widgets/Enemy_Health.DisplayHealth` _output_get (`self.Health Bar`))
  (if (<= _health 0.0)
    (`self.Death`)))

(event `Target Player`
  (bind _returnvalue (`self.K2_GetActorLocation`))
  (bind _player (`self.Player`))
  (bind _enemy_targeting_count (`/Game/Blueprints/Player/NewWalker.Enemy Targeting Count` _player))
  (bind _returnvalue_2 (`SceneComponent.K2_GetComponentLocation` (`/Game/Blueprints/Player/NewWalker.Box` _player)))
  (`/Engine/EditorBlueprintResources/StandardMacros.IsValid` _player
    (:`Is Valid`
      (if (<= (`KismetMathLibrary.Vector_Distance` _returnvalue _returnvalue_2) 12000.0)
        (bind (_outhit _returnvalue_3) (`KismetSystemLibrary.LineTraceSingle` _returnvalue _returnvalue_2 "TraceTypeQuery1" false (`self.All Players`)))
        (if _returnvalue_3
          (set `/Game/Blueprints/Player/NewWalker.Enemy Targeting` false _player)
          (set `self.Player Targeting` false)
          (`KismetArrayLibrary.Array_RemoveItem` _enemy_targeting_count self :!label _label_2)
          (else
            (set `/Game/Blueprints/Player/NewWalker.Enemy Targeting` true _player)
            (set `self.Player Targeting` true)
            (`KismetArrayLibrary.Array_Add` _enemy_targeting_count self)))
        (else
          (set `/Game/Blueprints/Player/NewWalker.Enemy Targeting` false _player)
          (set `self.Player Targeting` false)
          (goto _label_2))))))

(event `Death`
  (bind _returnvalue (`SceneComponent.K2_GetComponentLocation` (`self.Main Body`)))
  (`PrimitiveComponent.SetEnableGravity` (`self.Main Body`) true)
  (set `self.Dying` true)
  (`KismetArrayLibrary.Array_RemoveItem` (`/Game/Blueprints/Player/NewWalker.Enemy Targeting Count` (`self.Player`)) self)
  (`GameplayStatics.SpawnEmitterAtLocation` "/Game/Particles/P_Explosion.P_Explosion" _returnvalue (struct) (10.0 10.0 10.0))
  (`/Game/Widgets/WalkerHUD.Destroy Enemy` (`/Game/Blueprints/Player/NewWalker.HUD` (`self.Player`)) self)
  (`KismetSystemLibrary.Delay` 2.0)
  (`GameplayStatics.SpawnEmitterAtLocation` "/Game/Particles/P_Explosion.P_Explosion" _returnvalue (struct) (10.0 10.0 10.0))
  (`self.K2_DestroyActor`))

(event `self.Finding Cone.OnComponentBeginOverlap`
  (params (OverlappedComponent :type "PrimitiveComponent Object Reference") (OtherActor :type "Actor Object Reference") (OtherComp :type "PrimitiveComponent Object Reference") (OtherBodyIndex :type Integer) (bFromSweep :type Boolean) (SweepResult :type "HitResult Structure (by ref)"))
  (if (== (`GameplayStatics.GetObjectClass` OtherActor) "/Game/Blueprints/Player/NewWalker.NewWalker_C")
    (bind _asnew_walker (cast `/Game/Blueprints/Player/NewWalker` OtherActor))
    (set `self.Player` _asnew_walker)
    (set `self.Player Found` true)))

(event `self.Finding Cone.OnComponentEndOverlap`
  (params (OverlappedComponent :type "PrimitiveComponent Object Reference") (OtherActor :type "Actor Object Reference") (OtherComp :type "PrimitiveComponent Object Reference") (OtherBodyIndex :type Integer)))

(event `self.Target Cone.OnComponentBeginOverlap`
  (params (OverlappedComponent :type "PrimitiveComponent Object Reference") (OtherActor :type "Actor Object Reference") (OtherComp :type "PrimitiveComponent Object Reference") (OtherBodyIndex :type Integer) (bFromSweep :type Boolean) (SweepResult :type "HitResult Structure (by ref)")))

(event `self.Main Body.OnComponentHit`
  (params (HitComponent :type "PrimitiveComponent Object Reference") (OtherActor :type "Actor Object Reference") (OtherComp :type "PrimitiveComponent Object Reference") (NormalImpulse :type "Vector Structure") (Hit :type "HitResult Structure (by ref)"))
  (bind _returnvalue (`GameplayStatics.GetObjectClass` OtherActor))
  (if (>= (`self.GetGameTimeSinceCreation`) 0.5)
    (if (and (!= OtherActor self) (or (== _returnvalue "DropShip_C") (== _returnvalue "/Game/Blueprints/Scene/Communications_Tower.Communications_Tower_C")))
      (bind _asdrop_ship (cast `/Game/Blueprints/Enemies/DropShip` OtherActor)
        (:`then`
          (if (`/Game/Blueprints/Enemies/DropShip.Active` _asdrop_ship)
            (`self.Take Damage` _asdrop_ship 1000.0)))
        (:`CastFailed`
          (cast `/Game/Blueprints/Scene/Communications_Tower` OtherActor)
          (`self.Take Damage` 1000.0)))
      (elif (`|EnumEquality` (`SceneComponent.Mobility` OtherComp) "Static")
        (`/Engine/EditorBlueprintResources/StandardMacros.DoOnce` false :!label _label_3
          (:`Completed`
            (`self.Take Damage` (* (+ (.x (`KismetMathLibrary.Vector_GetAbs` (`self.GetVelocity`))) (.y (`KismetMathLibrary.Vector_GetAbs` (`self.GetVelocity`))) (.z (`KismetMathLibrary.Vector_GetAbs` (`self.GetVelocity`)))) 0.1))
            (`Timeline|Collide Cooldown` :!via `PlayFromStart`
              (:`Finished`
                (goto _label_3 :!via `Reset`)))))))))

(fn `Pull_Location`
  (params (`World Location` :type "Vector Structure")))

(fn `UserConstructionScript`)
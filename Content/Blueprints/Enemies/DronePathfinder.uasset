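; Drone pathfinder that wanders endlessly between random navigable points in a wide radius around a supplied Owner actor.
; The FindNewLocation event picks a point and sends this object's AI controller there with AIMoveTo, keeping its own current height instead of the point's Z.
; When the move finishes, it pauses briefly and loops to pick another point.
; Nothing in this graph calls the event, and BeginPlay and Tick are empty.
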(event `Find New Location`
  (params (Owner :type "Actor Object Reference"))
  (bind _randomlocation (`NavigationSystemV1.K2_GetRandomLocationInNavigableRadius` (`self.K2_GetActorLocation` Owner) 15000.0 null null :!label _label))
  (set `self.Random Location` _randomlocation)
  (`AITask_MoveTo.AIMoveTo` (`AIBlueprintHelperLibrary.GetAIController` self) (`KismetMathLibrary.MakeVector` (.x _randomlocation) (.y _randomlocation) (.z (`self.K2_GetActorLocation`))) null
    (:`OnMoveFinished`
      (`KismetSystemLibrary.Delay` 3.0)
      (goto _label))))

(event `self.ReceiveTick`
  (params (DeltaSeconds :type "Float (single-precision)")))

(fn `UserConstructionScript`)
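; Coaxial laser enemy weapon that fires a beam at the player, driven externally through FireLaser and StopFiringLaser rather than its own Tick.
; FireLaser aims at the player within a cone around the mesh's up vector, otherwise straight along it, then line-traces while ignoring the passed-in Worm.
; The trace sets the endpoint of either the aiming or firing Niagara beam and drains BP_Player health over time in both modes.
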(event `self.ReceiveBeginPlay`
  (`parent.ReceiveBeginPlay`)
  (set `self.Enemy Body` (`self.StaticMesh`)))

(fn `Fire Laser`
  (params (Delta :type "Float (double-precision)") (`Aiming Mode` :type Boolean) (Opacity :type "Float (double-precision)") (Worm :type "/Game/Blueprints/Enemies/BP_Worm Object Reference") (Player :type "/Game/Blueprints/Player/BP_Player Object Reference"))
  (bind _staticmesh (`self.StaticMesh`))
  (bind _returnvalue (`SceneComponent.K2_GetComponentLocation` _staticmesh))
  (bind _returnvalue_2 (`SceneComponent.GetUpVector` _staticmesh))
  (bind _returnvalue_3 (select `bool` `Aiming Mode` :`false` (`self.Niagara`) :`true` (`self.Aiming Laser`)))
  (bind _returnvalue_4 (`KismetMathLibrary.GetDirectionUnitVector` _returnvalue (`self.K2_GetActorLocation` Player)))
  (bind _returnvalue_5 (`KismetMathLibrary.SelectVector` (`KismetMathLibrary.VLerp` _returnvalue_2 _returnvalue_4 1.0) _returnvalue_2 (>= (`KismetMathLibrary.Dot_VectorVector` _returnvalue_4 _returnvalue_2) 0.5)))
  (bind _returnvalue_6 (+ (* (`KismetMathLibrary.VInterpTo_Constant` (`self.Laser Vector`) _returnvalue_5 Delta 1.0) 15000.0) _returnvalue))
  (set `self.Laser Vector` _returnvalue_5)
  (bind (_outhit _returnvalue_7) (`KismetSystemLibrary.LineTraceSingle` _returnvalue _returnvalue_6 "TraceTypeQuery1" false (`|MakeArray` Worm :!type "Actor Object Reference")))
  (`SceneComponent.SetVisibility` (`self.Niagara`) (not `Aiming Mode`) false)
  (`SceneComponent.SetVisibility` (`self.Aiming Laser`) `Aiming Mode` false)
  (if _returnvalue_7
    (bind (_bblockinghit _binitialoverlap _time _distance _location _impactpoint _normal _impactnormal _physmat _hitactor) (`GameplayStatics.BreakHitResult` _outhit))
    (`NiagaraComponent.SetVariableVec3` _returnvalue_3 "Beam End" _location)
    (bind _asbp_player (cast `/Game/Blueprints/Player/BP_Player` _hitactor)
      (:`then`
        (`/Game/Blueprints/Player/BP_Player.Health Change` _asbp_player (* -10.0 Delta) false))
      (:`CastFailed`
        _))
    (else
      (`NiagaraComponent.SetVariableVec3` _returnvalue_3 "Beam End" _returnvalue_6)))
  (`NiagaraComponent.SetVariableFloat` _returnvalue_3 "Opacity" Opacity))

(fn `Stop Firing Laser`
  (`SceneComponent.SetVisibility` (`self.Niagara`) false false)
  (`SceneComponent.SetVisibility` (`self.Aiming Laser`) false false))

(fn `UserConstructionScript`
  (`parent.UserConstructionScript`))
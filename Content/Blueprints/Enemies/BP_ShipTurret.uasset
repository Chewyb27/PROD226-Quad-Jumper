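; Enemy ship turret that fires missiles or laser blasts at the player or BP_Australis ships, then explodes and powers down on death.
; FindEnemy picks the nearest ship, using traces to discard blocked ones, and reruns when tracking fails.
; Tick drives WeaponAiming, which interpolates body yaw and clamped gun pitch, and WeaponTargeting, which gates fire by line of sight, plus barrel alignment for the player.
; Shots run on a cooldown with timeline recoil.
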(event `Weapon Aiming`
  (params (Delta :type "Float (double-precision)"))
  (bind _returnvalue (`self.GetTransform`))
  (bind _returnvalue_2 (`self.GetTransform`))
  (bind _playerreference (`self.PlayerReference`))
  (bind _gun_pivot (`self.Gun Pivot`))
  (bind _turret_body (`self.Turret Body`))
  (bind _rotation_speed (`self.Rotation Speed`))
  (bind _returnvalue_3 (`SceneComponent.K2_GetComponentLocation` (`self.Turret Body`)))
  (bind _returnvalue_4 (`self.K2_GetActorLocation` (`self.Ship Target`)))
  (bind _relativerotation (`SceneComponent.RelativeRotation` _turret_body))
  (bind _relativerotation_2 (`SceneComponent.RelativeRotation` (`self.Gun Pivot`)))
  (bind _returnvalue_5 (`SceneComponent.K2_GetComponentLocation` (`/Game/Blueprints/Player/BP_Player.Main Box Component` _playerreference)))
  (`/Engine/EditorBlueprintResources/StandardMacros.IsValid` _playerreference
    (:`Is Valid`
      (if (`self.No Ships Remaining`)
        (if (<= (`KismetMathLibrary.Vector_Distance` _returnvalue_5 _returnvalue_3) 35000.0)
          (if (`self.Can Fire`)
            _
            (else
              _))
          (`SceneComponent.K2_SetRelativeRotation` _turret_body (`KismetMathLibrary.MakeRotator` 0.0 0.0 (.yaw (`KismetMathLibrary.RInterpTo` _relativerotation (`KismetMathLibrary.FindLookAtRotation` (`KismetMathLibrary.InverseTransformDirection` _returnvalue_2 (`SceneComponent.K2_GetComponentLocation` _turret_body)) (`KismetMathLibrary.InverseTransformDirection` _returnvalue_2 _returnvalue_5)) Delta _rotation_speed))) false false)
          (`SceneComponent.K2_SetRelativeRotation` _gun_pivot (`KismetMathLibrary.MakeRotator` 0.0 (`KismetMathLibrary.ClampAngle` (.pitch (`KismetMathLibrary.RInterpTo` _relativerotation_2 (`KismetMathLibrary.FindLookAtRotation` (`KismetMathLibrary.InverseTransformDirection` _returnvalue_2 (`SceneComponent.K2_GetComponentLocation` (`self.Gun Pivot`))) (`KismetMathLibrary.InverseTransformDirection` _returnvalue_2 _returnvalue_5)) Delta _rotation_speed)) -5.0 100.0)) false false))
        (elif (not (`self.Targeting Player`))
          (if (<= (`KismetMathLibrary.Vector_Distance` _returnvalue_5 _returnvalue_3) 20000.0)
            _
            (else
              _))
          (if (`self.Can Fire`) :!label _label
            _
            (else
              _))
          (`SceneComponent.K2_SetRelativeRotation` _turret_body (`KismetMathLibrary.MakeRotator` 0.0 0.0 (.yaw (`KismetMathLibrary.RInterpTo` _relativerotation (`KismetMathLibrary.FindLookAtRotation` (`KismetMathLibrary.InverseTransformDirection` _returnvalue (`SceneComponent.K2_GetComponentLocation` (`self.Turret Body`))) (`KismetMathLibrary.InverseTransformDirection` _returnvalue _returnvalue_4)) Delta 2.0))) false false)
          (`SceneComponent.K2_SetRelativeRotation` _gun_pivot (`KismetMathLibrary.MakeRotator` 0.0 (`KismetMathLibrary.ClampAngle` (.pitch (`KismetMathLibrary.RInterpTo` _relativerotation_2 (`KismetMathLibrary.FindLookAtRotation` (`KismetMathLibrary.InverseTransformDirection` _returnvalue (`SceneComponent.K2_GetComponentLocation` (`self.Gun Pivot`))) (`KismetMathLibrary.InverseTransformDirection` _returnvalue _returnvalue_4)) Delta (`self.Rotation Speed`))) -5.0 100.0)) false false))))
    (:`Is Not Valid`
      (goto _label))))

(event `Find Enemy`
  (bind _allships (`self.Allships`))
  (bind _returnvalue (`SceneComponent.K2_GetComponentLocation` (`self.SM_Artillery_Base`)))
  (bind (_distance _returnvalue_2) (`GameplayStatics.FindNearestActor` _returnvalue _allships))
  (bind _outactors (`GameplayStatics.GetAllActorsOfClass` "/Game/Blueprints/Scene/BP_Australis.BP_Australis_C"))
  (bind _output_get (set `self.Allships` _outactors))
  (if (`KismetArrayLibrary.Array_IsEmpty` _output_get)
    (set `self.No Ships Remaining` true)
    (else
      (for _ _output_get
        (bind (_outhit _returnvalue_3) (`KismetSystemLibrary.LineTraceSingle` _returnvalue (`self.K2_GetActorLocation` _returnvalue_2) "TraceTypeQuery2" false _allships))
        (if _returnvalue_3
          (`KismetArrayLibrary.Array_RemoveItem` _allships _returnvalue_2)
          (else
            (set `self.Ship Target` _returnvalue_2))))
      (set `self.Ship Target` _returnvalue_2))))

(event `self.ReceiveBeginPlay`
  (bind _bulletspawn (`self.BulletSpawn`))
  (`KismetArrayLibrary.Array_Add` (`self.Bullet Spawn Pos`) _bulletspawn)
  (set `self.Selected Barrel` _bulletspawn)
  (set `self.Grounded` true)
  (set `self.Enemy Body` (`self.Turret Body`))
  (set `self.Firing Delay` (`KismetMathLibrary.RandomFloatInRange` 0.0 5.0))
  (`self.Find Enemy`)
  (`self.SetActorEnableCollision` (not (`self.IsChildActor`))))

(event `self.ReceiveTick`
  (params (DeltaSeconds :type "Float (single-precision)"))
  (bind _returnvalue (`self.GetActorScale3D`))
  (bind _playerreference (`self.PlayerReference`))
  (bind _playerreference_2 (`self.PlayerReference`))
  (bind _selected_barrel (`self.Selected Barrel`))
  (bind _location (.location (`SceneComponent.K2_GetComponentToWorld` (`self.Selected Barrel`))))
  (bind _rotation (.rotation (`SceneComponent.K2_GetComponentToWorld` (`self.Selected Barrel`))))
  (`/Engine/EditorBlueprintResources/StandardMacros.IsValid` _playerreference_2
    (:`Is Valid`
      (`self.Enemy Health Visibility`)
      (if (`self.EnemyAlive`)
        (if (<= (`KismetMathLibrary.Vector_Distance` (`SceneComponent.K2_GetComponentLocation` (`self.Enemy Body`)) (`SceneComponent.K2_GetComponentLocation` (`/Game/Blueprints/Player/BP_Player.Main Body` _playerreference_2))) 25000.0)
          (`|ExecutionSequence`
            (:`then_0`
              (`self.Enemy Health Visibility` :!label _label_2))
            (:`then_1`
              (`/Engine/EditorBlueprintResources/StandardMacros.IsValid` (`self.PlayerReference`)
                (:`Is Valid`
                  (`/Engine/EditorBlueprintResources/StandardMacros.IsValid` (`self.Ship Target`)
                    (:`Is Valid`
                      (`self.Weapon Aiming` DeltaSeconds :!label _label_3)
                      (`self.Weapon Targeting` DeltaSeconds)
                      (if (<= (`self.Firing Delay`) 0.0)
                        (if (`self.Can Fire`)
                          (set `self.Firing Delay` (`self.Firing Delay_0`))
                          (set `self.Selected Barrel` (`|GetArrayItem` (`self.Bullet Spawn Pos`) (`self.Barrel Index`)))
                          (if (== (`self.Projectile Type`) "/Game/Blueprints/Enemies/Weapons/BP_Missile.BP_Missile_C")
                            (`|SpawnActorFromClass` "/Game/Blueprints/Enemies/Weapons/BP_Missile.BP_Missile_C" (`KismetMathLibrary.MakeTransform` _location _rotation (* _returnvalue 0.3)) "AlwaysSpawn" "OverrideRootScale" null (`self.PlayerReference`) self null)
                            (bind (_direction _newtrack_0) (`Timeline|Recoil Absorbtion` :!via `PlayFromStart` :!label _label_4)
                              (:`Update`
                                (`SceneComponent.K2_SetRelativeLocation` _selected_barrel (+ (* (1.0 0.0 0.0) _newtrack_0 -50.0) (`KismetMathLibrary.MakeVector` 20.0 (.y (`SceneComponent.RelativeLocation` _selected_barrel)) (.z (`SceneComponent.RelativeLocation` _selected_barrel)))) false false)))
                            (else
                              (bind _returnvalue_2 (`|SpawnActorFromClass` "/Game/Blueprints/Enemies/Weapons/BP_LaserBlast.BP_LaserBlast_C" (`KismetMathLibrary.MakeTransform` _location _rotation (* _returnvalue 100.0)) "AlwaysSpawn" "OverrideRootScale" null (`self.Damage`) (`self.Projectile Speed`) (`self.Projectile Size`) (`self.Projectile Length`) null))
                              (goto _label_4 :!via `PlayFromStart`))))
                        (else
                          (set `self.Firing Delay` (`KismetMathLibrary.FClamp` (- (`self.Firing Delay`) DeltaSeconds) 0.0 100.0)))))
                    (:`Is Not Valid`
                      (if (`self.No Ships Remaining`)
                        (goto _label_3)
                        (else
                          (`self.Find Enemy` :!label _label_5)))))))))
          (else
            (`/Engine/EditorBlueprintResources/StandardMacros.IsValid` (`self.Ship Target`) :!label _label_6
              (:`Is Valid`
                (if (not (`self.Targeting Player`))
                  (if (>= (`self.time failed tracking`) 5.0)
                    (`self.Find Enemy`)
                    (set `self.time failed tracking` 0.0)
                    (else
                      (goto _label_3)))))
              (:`Is Not Valid`
                (if (`self.No Ships Remaining`)
                  (goto _label_2)
                  (else
                    (goto _label_5)))))))
        (else
          (`/Engine/EditorBlueprintResources/StandardMacros.DoOnce` false
            (:`Completed`
              (set `/Game/Blueprints/Player/BP_Player.Enemy Targeting` false _playerreference)
              (`KismetArrayLibrary.Array_RemoveItem` (`/Game/Blueprints/Player/BP_Player.Enemy Targeting Count` _playerreference) self)
              (`self.Death Animation`))))))
    (:`Is Not Valid`
      (goto _label_6))))

(event `Weapon Targeting`
  (params (Delta :type "Float (double-precision)"))
  (bind _ship_target (`self.Ship Target`))
  (bind _playerreference (`self.PlayerReference`))
  (bind _selected_barrel (`self.Selected Barrel`))
  (bind _barrel_index (`self.Barrel Index`))
  (bind _returnvalue (`SceneComponent.K2_GetComponentLocation` (`self.Turret Body`)))
  (bind _returnvalue_2 (`SceneComponent.K2_GetComponentLocation` (`/Game/Blueprints/Player/BP_Player.Main Box Component` _playerreference)))
  (bind _returnvalue_3 (<= (`KismetMathLibrary.Vector_Distance` _returnvalue_2 _returnvalue) (`self.Tracking Distance`)))
  (`/Engine/EditorBlueprintResources/StandardMacros.IsValid` _playerreference
    (:`Is Valid`
      (set `self.Targeting Player` _returnvalue_3)
      (if _returnvalue_3
        (set `self.Barrel Index` (`KismetMathLibrary.SelectInt` 0 (+ _barrel_index 1) (== _barrel_index (- (`KismetArrayLibrary.Array_Length` (`self.Bullet Spawn Pos`)) 1))))
        (bind (_outhit _returnvalue_4) (`KismetSystemLibrary.LineTraceSingle` _returnvalue _returnvalue_2 "TraceTypeQuery2" false (`|MakeArray` _playerreference :!type "Actor Object Reference")))
        (bind _returnvalue_5 (not _returnvalue_4))
        (set `self.Can Fire` (and _returnvalue_5 (>= (`KismetMathLibrary.Dot_VectorVector` (`SceneComponent.GetForwardVector` _selected_barrel) (`KismetMathLibrary.Normal` (- _returnvalue_2 (`SceneComponent.K2_GetComponentLocation` _selected_barrel)))) 0.98)))
        (if (not _returnvalue_5)
          (set `self.Targeting Player` _returnvalue_5))
        (else
          (if (not (`self.No Ships Remaining`)) :!label _label_7
            (`/Engine/EditorBlueprintResources/StandardMacros.IsValid` _ship_target
              (:`Is Valid`
                (bind (_outhit_2 _returnvalue_6) (`KismetSystemLibrary.LineTraceSingle` _returnvalue (`self.K2_GetActorLocation` _ship_target) "TraceTypeQuery2" false (`|MakeArray` _ship_target)))
                (set `self.Can Fire` (not _returnvalue_6))
                (set `self.time failed tracking` (`KismetMathLibrary.SelectFloat` (+ (`self.time failed tracking`) Delta) 0.0 _returnvalue_6)))
              (:`Is Not Valid`
                (set `self.Can Fire` false)))))))
    (:`Is Not Valid`
      (set `self.Targeting Player` false)
      (goto _label_7))))

(event `Death Animation`
  (bind _returnvalue (`SceneComponent.K2_GetComponentLocation` (`self.Turret Body`)))
  (`/Game/Widgets/WBP_PlayerHUD.Destroy Enemy` (`/Game/Blueprints/Player/BP_Player.HUD` (`self.PlayerReference`)) self)
  (`/Game/Blueprints/Player/BP_Player.Check Win State` (`self.PlayerReference`) false)
  (`GameplayStatics.SpawnEmitterAtLocation` "/Game/Particles/PS_Explosion.PS_Explosion" _returnvalue (struct) (40.0 40.0 40.0))
  (`KismetSystemLibrary.Delay` 0.1)
  (`GameplayStatics.SpawnEmitterAtLocation` "/Game/Particles/PS_Explosion.PS_Explosion" _returnvalue (struct) (25.0 25.0 25.0))
  (`/Engine/EditorBlueprintResources/StandardMacros.DoOnce` false
    (:`Completed`
      (set `self.EnemyAlive` false)
      (`PrimitiveComponent.SetMaterial` (`self.SM_Artillery_Energy`) 0 "/Game/Materials/GeneralMaterials/M_Black_Padding.M_Black_Padding")
      (`PrimitiveComponent.SetMaterial` (`self.Turret Body`) 0 "/Game/Materials/GeneralMaterials/M_Black_Padding.M_Black_Padding")
      (`self.Remove Lock`)
      (bind (_direction _newtrack_0) (`Timeline|Power Down Turret`)
        (:`Update`
          (`SceneComponent.K2_SetRelativeRotation` (`self.Gun Pivot`) (`KismetMathLibrary.MakeRotator` 0.0 (.pitch (`KismetMathLibrary.RInterpTo` (`SceneComponent.RelativeRotation` (`self.Gun Pivot`)) (struct :`Yaw` -50.0) 1.0 _newtrack_0))) false false))))))

(fn `UserConstructionScript`)
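; Flying enemy drone with a physics body that, while active, eases toward level, damps its spin and tilts two thrusters from body roll and pitch.
; BeginPlay picks a random NewWalker as Player, caches buildings and tanks, and sets up a health widget shown within range of that player.
; Zero health triggers death: gravity returns, it leaves the player's targeting list and explodes twice before being destroyed.
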(event `Gimbal Thrust`
  (params (Delta :type "Float (double-precision)"))
  (bind _roll (.roll (`SceneComponent.RelativeRotation` (`self.Body`))))
  (bind _pitch (.pitch (`SceneComponent.RelativeRotation` (`self.Body`))))
  (bind _returnvalue (* _pitch -0.25))
  (`SceneComponent.K2_SetRelativeRotation` (`self.Right Thrust`) (`KismetMathLibrary.MakeRotator` 0.0 (+ (`KismetMathLibrary.Lerp` (`KismetMathLibrary.ClampAngle` (+ (* _roll 3.0) 70.0 _returnvalue 0.0) -20.0 120.0) _pitch 0.025) 90.0)) false false)
  (`SceneComponent.K2_SetRelativeRotation` (`self.Left Thrust`) (`KismetMathLibrary.MakeRotator` 0.0 (+ (`KismetMathLibrary.Lerp` (`KismetMathLibrary.ClampAngle` (+ (* _roll -3.0) 70.0 _returnvalue 0.0) -20.0 120.0) _pitch 0.01) 90.0)) false false))

(event `Orientation Correction`
  (params (delta :type "Float (double-precision)"))
  (bind _body (`self.Body`))
  (`PrimitiveComponent.SetPhysicsAngularVelocityInDegrees` _body (`KismetMathLibrary.VInterpTo` (`PrimitiveComponent.GetPhysicsAngularVelocityInDegrees` _body "None") (0.0 0.0 0.0) delta 1.0) false "None")
  (`SceneComponent.K2_SetRelativeRotation` (`self.Body`) (`KismetMathLibrary.RInterpTo` (`self.K2_GetActorRotation`) (struct) delta 1.0) false false))

(event `self.ReceiveTick`
  (params (DeltaSeconds :type "Float (single-precision)"))
  (`self.Gimbal Thrust` DeltaSeconds)
  (`self.Health Visibility`)
  (`self.Orientation Correction` DeltaSeconds))

(event `Death`
  (bind _body (`self.Body`))
  (bind _returnvalue (`SceneComponent.K2_GetComponentLocation` _body))
  (`PrimitiveComponent.SetEnableGravity` _body true)
  (set `self.Dying` true)
  (`KismetArrayLibrary.Array_RemoveItem` (`/Game/Blueprints/Player/NewWalker.Enemy Targeting Count` (`self.Player`)) self)
  (`GameplayStatics.SpawnEmitterAtLocation` "/Game/Particles/P_Explosion.P_Explosion" _returnvalue (struct) (10.0 10.0 10.0))
  (`KismetSystemLibrary.Delay` 2.0)
  (`GameplayStatics.SpawnEmitterAtLocation` "/Game/Particles/P_Explosion.P_Explosion" _returnvalue (struct) (10.0 10.0 10.0))
  (`self.K2_DestroyActor`))

(event `Take Damage`
  (params (Damage :type "Float (double-precision)"))
  (bind _health (`self.Health`))
  (bind _output_get (set `self.Health` (- _health Damage)))
  (set `/Game/Stuff/Enemies/Enemy_Health.DisplayHealth` _output_get (`self.Health Bar`))
  (if (<= _health 0.0)
    (`self.Death`)))

(event `Health Visibility`
  (bind _display1 (`self.Display1`))
  (bind _player (`self.Player`))
  (`/Engine/EditorBlueprintResources/StandardMacros.IsValid` _player
    (:`Is Valid`
      (`SceneComponent.SetVisibility` _display1 (and (<= (`KismetMathLibrary.Vector_Distance` (`SceneComponent.K2_GetComponentLocation` (`/Game/Blueprints/Player/NewWalker.Main Body` _player)) (`SceneComponent.K2_GetComponentLocation` (`self.Body`))) 15000.0) (`self.Active`)) false))
    (:`Is Not Valid`
      (`SceneComponent.SetVisibility` _display1 false false))))

(event `self.ReceiveBeginPlay`
  (bind _health (`self.Health`))
  (`self.SetActorTickEnabled` (`self.Active`))
  (bind _outactors (`GameplayStatics.GetAllActorsOfClass` "/Game/Blueprints/Player/NewWalker.NewWalker_C"))
  (set `self.All Players` _outactors)
  (set `self.Player` (`KismetArrayLibrary.Array_Random` _outactors))
  (set `self.Height` (`KismetMathLibrary.RandomFloatInRange` 6000.0 6500.0))
  (bind _outactors_2 (`GameplayStatics.GetAllActorsOfClass` "/Game/Blueprints/Scene/BuildingV3.BuildingV3_C"))
  (`KismetArrayLibrary.Array_Append` (`self.Nearby Actors`) _outactors_2)
  (bind _outactors_3 (`GameplayStatics.GetAllActorsOfClass` "/Game/Blueprints/Enemies/EnemyTank.EnemyTank_C"))
  (set `self.Nearby Tanks` _outactors_3)
  (bind _asenemy_health (cast `/Game/Stuff/Enemies/Enemy_Health` (`WidgetComponent.GetUserWidgetObject` (`self.Display1`))))
  (bind _output_get (set `self.Health Bar` _asenemy_health))
  (set `/Game/Stuff/Enemies/Enemy_Health.MaxHealth` _health _output_get)
  (set `/Game/Stuff/Enemies/Enemy_Health.DisplayHealth` _health _output_get)
  (set `/Game/Stuff/Enemies/Enemy_Health.Enemy_Name` "Drone" _output_get)
  (set `self.Look Location` (`SceneComponent.K2_GetComponentLocation` (`Actor.RootComponent` (`.ReturnValue` (`GameplayStatics.FindNearestActor` (`self.K2_GetActorLocation`) (`self.Nearby Tanks`))))))
  (`self.Health Visibility`)
  (`PrimitiveComponent.SetEnableGravity` (`self.Body`) (not (`self.Active`))))

(fn `UserConstructionScript`)
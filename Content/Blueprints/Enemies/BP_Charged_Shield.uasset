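; Enemy shield actor that stays up while at least one of its linked generators is still active.
; BeginPlay puts a dynamic instance of MI_EnemyShield on the Shield component.
; While the shield is up, Tick polls the Generators array and drops the shield once all are disabled.
; The Dispersal timeline then animates the material's "Disperse Amount", and its event track turns off collision, with no path to raise the shield again.
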(event `self.ReceiveBeginPlay`
  (bind _returnvalue (`KismetMaterialLibrary.CreateDynamicMaterialInstance` "/Game/Materials/SpecialEffects/MI_EnemyShield.MI_EnemyShield"))
  (bind _output_get (set `self.Material` _returnvalue))
  (`PrimitiveComponent.SetMaterial` (`self.Shield`) 0 _output_get))

(event `self.ReceiveTick`
  (params (DeltaSeconds :type "Float (single-precision)"))
  (if (`self.Shield Up`)
    (set `self.Tower Up` false)
    (for _array_element (`self.Generators`)
      (if (not (`/Game/Blueprints/Scene/BP_Shield_Tower.Disabled` _array_element))
        (set `self.Tower Up` true)))
    (if (not (`self.Tower Up`))
      (set `self.Shield Up` false)
      (bind (_direction _newtrack_0) (`Timeline|Dispersal`)
        (:`Update`
          (`MaterialInstanceDynamic.SetScalarParameterValue` (`self.Material`) "Disperse Amount" _newtrack_0))
        (:`NewTrack_1`
          (`PrimitiveComponent.SetCollisionEnabled` (`self.Shield`) "NoCollision"))))))

(fn `UserConstructionScript`)
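; BP_Support_Structure is a grounded enemy structure that the player can destroy.
; BeginPlay sets its grounded flag and registers its Body as EnemyBody.
; While it is alive, Tick calls EnemyHealthVisibility whenever the player is within range.
; On death it leaves the player's targeting list, clears its HUD entry, triggers a win-state check, then plays two staggered explosions and destroys itself.
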(event `self.ReceiveBeginPlay`
  (set `self.Grounded` true)
  (set `self.Enemy Body` (`self.Body`)))

(event `self.ReceiveTick`
  (params (DeltaSeconds :type "Float (single-precision)"))
  (bind _playerreference (`self.PlayerReference`))
  (bind _playerreference_2 (`self.PlayerReference`))
  (`/Engine/EditorBlueprintResources/StandardMacros.IsValid` _playerreference_2
    (:`Is Valid`
      (if (`self.EnemyAlive`)
        (if (<= (`KismetMathLibrary.Vector_Distance` (`SceneComponent.K2_GetComponentLocation` (`self.Enemy Body`)) (`SceneComponent.K2_GetComponentLocation` (`/Game/Blueprints/Player/BP_Player.Main Body` _playerreference_2))) 55000.0)
          (`self.Enemy Health Visibility`))
        (else
          (`/Engine/EditorBlueprintResources/StandardMacros.DoOnce` false
            (:`Completed`
              (set `/Game/Blueprints/Player/BP_Player.Enemy Targeting` false _playerreference)
              (`KismetArrayLibrary.Array_RemoveItem` (`/Game/Blueprints/Player/BP_Player.Enemy Targeting Count` _playerreference) self)
              (`self.Death Animation`))))))))

(event `Death Animation`
  (bind _returnvalue (`SceneComponent.K2_GetComponentLocation` (`self.Body`)))
  (`/Game/Widgets/WBP_PlayerHUD.Destroy Enemy` (`/Game/Blueprints/Player/BP_Player.HUD` (`self.PlayerReference`)) self)
  (`/Game/Blueprints/Player/BP_Player.Check Win State` (`self.PlayerReference`) false)
  (`GameplayStatics.SpawnEmitterAtLocation` "/Game/Particles/PS_Explosion.PS_Explosion" _returnvalue (struct) (10.0 10.0 10.0))
  (`KismetSystemLibrary.Delay` 0.1)
  (`GameplayStatics.SpawnEmitterAtLocation` "/Game/Particles/PS_Explosion.PS_Explosion" _returnvalue (struct) (10.0 10.0 10.0))
  (`/Engine/EditorBlueprintResources/StandardMacros.DoOnce` false
    (:`Completed`
      (`self.K2_DestroyActor`))))

(fn `UserConstructionScript`)
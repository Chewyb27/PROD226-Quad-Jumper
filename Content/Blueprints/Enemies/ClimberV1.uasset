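; ClimberV1 is an enemy Blueprint that moves along walls and steers toward the nearest player, extending a parent class.
; While OnWall is set, Tick pushes the root forward with a swept local offset and, if a player is valid, yaws it by the dot of its right vector and the direction to that player.
; The construction script assigns the static mesh as EnemyBody.
; An actor-offset move and a vector projection attempt are left disconnected.
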(event `self.ReceiveTick`
  (params (DeltaSeconds :type "Float (single-precision)"))
  (bind _defaultsceneroot (`self.DefaultSceneRoot`))
  (bind _nearest_player (`self.Nearest Player`))
  (`parent.ReceiveTick` DeltaSeconds)
  (if (`self.On Wall`)
    (`SceneComponent.K2_AddLocalOffset` _defaultsceneroot (`KismetMathLibrary.MakeVector` (* DeltaSeconds 3000.0)) true false)
    (`/Engine/EditorBlueprintResources/StandardMacros.IsValid` _nearest_player
      (:`Is Valid`
        (`SceneComponent.K2_AddLocalRotation` _defaultsceneroot (`KismetMathLibrary.MakeRotator` 0.0 0.0 (* (`KismetMathLibrary.Dot_VectorVector` (`SceneComponent.GetRightVector` _defaultsceneroot) (`KismetMathLibrary.Normal` (- (`self.K2_GetActorLocation` _nearest_player) (`SceneComponent.K2_GetComponentLocation` _defaultsceneroot)))) DeltaSeconds 1000.0)) false false)))))

(fn `UserConstructionScript`
  (`parent.UserConstructionScript`)
  (set `self.Enemy Body` (`self.StaticMesh`)))
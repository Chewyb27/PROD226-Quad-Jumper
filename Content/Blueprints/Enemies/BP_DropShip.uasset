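; BP_DropShip is an enemy dropship that delivers ground units, then fights the player as a hovering gunship.
; A timeline lowers the shielded ship over DropLocation, spawns missile trucks and tanks, then lifts it before it activates as an enemy.
; Tick then holds height, turns toward the player, gimbals its thrusters and alternates pod missiles after a sustained line-of-sight lock.
; Impacts deal damage, and death triggers explosions and a win-state check.
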(event `Drop Sequence`
  (bind _main_body (`self.Main Body`))
  (bind _drop_amounts (`self.Drop Amounts`))
  (bind _main_body_2 (`self.Main Body`))
  (bind _drop_location (`self.Drop Location`))
  (bind _returnvalue (`KismetMathLibrary.MakeTransform` (+ _drop_location (* (`KismetMathLibrary.RandomUnitVector`) (2000.0 2000.0 0.0)) (0.0 0.0 100.0)) (`KismetMathLibrary.MakeRotator` 0.0 0.0 (.yaw (`KismetMathLibrary.RandomRotator` false)))))
  (if (not (== (`self.Drop Location`) (0.0 0.0 0.0) :`ErrorTolerance` 500.0))
    (`|ExecutionSequence`
      (:`then_0`
        (`self.Refresh Shield` true)
        (`Timeline|Drop Timer`
          (:`Update`
            (set `self.Dropping Units` true)
            (`SceneComponent.K2_SetWorldLocation` _main_body_2 (`KismetMathLibrary.VInterpTo` (`SceneComponent.K2_GetComponentLocation` _main_body_2) (+ _drop_location (0.0 0.0 3000.0)) (`self.Delta`) 0.5) false false)
            (`SceneComponent.K2_SetWorldRotation` _main_body_2 (`KismetMathLibrary.MakeRotator` 0.0 0.0 (.yaw (`SceneComponent.K2_GetComponentRotation` _main_body_2))) false false))
          (:`Finished`
            (for _ (range 1 (+ (`|GetArrayItem` _drop_amounts) 1))
              (bind _returnvalue_2 (`|SpawnActorFromClass` "/Game/Blueprints/Enemies/BP_Missile_Truck.BP_Missile_Truck_C" _returnvalue "AdjustIfPossibleButAlwaysSpawn" "OverrideRootScale" null true (`self.PlayerReference`) 200.0 false false false null))
              (`self.Initialize Enemy` _returnvalue_2))
            (for _ (range 1 (+ (`|GetArrayItem` _drop_amounts 1) 1))
              (bind _returnvalue_3 (`|SpawnActorFromClass` "/Game/Blueprints/Enemies/BP_Tank.BP_Tank_C" _returnvalue "AdjustIfPossibleButAlwaysSpawn" "OverrideRootScale" null true (`self.PlayerReference`) 300.0 false false false null))
              (`self.Initialize Enemy` _returnvalue_3))
            (`ActorComponent.K2_DestroyComponent` (`self.StaticMesh`))
            (`Timeline|move away from dropped enemies`
              (:`Update`
                (`SceneComponent.K2_SetWorldLocation` _main_body (`KismetMathLibrary.VInterpTo` (`SceneComponent.K2_GetComponentLocation` _main_body) (+ (`self.Drop Location`) (`KismetMathLibrary.MakeVector` 0.0 0.0 (+ 7000.0 (`KismetMathLibrary.RandomFloatInRange` 0.0 10000.0)))) (`self.Delta`) 0.5) false false))
              (:`Finished`
                (set `self.Dropping Units` false)
                (`self.Initialize Enemy`)
                (`self.Refresh Shield` false)))))))))

(event `self.ReceiveBeginPlay`
  (bind _returnvalue (`self.K2_GetActorLocation`))
  ;[1 0 0] Begin Play
  (set `self.Enemy Body` (`self.Main Body`))
  (`self.Initialize Shield`)
  (`self.SetActorTickEnabled` (`self.Active`))
  (set `self.Look Location` (0.0 0.0 0.0))
  (`PrimitiveComponent.SetEnableGravity` (`self.Main Body`) (not (`self.Active`)))
  ;[0.3333 0.2588 0.04514] Define Hover Position
  (bind (_outhit _returnvalue_2) (`KismetSystemLibrary.LineTraceSingle` _returnvalue (+ _returnvalue (* (`KismetMathLibrary.Vector_Down`) 10000.0)) "TraceTypeQuery1"))
  (set `self.Height` (`KismetMathLibrary.SelectFloat` (+ (.z (`.Location` (`GameplayStatics.BreakHitResult` _outhit))) (`KismetMathLibrary.RandomFloatInRange` 6000.0 6500.0)) (.z (`self.K2_GetActorLocation`)) _returnvalue_2))
  (`self.Drop Sequence`))

(event `self.ReceiveTick`
  (params (DeltaSeconds :type "Float (single-precision)"))
  (bind _returnvalue (`KismetMathLibrary.Vector_Up`))
  (bind _targeting_time (`self.Targeting Time`))
  (bind _playerreference (`self.PlayerReference`))
  (bind _playerreference_2 (`self.PlayerReference`))
  (bind _enemy_class_display (`self.Enemy Class Display`))
  (bind (_returnvalue_roll _returnvalue_pitch _returnvalue_yaw) (`KismetMathLibrary.BreakRotator` (`SceneComponent.K2_GetComponentRotation` (`self.Main Body`))))
  (bind _returnvalue_2 (`SceneComponent.K2_GetComponentLocation` (`/Game/Blueprints/Player/BP_Player.Main Box Component` (`self.PlayerReference`))))
  (bind _yaw (.yaw (`KismetMathLibrary.FindLookAtRotation` (`SceneComponent.K2_GetComponentLocation` (`self.Main Body`)) (`KismetMathLibrary.SelectVector` _returnvalue_2 _returnvalue_2 (`self.Player Found`)))))
  (set `self.Delta` DeltaSeconds)
  (`/Engine/EditorBlueprintResources/StandardMacros.IsValid` _playerreference
    (:`Is Valid`
      (if (`self.EnemyAlive`)
        (if (<= (`KismetMathLibrary.Vector_Distance` (`SceneComponent.K2_GetComponentLocation` (`self.Enemy Body`)) (`SceneComponent.K2_GetComponentLocation` (`/Game/Blueprints/Player/BP_Player.Main Body` _playerreference))) 35000.0)
          ;[1 0 0] Event Tick
          (if (`self.Dropping Units`)
            (`/Engine/EditorBlueprintResources/StandardMacros.IsValid` _enemy_class_display
              (:`Is Valid`
                (`SceneComponent.K2_SetWorldLocation` _enemy_class_display (`SceneComponent.K2_GetComponentLocation` (`self.Main Body`)) false false)
                (`self.Enemy Health Visibility`)))
            (else
              (`self.Enemy Health Visibility`)
              (`/Engine/EditorBlueprintResources/StandardMacros.IsValid` _playerreference_2
                (:`Is Valid`
                  (set `self.Player Found` (and (`KismetSystemLibrary.IsValid` _playerreference_2) (<= (`KismetMathLibrary.Vector_Distance` (`SceneComponent.K2_GetComponentLocation` (`/Game/Blueprints/Player/BP_Player.Main Box Component` _playerreference_2)) (`SceneComponent.K2_GetComponentLocation` (`self.Main Body`))) 25000.0)))
                  (set `self.ChangeInYaw` _yaw)
                  (`self.Gimbal Thrust`)
                  (`SceneComponent.K2_SetRelativeRotation` (`self.Main Body`) (`KismetMathLibrary.RInterpTo` (`SceneComponent.K2_GetComponentRotation` (`self.Main Body`)) (`KismetMathLibrary.MakeRotator` (`KismetMathLibrary.ClampAngle` (* (- _returnvalue_yaw _yaw) -6.0) -20.0 20.0) 0.0 _yaw) DeltaSeconds 1.0) false false)
                  (`self.K2_SetActorLocation` (`KismetMathLibrary.MakeVector` (.x (`self.K2_GetActorLocation`)) (.y (`self.K2_GetActorLocation`)) (`KismetMathLibrary.Lerp` (.z (`self.K2_GetActorLocation`)) (`KismetMathLibrary.SelectFloat` (`self.Height`) 0.0 true) 0.002)) false true)
                  (`self.K2_AddActorWorldOffset` (* (+ (* _returnvalue (`KismetMathLibrary.Abs` (.roll (`SceneComponent.RelativeRotation` (`self.Main Body`)))) -1.0) (* _returnvalue (`KismetMathLibrary.Abs` (.pitch (`SceneComponent.RelativeRotation` (`self.Main Body`)))) -1.0)) 0.1))
                  (`SceneComponent.K2_SetWorldLocation` (`self.Enemy Class Display`) (`SceneComponent.K2_GetComponentLocation` (`self.Main Body`)) false false)
                  (if (`self.Player Found`)
                    (`self.Target Player`)
                    (if (`self.Player Targeting`)
                      (set `self.Targeting Time` (+ DeltaSeconds _targeting_time))
                      (if (>= _targeting_time 3.0)
                        (set `self.Targeting Time` 0.0)
                        (`/Engine/EditorBlueprintResources/StandardMacros.FlipFlop`
                          (:`A`
                            (`|SpawnActorFromClass` "/Game/Blueprints/Enemies/Weapons/BP_Missile.BP_Missile_C" (`SceneComponent.K2_GetComponentToWorld` (`self.Left Missile Pod`)) "AlwaysSpawn" "OverrideRootScale" self (`self.PlayerReference`) null))
                          (:`B`
                            (`|SpawnActorFromClass` "/Game/Blueprints/Enemies/Weapons/BP_Missile.BP_Missile_C" (`SceneComponent.K2_GetComponentToWorld` (`self.Right Missile Pod`)) "AlwaysSpawn" "OverrideRootScale" self (`self.PlayerReference`) null))))
                      (else
                        (set `self.Targeting Time` 0.0)))
                    (else
                      (`self.Stop Targeting Player`))))))))
        (else
          (`self.Death Check`))))))

(event `Death Check`
  (bind _playerreference (`self.PlayerReference`))
  (bind _returnvalue (`SceneComponent.K2_GetComponentLocation` (`self.Main Body`)))
  ;[0 0 0] Death
  (`/Engine/EditorBlueprintResources/StandardMacros.DoOnce` false
    (:`Completed`
      (`PrimitiveComponent.SetEnableGravity` (`self.Main Body`) true)
      (set `/Game/Blueprints/Player/BP_Player.Enemy Targeting` false _playerreference)
      (set `self.Targeting Time` 0.0)
      (`KismetArrayLibrary.Array_RemoveItem` (`/Game/Blueprints/Player/BP_Player.Enemy Targeting Count` _playerreference) self)
      (`/Game/Blueprints/Player/BP_Player.Check Win State` (`self.PlayerReference`) false)
      (`GameplayStatics.SpawnEmitterAtLocation` "/Game/Particles/PS_Explosion.PS_Explosion" _returnvalue (struct) (10.0 10.0 10.0))
      (`KismetSystemLibrary.Delay` 2.0)
      (`GameplayStatics.SpawnEmitterAtLocation` "/Game/Particles/PS_Explosion.PS_Explosion" _returnvalue (struct) (10.0 10.0 10.0))
      (`/Engine/EditorBlueprintResources/StandardMacros.DoOnce` false
        (:`Completed`
          (`self.K2_DestroyActor`))))))

(event `Target Player`
  (bind _returnvalue (`self.K2_GetActorLocation`))
  (bind _playerreference (`self.PlayerReference`))
  (bind _returnvalue_2 (`SceneComponent.K2_GetComponentLocation` (`/Game/Blueprints/Player/BP_Player.Main Box Component` _playerreference)))
  ;[0.1116 0.003938 0.1458] Check for Obstacles blocking targeting
  (`/Engine/EditorBlueprintResources/StandardMacros.IsValid` _playerreference
    (:`Is Valid`
      (if (<= (`KismetMathLibrary.Vector_Distance` _returnvalue_2 _returnvalue) 12000.0)
        (bind (_outhit _returnvalue_3) (`KismetSystemLibrary.LineTraceSingle` _returnvalue _returnvalue_2 "TraceTypeQuery1" false (`self.All Players`)))
        (if _returnvalue_3
          (set `/Game/Blueprints/Player/BP_Player.Enemy Targeting` false _playerreference)
          (set `self.Player Targeting` false)
          (`KismetArrayLibrary.Array_RemoveItem` (`/Game/Blueprints/Player/BP_Player.Enemy Targeting Count` _playerreference) self)
          (else
            (set `/Game/Blueprints/Player/BP_Player.Enemy Targeting` true _playerreference)
            (set `self.Player Targeting` true)
            (`KismetArrayLibrary.Array_Add` (`/Game/Blueprints/Player/BP_Player.Enemy Targeting Count` _playerreference) self)))
        (else
          (set `/Game/Blueprints/Player/BP_Player.Enemy Targeting` false _playerreference)
          (set `self.Player Targeting` false)
          (`KismetArrayLibrary.Array_RemoveItem` (`/Game/Blueprints/Player/BP_Player.Enemy Targeting Count` _playerreference) self))))))

(event `Check for Player in Target Zone`
  ;[0.1116 0.003938 0.1458] Check for Obstacles blocking targeting
  (set `self.Player Targeting` (<= (`KismetMathLibrary.Vector_Distance` (`SceneComponent.K2_GetComponentLocation` (`/Game/Blueprints/Player/BP_Player.Main Box Component` (`self.PlayerReference`))) (`SceneComponent.K2_GetComponentLocation` (`self.Main Body`))) 10000.0)))

(event `self.Main Body.OnComponentHit`
  (params (HitComponent :type "PrimitiveComponent Object Reference") (OtherActor :type "Actor Object Reference") (OtherComp :type "PrimitiveComponent Object Reference") (NormalImpulse :type "Vector Structure") (Hit :type "HitResult Structure (by ref)"))
  (bind _returnvalue (`GameplayStatics.GetObjectClass` OtherActor))
  ;[1 0.3116 0.06994] Collision Damage
  (if (>= (`self.GetGameTimeSinceCreation`) 0.5)
    (if (and (!= OtherActor self) (or (== _returnvalue "BP_DropShip_C") (== _returnvalue "/Game/Blueprints/Scene/BP_Comms_Tower.BP_Comms_Tower_C")))
      (bind _asbp_drop_ship (cast `/Game/Blueprints/Enemies/BP_DropShip` OtherActor)
        (:`then`
          (`self.Take Damage` _asbp_drop_ship 2000.0))
        (:`CastFailed`
          (cast `/Game/Blueprints/Scene/BP_Comms_Tower` OtherActor)
          (`self.Take Damage` 2000.0)))
      (elif (`|EnumEquality` (`SceneComponent.Mobility` OtherComp) "Static")
        (`/Engine/EditorBlueprintResources/StandardMacros.DoOnce` false :!label _label
          (:`Completed`
            (`self.Take Damage` (* (+ (.x (`KismetMathLibrary.Vector_GetAbs` (`self.GetVelocity`))) (.y (`KismetMathLibrary.Vector_GetAbs` (`self.GetVelocity`))) (.z (`KismetMathLibrary.Vector_GetAbs` (`self.GetVelocity`)))) 0.1))
            (`Timeline|Collide Cooldown` :!via `PlayFromStart`
              (:`Finished`
                (goto _label :!via `Reset`)))))))))

(event `Gimbal Thrust`
  (bind _roll (.roll (`SceneComponent.RelativeRotation` (`self.Main Body`))))
  (bind _pitch (.pitch (`SceneComponent.RelativeRotation` (`self.Main Body`))))
  (bind _returnvalue (* _pitch -0.25))
  ;[0.4323 0.4323 0.4323] Gimble Thrusters
  (`SceneComponent.K2_SetRelativeRotation` (`self.Right Thruster`) (`KismetMathLibrary.MakeRotator` 0.0 (`KismetMathLibrary.Lerp` (`KismetMathLibrary.ClampAngle` (+ (* _roll 3.0) 70.0 _returnvalue 0.0) -20.0 120.0) _pitch 0.025)) false false)
  (`SceneComponent.K2_SetRelativeRotation` (`self.Left Thruster`) (`KismetMathLibrary.MakeRotator` 0.0 (`KismetMathLibrary.Lerp` (`KismetMathLibrary.ClampAngle` (+ (* _roll -3.0) 70.0 _returnvalue 0.0) -20.0 120.0) _pitch 0.01)) false false))

(fn `Pull_Location`
  (params (`World Location` :type "Vector Structure")))

(fn `Stop Targeting Player`
  (bind _playerreference (`self.PlayerReference`))
  (set `/Game/Blueprints/Player/BP_Player.Enemy Targeting` false _playerreference)
  (set `self.Targeting Time` 0.0)
  (`KismetArrayLibrary.Array_RemoveItem` (`/Game/Blueprints/Player/BP_Player.Enemy Targeting Count` _playerreference) self))

(fn `UserConstructionScript`)
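; Copycat enemy that trails a spline path a set number of points (Lag) behind its end and registers itself with the player's HUD.
; Each Tick interpolates it toward that point, and a periodic box trace switches between ground and air modes.
; Grounded, it follows spline rotation and animates four legs; airborne, it sways, turns toward the player and tilts two rotors.
; A laser beam shows when its line-of-sight and facing checks pass.
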(event `Ground Check`
  (bind _groundcheck (`self.GroundCheck`))
  (bind _cube (`self.Cube`))
  (bind _returnvalue (`SceneComponent.K2_GetComponentLocation` _cube))
  (if (> _groundcheck 0.2)
    (set `self.GroundCheck` 0.0)
    (bind (_outhit _returnvalue_2) (`KismetSystemLibrary.BoxTraceSingle` _returnvalue (+ (* (`SceneComponent.GetUpVector` _cube) -300.0) _returnvalue) (450.0 550.0 150.0) (`self.K2_GetActorRotation`) "TraceTypeQuery1"))
    (bind _output_get (set `self.OnGround` _returnvalue_2))
    (set `self.Grounded` _returnvalue_2)
    (else
      (set `self.GroundCheck` (+ (stale `self.ReceiveTick` DeltaSeconds) _groundcheck))))
  (if _output_get
    _))

(event `self.ReceiveTick`
  (params (DeltaSeconds :type "Float (single-precision)"))
  (bind _returnvalue (`self.K2_GetActorLocation`))
  (bind _grounded (`self.Grounded`))
  (bind _spline_instance (`self.Spline Instance`))
  (bind _delta_seconds (`self.Delta Seconds`))
  (bind _returnvalue_2 (`KismetMathLibrary.DegSin` (`KismetSystemLibrary.GetGameTimeInSeconds`)))
  (bind _spline (`/Game/Blueprints/Player/PlayerFollowSpline.Spline` _spline_instance))
  (bind _returnvalue_3 (`SplineComponent.GetNumberOfSplinePoints` _spline))
  (bind _returnvalue_4 (`KismetMathLibrary.Lerp` 0.0 (`SplineComponent.GetSplineLength` _spline) (`self.Alpha`)))
  (bind _returnvalue_5 (`SplineComponent.GetLocationAtDistanceAlongSpline` _spline _returnvalue_4 "World"))
  (bind _returnvalue_6 (`KismetMathLibrary.VInterpTo` _returnvalue (`KismetMathLibrary.SelectVector` _returnvalue_5 (+ _returnvalue_5 (* (`KismetMathLibrary.MakeVector` _returnvalue_2 _returnvalue_2 _returnvalue_2) 1000.0)) (`self.Grounded`)) _delta_seconds 2.0))
  (bind _returnvalue_7 (- _returnvalue_6 _returnvalue))
  (set `self.Delta Seconds` DeltaSeconds)
  (`/Engine/EditorBlueprintResources/StandardMacros.IsValid` _spline_instance
    (:`Is Valid`
      (`|ExecutionSequence`
        (:`then_0`
          (set `self.Alpha` (/ (- _returnvalue_3 (`self.Lag`)) _returnvalue_3))
          (`self.K2_SetActorRotation` (`KismetMathLibrary.RInterpTo` (`self.K2_GetActorRotation`) (`KismetMathLibrary.SelectRotator` (`SplineComponent.GetRotationAtDistanceAlongSpline` _spline _returnvalue_4 "World") (`KismetMathLibrary.MakeRotator` 0.0 0.0 (.yaw (`KismetMathLibrary.FindLookAtRotation` _returnvalue (`SceneComponent.K2_GetComponentLocation` (`/Game/Blueprints/Player/NewWalker.Box` (`self.Player Instance`)))))) _grounded) _delta_seconds (`KismetMathLibrary.SelectFloat` 8.0 0.5 _grounded)))
          (`self.K2_SetActorLocation` _returnvalue_6 true)
          (set `self.Forward Speed` (* (`KismetMathLibrary.VSize` (`KismetMathLibrary.ClampVectorSize` _returnvalue_7 -1.0 1.0)) 0.3))
          (if (`self.Grounded`)
            (`SceneComponent.K2_SetRelativeRotation` :`self` (`self.Rotor 2`))
            (`SceneComponent.K2_SetRelativeRotation` :`self` (`self.Rotor 1`))
            (else
              (`self.Gimbal Thrust` 0.0 (.y (`KismetMathLibrary.TransformLocation` (`self.GetTransform`) _returnvalue_7))))))
        (:`then_1`
          (`self.Animate BL`))
        (:`then_2`
          (`self.Animate BR`))
        (:`then_3`
          (`self.animate FL`))
        (:`then_4`
          (`self.Animate FR`))
        (:`then_5`
          (`self.Ground Check`))
        (:`then_6`
          (`self.Aim laser`))
        (:`then_7`
          (`/Engine/EditorBlueprintResources/StandardMacros.DoOnce` false
            (:`Completed`
              (`/Game/Widgets/WalkerHUD.Add Enemy` (`/Game/Blueprints/Player/NewWalker.HUD` (`self.Player Instance`)) self))))))))

(event `self.ReceiveBeginPlay`)

(event `Gimbal Thrust`
  (params (Delta :type "Float (double-precision)") (MoveAmount :type "Float (double-precision)"))
  (bind _returnvalue (* 0.0 1.0))
  (bind _roll (.roll (`SceneComponent.RelativeRotation` (`self.Main Body`))))
  (bind _pitch (.pitch (`SceneComponent.RelativeRotation` (`self.Main Body`))))
  (bind _returnvalue_2 (* _pitch -0.25))
  (`SceneComponent.K2_SetRelativeRotation` (`self.Rotor 1`) (`KismetMathLibrary.MakeRotator` _returnvalue (+ (`KismetMathLibrary.Lerp` (`KismetMathLibrary.ClampAngle` (+ (* _roll 3.0) 70.0 _returnvalue_2 0.0) -20.0 120.0) _pitch 0.025) 90.0)) false false)
  (`SceneComponent.K2_SetRelativeRotation` (`self.Rotor 2`) (`KismetMathLibrary.MakeRotator` _returnvalue (+ (`KismetMathLibrary.Lerp` (`KismetMathLibrary.ClampAngle` (+ (* _roll -3.0) 70.0 _returnvalue_2 0.0) -20.0 120.0) _pitch 0.01) 90.0)) false false))

(event `Follow Sequence`
  (bind _followspeed (`self.FollowSpeed`))
  (`TimelineComponent.SetPlayRate` _followspeed (/ 1.0 (`self.StartDuration`)))
  (`TimelineComponent.SetNewTime` _followspeed (`self.StartOffset`))
  (`Timeline|FollowSpeed`))

(event `Aim laser`
  (bind _player_instance (`self.Player Instance`))
  (bind _laser (`self.Laser`))
  (bind _returnvalue (`SceneComponent.K2_GetComponentLocation` (`self.Sphere`)))
  (bind _returnvalue_2 (`SceneComponent.K2_GetComponentLocation` (`/Game/Blueprints/Player/NewWalker.Main Body` _player_instance)))
  (`/Engine/EditorBlueprintResources/StandardMacros.IsValid` _player_instance
    (:`Is Valid`
      (bind (_outhit _returnvalue_3) (`KismetSystemLibrary.LineTraceSingle` _returnvalue _returnvalue_2 "TraceTypeQuery1" false (`|MakeArray` self _player_instance :!type "Actor Object Reference")))
      (`SceneComponent.SetVisibility` _laser (and (not _returnvalue_3) (< (`KismetMathLibrary.Dot_VectorVector` (`SceneComponent.GetUpVector` (`self.Sphere`)) (- _returnvalue_2 _returnvalue)) 0.0)) false)
      (`FXSystemComponent.SetVectorParameter` _laser "Beam End" _returnvalue_2))))

(event `animate FL`
  (bind _asback_left_leg (cast `/Game/Animations/BackLeftLeg` (`SkeletalMeshComponent.GetAnimInstance` (`self.legFLSM`))))
  (`KismetSystemLibrary.Delay` 0.0)
  (set `/Game/Animations/BackLeftLeg.ForwardSpeed` (* (`self.Forward Speed`) -1.0 (`KismetMathLibrary.SelectFloat` 1.8 0.0 (`self.Grounded`))) _asback_left_leg))

(event `Animate FR`
  (bind _asback_left_leg (cast `/Game/Animations/BackLeftLeg` (`SkeletalMeshComponent.GetAnimInstance` (`self.legFRSM`))))
  (`KismetSystemLibrary.Delay` 0.2)
  (set `/Game/Animations/BackLeftLeg.ForwardSpeed` (* (`self.Forward Speed`) (`KismetMathLibrary.SelectFloat` 1.8 0.0 (`self.Grounded`))) _asback_left_leg))

(event `Animate BL`
  (bind _asback_left_leg (cast `/Game/Animations/BackLeftLeg` (`SkeletalMeshComponent.GetAnimInstance` (`self.legBLSM`))))
  (`KismetSystemLibrary.Delay` 0.2)
  (set `/Game/Animations/BackLeftLeg.ForwardSpeed` (* (`self.Forward Speed`) (`KismetMathLibrary.SelectFloat` 1.8 0.0 (`self.Grounded`))) _asback_left_leg))

(event `Animate BR`
  (bind _asback_left_leg (cast `/Game/Animations/BackLeftLeg` (`SkeletalMeshComponent.GetAnimInstance` (`self.legBRSM`))))
  (`KismetSystemLibrary.Delay` 0.0)
  (set `/Game/Animations/BackLeftLeg.ForwardSpeed` (* (`self.Forward Speed`) (`KismetMathLibrary.SelectFloat` 1.8 0.0 (`self.Grounded`))) _asback_left_leg))

(fn `UserConstructionScript`)
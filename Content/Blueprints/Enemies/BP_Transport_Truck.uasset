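; Transport truck enemy, a grounded target that does not attack as currently wired.
; On Tick it updates health visibility while the player is in range.
; When no longer alive, it clears itself from player targeting, then removes its HUD entry, triggers a win-state check, plays two explosions and destroys itself.
; Pod aiming, line-of-sight targeting and missile-firing logic remains in the graph but never runs.
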(event `self.ReceiveBeginPlay`
  (set `self.Grounded` true)
  (set `self.Enemy Body` (`self.Truck Body`)))

(event `Pod Aiming`
  (params (Delta :type "Float (double-precision)"))
  (bind _pod_rotator (`self.Pod Rotator`))
  (bind _returnvalue (`SceneComponent.K2_GetComponentLocation` (`/Game/Blueprints/Player/BP_Player.Main Box Component` (`self.PlayerReference`))))
  (bind _returnvalue_2 (`KismetMathLibrary.FindLookAtRotation` (`SceneComponent.K2_GetComponentLocation` _pod_rotator) _returnvalue))
  (bind _yaw (.yaw (`KismetMathLibrary.RInterpTo` (`SceneComponent.K2_GetComponentRotation` _pod_rotator) _returnvalue_2 Delta 1.0)))
  (if (<= (`KismetMathLibrary.Vector_Distance` _returnvalue (`SceneComponent.K2_GetComponentLocation` (`self.Truck Body`))) 20000.0)
    (`SceneComponent.K2_SetWorldRotation` _pod_rotator (`KismetMathLibrary.MakeRotator` 0.0 0.0 _yaw) false false)
    (`SceneComponent.K2_SetWorldRotation` (`self.Pod Pitcher`) (`KismetMathLibrary.MakeRotator` 0.0 (.pitch (`KismetMathLibrary.RInterpTo` (`SceneComponent.K2_GetComponentRotation` (`self.Pod Pitcher`)) _returnvalue_2 Delta 1.0)) _yaw) false false)))

(event `self.ReceiveTick`
  (params (DeltaSeconds :type "Float (single-precision)"))
  (bind _playerreference (`self.PlayerReference`))
  (bind _playerreference_2 (`self.PlayerReference`))
  (set `self.Timeline Tick` (+ DeltaSeconds (`self.Timeline Tick`)))
  (`/Engine/EditorBlueprintResources/StandardMacros.IsValid` _playerreference_2
    (:`Is Valid`
      (if (`self.EnemyAlive`)
        (if (<= (`KismetMathLibrary.Vector_Distance` (`SceneComponent.K2_GetComponentLocation` (`self.Enemy Body`)) (`SceneComponent.K2_GetComponentLocation` (`/Game/Blueprints/Player/BP_Player.Main Body` _playerreference_2))) 35000.0)
          (`self.Enemy Health Visibility`)
          (`/Engine/EditorBlueprintResources/StandardMacros.IsValid` (`self.PlayerReference`)))
        (else
          (`/Engine/EditorBlueprintResources/StandardMacros.DoOnce` false
            (:`Completed`
              (set `/Game/Blueprints/Player/BP_Player.Enemy Targeting` false _playerreference)
              (`KismetArrayLibrary.Array_RemoveItem` (`/Game/Blueprints/Player/BP_Player.Enemy Targeting Count` _playerreference) self)
              (`self.Death Animation`))))))))

(event `Pod Targeting`
  (params (Delta :type "Float (double-precision)")))

(event `Death Animation`
  (bind _returnvalue (`SceneComponent.K2_GetComponentLocation` (`self.Truck Body`)))
  (`/Game/Widgets/WBP_PlayerHUD.Destroy Enemy` (`/Game/Blueprints/Player/BP_Player.HUD` (`self.PlayerReference`)) self)
  (`/Game/Blueprints/Player/BP_Player.Check Win State` (`self.PlayerReference`) false)
  (`GameplayStatics.SpawnEmitterAtLocation` "/Game/Particles/PS_Explosion.PS_Explosion" _returnvalue (struct) (10.0 10.0 10.0))
  (`KismetSystemLibrary.Delay` 0.1)
  (`GameplayStatics.SpawnEmitterAtLocation` "/Game/Particles/PS_Explosion.PS_Explosion" _returnvalue (struct) (10.0 10.0 10.0))
  (`/Engine/EditorBlueprintResources/StandardMacros.DoOnce` false
    (:`Completed`
      (`self.K2_DestroyActor`))))

(fn `UserConstructionScript`)
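; Activate-Hover-Mode is a trigger actor Blueprint that switches the player into hover mode.
; It overrides Trigger Action, running the parent logic, then setting the player's HoverMode flag and collapsing the HideBoost element in the HUD's StatusInfo.
; The event graph holds only disabled default events, and the construction script just calls its parent.
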(fn `Trigger Action`
  (params (player :type "/Game/Blueprints/Player/BP_Player Object Reference"))
  (`parent.Trigger Action` player)
  (set `/Game/Blueprints/Player/BP_Player.HoverMode` true player)
  (set `Widget.Visibility` "Collapsed" (`/Game/Widgets/StatusInfo.HideBoost` (`/Game/Widgets/WBP_PlayerHUD.StatusInfo` (`/Game/Blueprints/Player/BP_Player.HUD` player)))))

(fn `UserConstructionScript`
  (`parent.UserConstructionScript`))
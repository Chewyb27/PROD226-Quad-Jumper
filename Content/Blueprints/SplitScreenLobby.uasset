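; Split-screen lobby logic that readies local players in kit selection wheels and launches the match.
; BeginPlay creates extra local players if the level name contains "split".
; Checkifready counts ready players and starts a timeline countdown, which updates each wheel's display and stops if someone unreadies.
; On finish it shows a loading screen, saves the player count to the Loadout save, removes extra players and opens the saved level.
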(event `self.ReceiveBeginPlay`
  (bind _returnvalue (`GameplayStatics.GetCurrentLevelName` true))
  (if (`KismetStringLibrary.Contains` _returnvalue "split")
    (for _ (range 3)
      (`GameplayStatics.CreatePlayer` -1))))

(event `Check if ready`
  (set `self.Number of Players` 0)
  (bind _foundwidgets (`WidgetBlueprintLibrary.GetAllWidgetsOfClass` "/Game/Widgets/KitSelectionWheel.KitSelectionWheel_C"))
  (set `self.Ready to play` true)
  (for _array_element _foundwidgets
    (if (`/Game/Widgets/KitSelectionWheel.JoinedGame` _array_element)
      (if (`/Game/Widgets/KitSelectionWheel.Ready` _array_element)
        (set `self.Number of Players` (+ (`self.Number of Players`) 1))
        (else
          (set `self.Ready to play` false)))))
  (if (`self.Ready to play`)
    (bind (_direction _newtrack_0) (`Timeline|Countdown` :!via `PlayFromStart` :!label _label)
      (:`Update`
        (`self.Countdown Step` _foundwidgets (`KismetMathLibrary.FTrunc` _newtrack_0))
        (if (not (`self.Ready to play`))
          (goto _label :!via `Stop`)))
      (:`Finished`
        (bind _returnvalue (`|CreateWidget` "/Game/Widgets/Loading_Screen.Loading_Screen_C"))
        (`UserWidget.AddToViewport` _returnvalue 0)
        (bind _returnvalue_2 (`GameplayStatics.LoadGameFromSlot` "Loadout"))
        (bind _asloadout_settings (cast `/Game/Savegames/LoadoutSettings` _returnvalue_2))
        (set `/Game/Savegames/LoadoutSettings.playernum` (`self.Number of Players`) _asloadout_settings)
        (`GameplayStatics.SaveGameToSlot` _asloadout_settings "Loadout")
        (`KismetSystemLibrary.Delay` 0.2)
        (bind _outactors (`GameplayStatics.GetAllActorsOfClass` "/Script/Engine.PlayerController"))
        (for (_array_element_2 _array_index) _outactors
          (if (!= _array_index 0)
            (`GameplayStatics.RemovePlayer` _array_element_2 true)))
        (`GameplayStatics.OpenLevelBySoftObjectPtr` (`/Game/Savegames/LoadoutSettings.Level Reference` _asloadout_settings))))))

(fn `Countdown Step`
  (params (InputPin :type "Array of /Game/Widgets/KitSelectionWheel Object Reference") (Value :type Integer))
  (for (_array_element _array_index) InputPin
    (if (or (`/Game/Widgets/KitSelectionWheel.JoinedGame` _array_element) (== _array_index 0))
      (if (not (`/Game/Widgets/KitSelectionWheel.Ready` _array_element))
        (set `self.Ready to play` false))))
  (for _array_element_2 InputPin
    (`Widget.SetVisibility` (`/Game/Widgets/KitSelectionWheel.StartingCountdownBox` _array_element_2) (select `bool` (and (`self.Ready to play`) (`/Game/Widgets/KitSelectionWheel.JoinedGame` _array_element_2)) :`false` "Collapsed" :`true` "Visible" :!type "ESlateVisibility Enum"))
    (set `TextBlock.Text` (`KismetTextLibrary.Conv_IntToText` Value) (`/Game/Widgets/KitSelectionWheel.StartingCountdownNumber` _array_element_2))))

(fn `UserConstructionScript`)
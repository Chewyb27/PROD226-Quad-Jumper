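; Learning Agents trainer that rewards BP_P08A agents for navigating toward the AI_Target actor.
; A planar distance penalty, thresholded by the manager-to-target distance at setup, combines with a small speed reward, both fed from each agent's MainBoxComponent.
; SetCompletions prints agent speed and flags MoveFail when nearly stationary, but that completion's creation is disconnected, leaving it unassigned.
; Episode reset is empty.
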(event `self.ReceiveBeginPlay`
  (`GameplayStatics.GetActorOfClass` "/Game/Blueprints/Player/AI/AI_Target.AI_Target_C"))

(event `self.SetupRewards`
  (bind _returnvalue (`GameplayStatics.GetActorOfClass` "/Game/Blueprints/Player/AI/learning_agents/BP_MechTrainingManager.BP_MechTrainingManager_C"))
  (bind _returnvalue_2 (`GameplayStatics.GetActorOfClass` "/Game/Blueprints/Player/AI/AI_Target.AI_Target_C"))
  (set `self.Target` _returnvalue_2)
  (`|ExecutionSequence`
    (:`then_0`
      (bind _returnvalue_3 (`PlanarPositionDifferencePenalty.AddPlanarPositionDifferencePenalty` null "DistanceFromTargetPenalty" 1.0 100.0 (`KismetMathLibrary.Vector_Distance` (* (`Actor.K2_GetActorLocation` _returnvalue) (1.0 1.0 0.0)) (* (`Actor.K2_GetActorLocation` _returnvalue_2) (1.0 1.0 0.0)))))
      (set `self.Distance Penalty` _returnvalue_3))
    (:`then_1`
      (bind _returnvalue_4 (`ScalarVelocityReward.AddScalarVelocityReward` null "SpeedReward" 0.1))
      (set `self.SpeedReward` _returnvalue_4))))

(event `self.SetRewards`
  (params (AgentIds :type "Array of Integer (by ref)"))
  (for _array_element AgentIds
    (`|ExecutionSequence`
      (:`then_0`
        (bind _main_box_component (`/Game/Blueprints/Player/BP_Player.Main Box Component` (`self.GetAgent` _array_element "/Game/Blueprints/Player/AI/learning_agents/BP_P-08A.BP_P-08A_C")))
        (`PlanarPositionDifferencePenalty.SetPlanarPositionDifferencePenalty` (`self.Distance Penalty`) _array_element (`SceneComponent.K2_GetComponentLocation` _main_box_component) (`Actor.K2_GetActorLocation` (`self.Target`))))
      (:`then_1`
        (`ScalarVelocityReward.SetScalarVelocityReward` (`self.SpeedReward`) _array_element (`KismetMathLibrary.VSize` (`SceneComponent.GetComponentVelocity` _main_box_component)))))))

(event `self.SetCompletions`
  (params (AgentIds :type "Array of Integer (by ref)"))
  (for _array_element AgentIds
    (bind _returnvalue (`KismetMathLibrary.VSize` (`Actor.GetVelocity` (`self.GetAgent` _array_element "/Game/Blueprints/Player/AI/learning_agents/BP_P-08A.BP_P-08A_C"))))
    (`KismetSystemLibrary.PrintString` (`KismetStringLibrary.Conv_DoubleToString` _returnvalue))
    (`ConditionalCompletion.SetConditionalCompletion` (`self.MoveFail`) _array_element (< _returnvalue 1.0))))

(event `self.SetupCompletions`)
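; Learning Agents manager that spawns BP_P08A mechs and sets up a navigation interactor, policy, trainer, recorder and controller.
; Each tick it copies every mech's movement, aim, boost, jump and roll values into float actions, then encodes observations and actions and feeds them to the recorder as demonstration experience.
; RunTraining and the timed loop that relocates the AI_Target, records and saves are disconnected, so neither training nor recording is started here.
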(event `self.ReceiveBeginPlay`
  (for _ (range (+ (`self.Agent Number`) 1))
    (`|SpawnActorFromClass` "/Game/Blueprints/Player/AI/learning_agents/BP_P-08A.BP_P-08A_C" (`KismetMathLibrary.MakeTransform` (`self.K2_GetActorLocation`) (`self.K2_GetActorRotation`)) "AdjustIfPossibleButAlwaysSpawn" "MultiplyWithRoot" null null))
  (bind _returnvalue (`GameplayStatics.GetActorOfClass` "/Game/Blueprints/Player/AI/AI_Target.AI_Target_C"))
  (set `self.Target` _returnvalue)
  (`|ExecutionSequence`
    (:`then_0`
      (`LearningAgentsInteractor.SetupInteractor` (`self.BP_Navinteractor`))
      (`LearningAgentsPolicy.SetupPolicy` (`self.BP_NavPolicy`) (`self.BP_Navinteractor`) (`self.Policy Settings`) "/Game/Blueprints/Player/AI/learning_agents/DA_NavNetwork.DA_NavNetwork")
      (`LearningAgentsTrainer.SetupTrainer` (`self.BP_NavTrainer`) (`self.BP_Navinteractor`) (`self.BP_NavPolicy`) null (`self.Trainer Settings`)))
    (:`then_1`
      (`LearningAgentsRecorder.SetupRecorder` (`self.NavRecorder`) (`self.BP_Navinteractor`) (`self.Recorder Path Settings`) "/Game/Blueprints/Player/AI/learning_agents/NavRecording2.NavRecording2")
      (`LearningAgentsController.SetupController` (`self.NavController`) (`self.BP_Navinteractor`)))))

(event `self.ReceiveTick`
  (params (DeltaSeconds :type "Float (single-precision)"))
  (bind _bp_navinteractor (`self.BP_Navinteractor`))
  (bind (_outagents _outagentids) (`self.GetAllAgents` "/Game/Blueprints/Player/AI/learning_agents/BP_P-08A.BP_P-08A_C"))
  (for _array_element _outagentids
    (bind _returnvalue (`self.GetAgent` _array_element "/Game/Blueprints/Player/AI/learning_agents/BP_P-08A.BP_P-08A_C"))
    (set `self.Recording Agent` _returnvalue)
    (`FloatAction.SetFloatAction` (`/Game/Blueprints/Player/AI/learning_agents/BP_Navinteractor.MoveForwardAction` _bp_navinteractor) _array_element (`/Game/Blueprints/Player/BP_Player.Forward Speed` _returnvalue))
    (`FloatAction.SetFloatAction` (`/Game/Blueprints/Player/AI/learning_agents/BP_Navinteractor.TurnAction` _bp_navinteractor) _array_element (`/Game/Blueprints/Player/BP_Player.AI Turn` _returnvalue))
    (`FloatAction.SetFloatAction` (`/Game/Blueprints/Player/AI/learning_agents/BP_Navinteractor.LookUpAction` _bp_navinteractor) _array_element (`/Game/Blueprints/Player/BP_Player.AI Pitch` _returnvalue))
    (`FloatAction.SetFloatAction` (`/Game/Blueprints/Player/AI/learning_agents/BP_Navinteractor.StrafeAction` _bp_navinteractor) _array_element (`/Game/Blueprints/Player/BP_Player.Strafe Speed` _returnvalue))
    (`FloatAction.SetFloatAction` (`/Game/Blueprints/Player/AI/learning_agents/BP_Navinteractor.BoostAction` _bp_navinteractor) _array_element (`/Game/Blueprints/Player/BP_Player.AI Boost Axis` _returnvalue))
    (`FloatAction.SetFloatAction` (`/Game/Blueprints/Player/AI/learning_agents/BP_Navinteractor.JumpAction` _bp_navinteractor) _array_element (`/Game/Blueprints/Player/BP_Player.Jump Axis` _returnvalue))
    (`FloatAction.SetFloatAction` (`/Game/Blueprints/Player/AI/learning_agents/BP_Navinteractor.RollAction` _bp_navinteractor) _array_element (* (`/Game/Blueprints/Player/BP_Player.CurrentRollSpeed` _returnvalue) -1.0)))
  (`LearningAgentsInteractor.EncodeObservations` (`self.BP_Navinteractor`))
  (`LearningAgentsController.EncodeActions` (`self.NavController`))
  (`LearningAgentsRecorder.AddExperience` (`self.NavRecorder`)))

(fn `UserConstructionScript`)
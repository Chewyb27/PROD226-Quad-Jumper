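; Learning Agents interactor that defines how BP_P08A agents sense and act for machine-learned control.
; Observes enemy target position relative to the agent's main box, wall trace distances, and boost and grapple meters.
; Float actions drive each pawn's movement, turn, strafe, boost, jump, grapple, roll and look-up functions.
; The jump action reuses the "TurnAction" name, and look-up reads agent ID -1 instead of the looped agent.
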(event `self.SetupActions`
  (`|ExecutionSequence`
    (:`then_0`
      (bind _returnvalue (`FloatAction.AddFloatAction` null "ForwardAction" 10.0))
      (set `self.MoveForwardAction` _returnvalue))
    (:`then_1`
      (bind _returnvalue_2 (`FloatAction.AddFloatAction` null "TurnAction"))
      (set `self.TurnAction` _returnvalue_2))
    (:`then_2`
      (bind _returnvalue_3 (`FloatAction.AddFloatAction` null "StrafeAction"))
      (set `self.StrafeAction` _returnvalue_3))
    (:`then_3`
      (bind _returnvalue_4 (`FloatAction.AddFloatAction` null "BoostAction"))
      (set `self.BoostAction` _returnvalue_4))
    (:`then_4`
      (bind _returnvalue_5 (`FloatAction.AddFloatAction` null "TurnAction"))
      (set `self.JumpAction` _returnvalue_5))
    (:`then_5`
      (bind _returnvalue_6 (`FloatAction.AddFloatAction` null "GrappleAction"))
      (set `self.GrappleAction` _returnvalue_6))
    (:`then_6`
      (bind _returnvalue_7 (`FloatAction.AddFloatAction` null "RollAction"))
      (set `self.RollAction` _returnvalue_7))
    (:`then_7`
      (bind _returnvalue_8 (`FloatAction.AddFloatAction` null "LookUp"))
      (set `self.LookUpAction` _returnvalue_8))))

(event `self.SetupObservations`
  (bind _returnvalue (`PositionObservation.AddPositionObservation` null "Target Location" 100000.0))
  (set `self.Target Location Observation` _returnvalue)
  (bind _returnvalue_2 (`FloatArrayObservation.AddFloatArrayObservation` null "WallDistances" 10))
  (set `self.WallDistances` _returnvalue_2)
  (bind _returnvalue_3 (`FloatObservation.AddFloatObservation` null "BoostBar"))
  (set `self.Boostbar` _returnvalue_3)
  (bind _returnvalue_4 (`FloatObservation.AddFloatObservation` null "GrappleBar"))
  (set `self.GrappleBar` _returnvalue_4))

(event `self.GetActions`
  (params (AgentIds :type "Array of Integer (by ref)"))
  (for _array_element AgentIds
    (`|ExecutionSequence`
      (:`then_0`
        (bind _returnvalue (`FloatAction.GetFloatAction` (`self.MoveForwardAction`) _array_element))
        (bind _returnvalue_2 (`self.GetAgent` _array_element "/Game/Blueprints/Player/AI/learning_agents/BP_P-08A.BP_P-08A_C"))
        (`/Game/Blueprints/Player/BP_Player.MoveForward` _returnvalue_2 _returnvalue))
      (:`then_1`
        (bind _returnvalue_3 (`FloatAction.GetFloatAction` (`self.TurnAction`) _array_element))
        (`/Game/Blueprints/Player/BP_Player.Turn Left/Right` _returnvalue_2 _returnvalue_3))
      (:`then_2`
        (bind _returnvalue_4 (`FloatAction.GetFloatAction` (`self.StrafeAction`) _array_element))
        (`/Game/Blueprints/Player/BP_Player.AI Strafe` _returnvalue_2 _returnvalue_4))
      (:`then_3`
        (bind _returnvalue_5 (`FloatAction.GetFloatAction` (`self.BoostAction`) _array_element))
        (`/Game/Blueprints/Player/BP_Player.AI Boost` _returnvalue_2 _returnvalue_5))
      (:`then_4`
        (bind _returnvalue_6 (`FloatAction.GetFloatAction` (`self.JumpAction`) _array_element))
        (`/Game/Blueprints/Player/BP_Player.AI Jump` _returnvalue_2 _returnvalue_6))
      (:`then_5`
        (bind _returnvalue_7 (`FloatAction.GetFloatAction` (`self.GrappleAction`) _array_element))
        (`/Game/Blueprints/Player/BP_Player.AI Grapple` _returnvalue_2 _returnvalue_7))
      (:`then_6`
        (bind _returnvalue_8 (`FloatAction.GetFloatAction` (`self.RollAction`) _array_element))
        (`/Game/Blueprints/Player/BP_Player.AI Roll` _returnvalue_2 _returnvalue_8))
      (:`then_7`
        (bind _returnvalue_9 (`FloatAction.GetFloatAction` (`self.LookUpAction`) -1))
        (`/Game/Blueprints/Player/BP_Player.Look Up/Down` _returnvalue_2 _returnvalue_9)))))

(event `self.SetObservations`
  (params (AgentIds :type "Array of Integer (by ref)"))
  (for _array_element AgentIds
    (bind _returnvalue (`self.GetAgent` _array_element "/Game/Blueprints/Player/AI/learning_agents/BP_P-08A.BP_P-08A_C"))
    (bind _main_box_component (`/Game/Blueprints/Player/BP_Player.Main Box Component` _returnvalue))
    (`PositionObservation.SetPositionObservation` (`self.Target Location Observation`) _array_element (`/Game/Blueprints/Player/BP_Player.Enemy Target Location` _returnvalue) (`SceneComponent.K2_GetComponentLocation` _main_box_component) (`SceneComponent.K2_GetComponentRotation` _main_box_component))
    (`FloatArrayObservation.SetFloatArrayObservation` (`self.WallDistances`) _array_element (`/Game/Blueprints/Player/BP_Player.AI Trace Distances` _returnvalue))
    (`FloatObservation.SetFloatObservation` (`self.Boostbar`) _array_element (`/Game/Blueprints/Player/BP_Player.BoostAmount` _returnvalue))
    (`FloatObservation.SetFloatObservation` (`self.GrappleBar`) _array_element (`/Game/Blueprints/Player/BP_Player.GrappleRemaining` _returnvalue))))
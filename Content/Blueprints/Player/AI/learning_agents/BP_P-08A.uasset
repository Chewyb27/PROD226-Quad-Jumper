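; BP_P-08A is an AI-trained variant of a player pawn that registers itself as a Learning Agents agent.
; On BeginPlay it runs AISetup, calls the parent, then adds itself to the level's LearningAgentsManager and stores the AgentId, printing a warning if none exists.
; Tick runs AITracking and the parent tick, then prints ForwardAxis for debugging.
; Direct movement calls and RunOnLocal are present but unconnected.
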(event `self.ReceiveBeginPlay`
  ;[1 1 1] Register agents with Manager
  (`self.AI Setup`)
  (`parent.ReceiveBeginPlay`)
  (bind _returnvalue (`GameplayStatics.GetActorOfClass` "/Script/LearningAgents.LearningAgentsManager"))
  (`/Engine/EditorBlueprintResources/StandardMacros.IsValid` _returnvalue
    (:`Is Valid`
      (bind _returnvalue_2 (`LearningAgentsManager.AddAgent` _returnvalue self))
      (set `self.AgentId` _returnvalue_2))
    (:`Is Not Valid`
      (`KismetSystemLibrary.PrintString` "Could not find Learning Agents manager. Did we forget to add one to the scene?"))))

(event `self.ReceiveTick`
  (params (DeltaSeconds :type "Float (single-precision)"))
  (`self.AI Tracking`)
  (`parent.ReceiveTick` DeltaSeconds)
  (`KismetSystemLibrary.PrintString` (`KismetStringLibrary.Conv_DoubleToString` (`self.Forward Axis`))))

(fn `UserConstructionScript`
  (`parent.UserConstructionScript`))
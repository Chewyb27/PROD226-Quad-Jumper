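; AI-driven P-08X player variant that learns to navigate through neuroevolution, steering with a single layer of six sigmoid neurons.
; Periodically, line-trace distances, target alignment and up vector feed the neurons; the strongest output sets turn or elevation.
; BeginPlay takes random weights, or mutates Training_Manager's best (interpolated, score-averaged or picked from the top three).
; Tick applies movement and scores accumulated travel plus displacement; wall and goal terms are zero.
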(event `Run Neural Network`
  (bind _aistruct_ai_weight (break `/Game/Blueprints/Player/AI/AI_Struct` (`self.AIStruct`)))
  (bind (_neuron1 _neuron2 _neuron3 _neuron4 _neuron5 _neuron6) (break `/Game/Blueprints/Player/AI/AI_Weight_Struct` _aistruct_ai_weight))
  (`self.GetData`)
  (bind _probability (`self.Run General Neuron` _neuron1))
  (bind _probability_2 (`self.Run General Neuron` _neuron2))
  (bind _probability_3 (`self.Run General Neuron` _neuron3))
  (bind _probability_4 (`self.Run General Neuron` _neuron4))
  (bind _probability_5 (`self.Run General Neuron` _neuron5))
  (bind _probability_6 (`self.Run General Neuron` _neuron6))
  (switch `int` (`KismetMathLibrary.MaxOfFloatArray` (`|MakeArray` _probability _probability_2 _probability_3 _probability_4 _probability_5 _probability_6 :!type "Float (single-precision)"))
    (:`0`
      (set `self.Turn Override` 1.0)
      (set `self.Elevation Override` 0.0))
    (:`1`
      (set `self.Turn Override` 0.0)
      (set `self.Elevation Override` 0.0))
    (:`2`
      (set `self.Turn Override` -1.0)
      (set `self.Elevation Override` 0.0))
    (:`3`
      (set `self.Elevation Override` 1.0)
      (set `self.Turn Override` 0.0))
    (:`4`
      (set `self.Elevation Override` 0.0)
      (set `self.Turn Override` 0.0))
    (:`5`
      (set `self.Elevation Override` -1.0)
      (set `self.Turn Override` 0.0))))

(event `self.ReceiveBeginPlay`
  (`parent.ReceiveBeginPlay`)
  (bind _returnvalue (`GameplayStatics.GetActorOfClass` "/Game/Blueprints/Player/AI/AI_Target.AI_Target_C"))
  (set `self.AI Target` _returnvalue)
  (`self.Weight System`)
  (bind _output_get (set `self.Start Location` (`SceneComponent.K2_GetComponentLocation` (`self.Main Box Component`))))
  (set `self.Origin Location` _output_get))

(event `self.ReceiveTick`
  (params (DeltaSeconds :type "Float (single-precision)"))
  (bind _returnvalue (+ 0 0))
  (bind _neural_network_period (`self.Neural Network Period`))
  (bind _main_box_component (`self.Main Box Component`))
  (bind _main_box_component_2 (`self.Main Box Component`))
  (bind _aistruct_ai_weight (break `/Game/Blueprints/Player/AI/AI_Struct` (`self.AIStruct`)))
  (bind _returnvalue_2 (`KismetMathLibrary.SelectInt` 0 0 (`self.Onglass`)))
  (bind _returnvalue_3 (`SceneComponent.K2_GetComponentLocation` (`self.Main Box Component`)))
  (bind _returnvalue_4 (`KismetMathLibrary.FTrunc` (* (`self.Displacement`) 10.0)))
  (bind _returnvalue_5 (`KismetMathLibrary.FTrunc` (/ (`self.Amount Moved`) 30.0)))
  (bind _returnvalue_6 (+ _returnvalue_2 _returnvalue_5 _returnvalue_4 _returnvalue))
  (`|ExecutionSequence`
    (:`then_0`
      (`self.MoveForward` (`self.Forward Override`))
      (`self.Turn Left/Right` (`self.Turn Override`))
      (`self.Look Up/Down` (`self.Elevation Override`))
      (`self.Run On Local` DeltaSeconds))
    (:`then_1`
      (set `self.Amount Moved` (+ (`KismetMathLibrary.Vector_Distance` (`self.Start Location`) _returnvalue_3) (`self.Amount Moved`)))
      (set `self.Start Location` _returnvalue_3)
      (set `self.Displacement` (`KismetMathLibrary.Vector_Distance` _returnvalue_3 (`self.Origin Location`)))
      (set `self.AIStruct` (make `/Game/Blueprints/Player/AI/AI_Struct` _aistruct_ai_weight _returnvalue_6))
      (`KismetSystemLibrary.PrintString` (`KismetStringLibrary.Concat_StrStr` "On wall: " (`KismetStringLibrary.Conv_IntToString` _returnvalue_2) " Amount Moved: " (`KismetStringLibrary.Conv_IntToString` _returnvalue_5) " Displacement: " (`KismetStringLibrary.Conv_IntToString` _returnvalue_4) " Distance from goal: " (`KismetStringLibrary.Conv_IntToString` _returnvalue) " Total: " (`KismetStringLibrary.Conv_IntToString` _returnvalue_6)) true true (struct :`R` 1.0 :`G` 0.473817 :`A` 1.0) DeltaSeconds))
    (:`then_2`
      (set `self.Target Dot Product` (`KismetMathLibrary.Dot_VectorVector` (`SceneComponent.GetForwardVector` _main_box_component_2) (`KismetMathLibrary.Normal` (- (`self.K2_GetActorLocation` (`self.AI Target`)) (`SceneComponent.K2_GetComponentLocation` _main_box_component_2)))))
      (set `self.Up Vector` (`SceneComponent.GetUpVector` _main_box_component_2))
      (bind _output_get (set `self.Target Left Right` (* (`KismetMathLibrary.Dot_VectorVector` (`KismetMathLibrary.Cross_VectorVector` (`SceneComponent.GetForwardVector` _main_box_component) (`SceneComponent.GetUpVector` _main_box_component)) (`KismetMathLibrary.Normal` (- (`self.K2_GetActorLocation` (`self.AI Target`)) (`SceneComponent.K2_GetComponentLocation` _main_box_component)))) 10000.0))))
    (:`then_3`
      (if (>= _neural_network_period (`self.Neural Network Max Period`))
        (`self.Run Neural Network`)
        (set `self.Neural Network Period` 0.0)
        (else
          (set `self.Neural Network Period` (+ _neural_network_period DeltaSeconds)))))))

(event `GetData`
  (bind _distance (`self.LineTrace` (`self.Arrow`)))
  (set `self.Forward Distance` _distance)
  (bind _distance_2 (`self.LineTrace` (`self.Arrow1`)))
  (set `self.45 Distance` _distance_2)
  (bind _distance_3 (`self.LineTrace` (`self.Arrow2`)))
  (set `self.90 Distance` _distance_3)
  (bind _distance_4 (`self.LineTrace` (`self.Arrow3`)))
  (set `self.-45 Distance` _distance_4)
  (bind _distance_5 (`self.LineTrace` (`self.Arrow4`)))
  (set `self.-90 Distance` _distance_5)
  (bind _distance_6 (`self.LineTrace` (`self.Arrow5`)))
  (set `self.Down Distance` _distance_6))

(event `Weight System`
  (bind _returnvalue (`GameplayStatics.GetActorOfClass` "/Game/Blueprints/Player/AI/Training_Manager.Training_Manager_C"))
  (if (`/Game/Blueprints/Player/AI/Training_Manager.Best_AI_Found` _returnvalue)
    (bind _new (`self.Update Weight` (select `bool` (`self.Use History`) :`false` (`/Game/Blueprints/Player/AI/Training_Manager.Best_AI_List` _returnvalue) :`true` (`/Game/Blueprints/Player/AI/Training_Manager.Best History` _returnvalue)) (`/Game/Blueprints/Player/AI/Training_Manager.Interpolated Best` _returnvalue)))
    (set `self.AIStruct` (make `/Game/Blueprints/Player/AI/AI_Struct` _new))
    (else
      (bind _weight (`self.Random Weight`))
      (set `self.AIStruct` (make `/Game/Blueprints/Player/AI/AI_Struct` _weight)))))

(fn `Alignment Neuron`
  (params (`Down Input` :type "Float (double-precision)") (`Weight 1` :type "Float (double-precision)") (`Input 2` :type "Float (double-precision)") (`Weight 2` :type "Float (double-precision)") (`Input 3` :type "Float (double-precision)") (`Weight 3` :type "Float (double-precision)") (`Input 4` :type "Float (double-precision)") (`Weight 4` :type "Float (double-precision)") (`Input 5` :type "Float (double-precision)") (`Weight 5` :type "Float (double-precision)") (`Input 6` :type "Float (double-precision)") (`Weight 6` :type "Float (double-precision)"))
  (returns (Probability :type "Float (double-precision)"))
  (bind _output (`self.Sigmoid` (/ (+ (* `Down Input` `Weight 1`) (* `Input 2` `Weight 2`) (* `Input 3` `Weight 3`) (* `Input 4` `Weight 4`) (* `Input 5` `Weight 5`) (* `Input 6` `Weight 6`)) 100.0)))
  (return _output))

(fn `General Nav Neuron`
  (params (`Forward Distance` :type "Float (double-precision)") (`Weight 1` :type "Float (double-precision)") (`45 Distance` :type "Float (double-precision)") (`Weight 2` :type "Float (double-precision)") (`90 Distance` :type "Float (double-precision)") (`Weight 3` :type "Float (double-precision)") (`-45 Distance` :type "Float (double-precision)") (`Weight 4` :type "Float (double-precision)") (`-90 Distance` :type "Float (double-precision)") (`Weight 5` :type "Float (double-precision)") (`Down Distance` :type "Float (double-precision)") (`Weight 6` :type "Float (double-precision)") (`Target Dot Product` :type "Float (double-precision)") (`Weight 7` :type "Float (double-precision)") (`Up X` :type "Float (double-precision)") (`Weight 8` :type "Float (double-precision)") (`Up Y` :type "Float (double-precision)") (`Weight 9` :type "Float (double-precision)") (`Up Z` :type "Float (double-precision)") (`Weight 10` :type "Float (double-precision)") (`Target Left Right` :type "Float (double-precision)") (`Weight 11` :type "Float (double-precision)"))
  (returns (Probability :type "Float (double-precision)"))
  (bind _output (`self.Sigmoid` (/ (+ (* `Forward Distance` `Weight 1`) (* `45 Distance` `Weight 2`) (* `90 Distance` `Weight 3`) (* `-45 Distance` `Weight 4`) (* `-90 Distance` `Weight 5`) (* `Down Distance` `Weight 6`) (* `Target Dot Product` `Weight 7`) (* `Up X` `Weight 8`) (* `Up Y` `Weight 9`) (* `Up Z` `Weight 10`)) 100.0)))
  (return _output))

(fn `LineTrace`
  (params (Object :type "PrimitiveComponent Object Reference"))
  (returns (Distance :type "Float (double-precision)") (Normal :type "Vector Structure"))
  (bind _returnvalue (`SceneComponent.K2_GetComponentLocation` Object))
  (bind _outhit (`KismetSystemLibrary.LineTraceSingle` :`Start` _returnvalue :`End` (+ _returnvalue (* (`SceneComponent.GetForwardVector` Object) 10000.0)) :`TraceChannel` "TraceTypeQuery1" :`DrawTime` 0.1))
  (bind (_bblockinghit _binitialoverlap _time _distance _location _impactpoint _normal _impactnormal) (`GameplayStatics.BreakHitResult` _outhit))
  (return _distance _impactnormal))

(fn `Random Weight`
  (returns (Weight :type "/Game/Blueprints/Player/AI/AI_Weight_Struct Structure"))
  (return (make `/Game/Blueprints/Player/AI/AI_Weight_Struct` (`self.Random Neuron Weight`) (`self.Random Neuron Weight`) (`self.Random Neuron Weight`) (`self.Random Neuron Weight`) (`self.Random Neuron Weight`) (`self.Random Neuron Weight`))))

(fn `Run General Neuron`
  (params (Nav_Neuron_Weights :type "/Game/Blueprints/Player/AI/Nav_Neuron_Weights Structure (by ref)"))
  (returns (Probability :type "Float (double-precision)"))
  (bind (_forwardweight _45weight _90weight __45weight __90weight _downweight _targetdotweight _upxweight _upyweight _upzweight _targetleftrightweight) (break `/Game/Blueprints/Player/AI/Nav_Neuron_Weights` Nav_Neuron_Weights))
  (bind (_x _y _z) (`KismetMathLibrary.BreakVector3f` (`self.Up Vector`)))
  (bind _probability (`self.General Nav Neuron` (`self.Forward Distance`) _forwardweight (`self.45 Distance`) _45weight (`self.90 Distance`) _90weight (`self.-45 Distance`) __45weight (`self.-90 Distance`) __90weight (`self.Down Distance`) _downweight (`self.Target Dot Product`) _targetdotweight _x _upxweight _y _upyweight _z _upzweight (`self.Target Left Right`) _targetleftrightweight))
  (return _probability))

(fn `Sigmoid`
  (params (Value :type "Float (double-precision)"))
  (returns (Output :type "Float (double-precision)"))
  (return (/ 1.0 (+ (`KismetMathLibrary.Exp` Value) 1.0))))

(fn `Update Weight`
  (params (`Best AI List` :type "/Game/Blueprints/Player/AI/Best_AI_List Structure") (Interp :type "/Game/Blueprints/Player/AI/AI_Struct Structure"))
  (returns (New :type "/Game/Blueprints/Player/AI/AI_Weight_Struct Structure"))
  (bind (_bestai1 _bestai2 _bestai3) (break `/Game/Blueprints/Player/AI/Best_AI_List` `Best AI List`))
  (bind (_ai_weight _ai_score) (break `/Game/Blueprints/Player/AI/AI_Struct` _bestai1))
  (bind (_ai_weight_2 _ai_score_2) (break `/Game/Blueprints/Player/AI/AI_Struct` _bestai3))
  (bind (_ai_weight_3 _ai_score_3) (break `/Game/Blueprints/Player/AI/AI_Struct` _bestai2))
  (bind (_neuron1 _neuron2 _neuron3 _neuron4 _neuron5 _neuron6) (break `/Game/Blueprints/Player/AI/AI_Weight_Struct` (select `bool` (`self.Use Interpolated Weights`) :`false` (select `bool` (`self.Use Average Top Weights`) :`false` (break `/Game/Blueprints/Player/AI/AI_Struct` (`KismetArrayLibrary.Array_Random` (`|MakeArray` _bestai1 _bestai2 _bestai3))) :`true` (make `/Game/Blueprints/Player/AI/AI_Weight_Struct` (`self.Average Weights for 1 Neuron` (break `/Game/Blueprints/Player/AI/AI_Weight_Struct` _ai_weight) (break `/Game/Blueprints/Player/AI/AI_Weight_Struct` _ai_weight_3) (break `/Game/Blueprints/Player/AI/AI_Weight_Struct` _ai_weight_2) _ai_score _ai_score_3 _ai_score_2) (`self.Average Weights for 1 Neuron` (`.Neuron2_80_EF4E38EB4615A69FC08CFFA22187AE8A` (break `/Game/Blueprints/Player/AI/AI_Weight_Struct` _ai_weight)) (`.Neuron2_80_EF4E38EB4615A69FC08CFFA22187AE8A` (break `/Game/Blueprints/Player/AI/AI_Weight_Struct` _ai_weight_3)) (`.Neuron2_80_EF4E38EB4615A69FC08CFFA22187AE8A` (break `/Game/Blueprints/Player/AI/AI_Weight_Struct` _ai_weight_2)) _ai_score _ai_score_3 _ai_score_2) (`self.Average Weights for 1 Neuron` (`.Neuron3_81_7A4E4E4C43B783D9AD35B3947891F5BC` (break `/Game/Blueprints/Player/AI/AI_Weight_Struct` _ai_weight)) (`.Neuron3_81_7A4E4E4C43B783D9AD35B3947891F5BC` (break `/Game/Blueprints/Player/AI/AI_Weight_Struct` _ai_weight_3)) (`.Neuron3_81_7A4E4E4C43B783D9AD35B3947891F5BC` (break `/Game/Blueprints/Player/AI/AI_Weight_Struct` _ai_weight_2)) _ai_score _ai_score_3 _ai_score_2) (`self.Average Weights for 1 Neuron` (`.Neuron4_82_80C177944901A8F9CD372AB78EC863A4` (break `/Game/Blueprints/Player/AI/AI_Weight_Struct` _ai_weight)) (`.Neuron4_82_80C177944901A8F9CD372AB78EC863A4` (break `/Game/Blueprints/Player/AI/AI_Weight_Struct` _ai_weight_3)) (`.Neuron4_82_80C177944901A8F9CD372AB78EC863A4` (break `/Game/Blueprints/Player/AI/AI_Weight_Struct` _ai_weight_2)) _ai_score _ai_score_3 _ai_score_2) (`self.Average Weights for 1 Neuron` (`.Neuron5_85_4A6FDC8749D97F0313D602808E9163BC` (break `/Game/Blueprints/Player/AI/AI_Weight_Struct` _ai_weight)) (`.Neuron5_85_4A6FDC8749D97F0313D602808E9163BC` (break `/Game/Blueprints/Player/AI/AI_Weight_Struct` _ai_weight_3)) (`.Neuron5_85_4A6FDC8749D97F0313D602808E9163BC` (break `/Game/Blueprints/Player/AI/AI_Weight_Struct` _ai_weight_2)) _ai_score _ai_score_3 _ai_score_2) (`self.Average Weights for 1 Neuron` (`.Neuron6_86_6E8B7A3A440DC048F3BDA5A68844ACF6` (break `/Game/Blueprints/Player/AI/AI_Weight_Struct` _ai_weight)) (`.Neuron6_86_6E8B7A3A440DC048F3BDA5A68844ACF6` (break `/Game/Blueprints/Player/AI/AI_Weight_Struct` _ai_weight_3)) (`.Neuron6_86_6E8B7A3A440DC048F3BDA5A68844ACF6` (break `/Game/Blueprints/Player/AI/AI_Weight_Struct` _ai_weight_2)) _ai_score _ai_score_3 _ai_score_2))) :`true` (`.AI_Weight_2_0F3615DB48E5D3727F8AC8842C7A906B` (break `/Game/Blueprints/Player/AI/AI_Struct` Interp)))))
  (return (make `/Game/Blueprints/Player/AI/AI_Weight_Struct` (`self.Adjust All Values` _neuron1) (`self.Adjust All Values` _neuron2) (`self.Adjust All Values` _neuron3) (`self.Adjust All Values` _neuron4) (`self.Adjust All Values` _neuron5) (`self.Adjust All Values` _neuron6))))

(fn `UserConstructionScript`
  (`parent.UserConstructionScript`))
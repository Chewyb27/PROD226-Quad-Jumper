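; Main-menu mech pawn that previews the player's loadout and opens WBP_MainMenu when play begins.
; Events swap the gun mesh and materials, toggle ability visuals (hover legs, thrusters, shield, friend meshes) and apply colour through dynamic glow and shield materials.
; A SmoothCamera timeline moves the camera between main and top positions while adjusting widget blur.
; Debug keys overwrite the Loadout save: T unlocks techs and levels, R resets progress.
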(event `Refresh Extra Models`
  (params (Ability :type Integer))
  (bind _returnvalue (select `int` Ability :`0` false :`1` false :`2` false :`3` false :`4` true :`5` false :`6` false))
  (bind _returnvalue_2 (select `int` Ability :`0` false :`1` true :`2` false :`3` false :`4` false :`5` false :`6` false))
  (`|ExecutionSequence`
    (:`then_0`
      (if _returnvalue_2
        (for _array_element (`|MakeArray` (`self.Leg_Export_45_LowerLeg6`) (`self.Leg_Export_45_LowerLeg4`) (`self.Leg_Export_45_LowerLeg3`) (`self.Leg_Export_45_LowerLeg5`))
          (`StaticMeshComponent.SetStaticMesh` _array_element (select `bool` _returnvalue_2 :`false` "/Game/Animations/Leg_Export_45_LowerLeg.Leg_Export_45_LowerLeg" :`true` "/Game/Models/PlayerModel/Extra/Hover_Leg_1.Hover_Leg_1" :!type "StaticMesh Object Reference")))))
    (:`then_1`
      (if (select `int` Ability :`0` false :`1` false :`2` false :`3` true :`4` false :`5` false :`6` false)
        (`SceneComponent.SetVisibility` (`self.FriendMesh`) true false)))
    (:`then_2`
      (if (select `int` Ability :`0` false :`1` false :`2` true :`3` false :`4` false :`5` false :`6` false)
        (`SceneComponent.SetVisibility` (`self.Shield`) true false)))
    (:`then_3`
      (if (select `int` Ability :`0` false :`1` false :`2` false :`3` false :`4` false :`5` false :`6` true)
        (`SceneComponent.SetVisibility` (`self.RepairFriendMesh`) true false)))
    (:`then_4`
      (if _returnvalue
        (for _array_element_2 (`|MakeArray` (`self.ThrusterMesh2`) (`self.ThrusterMesh3`) (`self.ThrusterMesh4`) (`self.ThrusterMesh5`))
          (`StaticMeshComponent.SetStaticMesh` _array_element_2 (select `bool` _returnvalue :`false` "/Game/Models/PlayerModel/Extra/Mech_Thruster_2.Mech_Thruster_2" :`true` "/Game/Models/PlayerModel/Extra/Mech_Thruster_3.Mech_Thruster_3" :!type "StaticMesh Object Reference")))))))

(event `Reset Extra Models`
  (params (Item :type Integer))
  (switch `int` Item
    (:`1`
      (for _array_element (`|MakeArray` (`self.Leg_Export_45_LowerLeg6`) (`self.Leg_Export_45_LowerLeg4`) (`self.Leg_Export_45_LowerLeg3`) (`self.Leg_Export_45_LowerLeg5`))
        (`StaticMeshComponent.SetStaticMesh` _array_element (select `bool` false :`false` "/Game/Animations/Leg_Export_45_LowerLeg.Leg_Export_45_LowerLeg" :`true` "/Game/Models/PlayerModel/Extra/Hover_Leg_1.Hover_Leg_1" :!type "StaticMesh Object Reference"))))
    (:`2`
      (`SceneComponent.SetVisibility` (`self.Shield`) false false))
    (:`3`
      (`SceneComponent.SetVisibility` (`self.FriendMesh`) false false))
    (:`4`
      (for _array_element_2 (`|MakeArray` (`self.ThrusterMesh2`) (`self.ThrusterMesh3`) (`self.ThrusterMesh4`) (`self.ThrusterMesh5`))
        (`StaticMeshComponent.SetStaticMesh` _array_element_2 (select `bool` false :`false` "/Game/Models/PlayerModel/Extra/Mech_Thruster_2.Mech_Thruster_2" :`true` "/Game/Models/PlayerModel/Extra/Mech_Thruster_3.Mech_Thruster_3" :!type "StaticMesh Object Reference"))))
    (:`6`
      (`SceneComponent.SetVisibility` (`self.RepairFriendMesh`) false false))))

(event `Refresh Base Mat`
  (params (Colour :type "LinearColor Structure"))
  (bind _main_material (`self.Main Material`))
  (bind _shield_material (`self.Shield Material`))
  (`PrimitiveComponent.SetMaterial` (`self.FrontMesh`) 0 _main_material)
  (`PrimitiveComponent.SetMaterial` (`self.BackMesh`) 1 _main_material)
  (`PrimitiveComponent.SetMaterial` (`self.Leg_Export_45_LowerLeg3`) 3 _main_material)
  (`PrimitiveComponent.SetMaterial` (`self.Leg_Export_45_LowerLeg6`) 3 _main_material)
  (`PrimitiveComponent.SetMaterial` (`self.Leg_Export_45_LowerLeg4`) 3 _main_material)
  (`PrimitiveComponent.SetMaterial` (`self.Leg_Export_45_LowerLeg5`) 3 _main_material)
  (`PrimitiveComponent.SetMaterial` (`self.Leg_Export_45_UpperLeg5`) 1 _main_material)
  (`PrimitiveComponent.SetMaterial` (`self.Leg_Export_45_UpperLeg6`) 1 _main_material)
  (`PrimitiveComponent.SetMaterial` (`self.Leg_Export_45_UpperLeg4`) 1 _main_material)
  (`PrimitiveComponent.SetMaterial` (`self.Leg_Export_45_UpperLeg3`) 1 _main_material)
  (`PrimitiveComponent.SetMaterial` (`self.ThrusterMesh4`) 1 _main_material)
  (`PrimitiveComponent.SetMaterial` (`self.ThrusterMesh3`) 1 _main_material)
  (`PrimitiveComponent.SetMaterial` (`self.ThrusterMesh5`) 1 _main_material)
  (`PrimitiveComponent.SetMaterial` (`self.ThrusterMesh2`) 1 _main_material)
  (`MaterialInstanceDynamic.SetVectorParameterValue` (`self.Glow Material`) "Colour" (* Colour 0.18))
  (`PrimitiveComponent.SetMaterial` (`self.FriendMesh`) 1 _main_material)
  (`PrimitiveComponent.SetMaterial` (`self.RepairFriendMesh`) 1 _main_material)
  (`/Engine/EditorBlueprintResources/StandardMacros.IsValid` _shield_material
    (:`Is Valid`
      (`MaterialInstanceDynamic.SetVectorParameterValue` _shield_material "Fill Tint" Colour))))

(event `Refresh Weapon Mat`
  (bind _gunmesh (`self.GunMesh`))
  (bind _glow_material (`self.Glow Material`))
  (bind _main_material (`self.Main Material`))
  (`PrimitiveComponent.SetMaterial` _gunmesh 0 (select `int` (stale `Set Main Weapon` `Weapon Num`) :`0` "/Game/Materials/Scene/M_BuildingAccent.M_BuildingAccent" :`1` _main_material :`2` "/Game/Materials/Scene/M_BuildingAccent.M_BuildingAccent" :`3` _main_material :`4` "/Game/Materials/Scene/M_BuildingAccent.M_BuildingAccent"))
  (`PrimitiveComponent.SetMaterial` _gunmesh 1 (select `int` (stale `Set Main Weapon` `Weapon Num`) :`0` "/Game/Materials/PlayerMaterials/M_MechExterior.M_MechExterior" :`1` "/Game/Materials/PlayerMaterials/M_MechAccent.M_MechAccent" :`2` _main_material :`3` _glow_material :`4` _main_material :!type "MaterialInterface Object Reference"))
  (`PrimitiveComponent.SetMaterial` _gunmesh 2 (select `int` (stale `Set Main Weapon` `Weapon Num`) :`0` _main_material :`1` _main_material :`2` _glow_material :`3` "/Game/Materials/Scene/M_BuildingAccent.M_BuildingAccent" :`4` _glow_material :!type "MaterialInterface Object Reference"))
  (`PrimitiveComponent.SetMaterial` _gunmesh 3 (select `int` (stale `Set Main Weapon` `Weapon Num`) :`0` _glow_material :`1` _glow_material :`2` _main_material :`3` _main_material :`4` "/Game/Materials/Scene/M_BuildingAccent.M_BuildingAccent" :!type "MaterialInterface Object Reference"))
  (`PrimitiveComponent.SetMaterial` _gunmesh 4 (select `int` (stale `Set Main Weapon` `Weapon Num`) :`0` _main_material :`1` _glow_material :`2` _main_material :`3` _main_material :`4` _main_material :!type "MaterialInterface Object Reference")))

(event `Set Main Weapon`
  (params (`Weapon Num` :type Integer) (Upgraded :type Boolean))
  (bind _gunmesh (`self.GunMesh`))
  (if (== `Weapon Num` -1)
    (`StaticMeshComponent.SetStaticMesh` _gunmesh null)
    (else
      (`StaticMeshComponent.SetStaticMesh` _gunmesh (select `int` `Weapon Num` :`0` "/Game/Models/PlayerModel/Weapons/Quad_Jumper_Weapon_1.Quad_Jumper_Weapon_1" :`1` "/Game/Models/PlayerModel/Weapons/Quad_Jumper_Weapon_Laser.Quad_Jumper_Weapon_Laser" :`2` "/Game/Models/PlayerModel/Weapons/Quad_Jumper_Weapon_Launcher.Quad_Jumper_Weapon_Launcher" :`3` "/Game/Models/PlayerModel/Weapons/Quad_Jumper_Weapon_Railgun.Quad_Jumper_Weapon_Railgun" :`4` "/Game/Models/PlayerModel/Weapons/Quad_Jumper_Weapon_Rockets.Quad_Jumper_Weapon_Rockets" :`5` null :!type "StaticMesh Object Reference"))
      (`self.Refresh Weapon Mat`))))

(event `self.ReceiveTick`
  (params (DeltaSeconds :type "Float (single-precision)"))
  (set `self.Delta` DeltaSeconds))

(event `Switch Camera to Top`
  (params (blur :type "BackgroundBlur Object Reference"))
  (bind _main_position (`self.Main Position`))
  (bind _top_position (`self.Top Position`))
  (bind _cameracomponent (`CameraActor.CameraComponent` (`self.Main Camera`)))
  (set `self.Blur` blur)
  (bind (_direction _newtrack_0) (`Timeline|Smooth Camera` :!label _label)
    (:`Update`
      (`SceneComponent.K2_SetWorldLocation` _cameracomponent (`KismetMathLibrary.VInterpTo` (`self.K2_GetActorLocation` _main_position) (`self.K2_GetActorLocation` _top_position) _newtrack_0 1.0) false false)
      (`SceneComponent.K2_SetWorldRotation` _cameracomponent (`KismetMathLibrary.RInterpTo` (`self.K2_GetActorRotation` _main_position) (`self.K2_GetActorRotation` _top_position) _newtrack_0 1.0) false false)
      (`BackgroundBlur.SetBlurStrength` (`self.Blur`) (- 3.0 (* _newtrack_0 3.0))))))

(event `Key|T`
  (params (Key :type "Key Structure"))
  (bind _savegame (`self.Savegame`))
  (bind _techs (`/Game/Savegames/LoadoutSettings.Techs` _savegame))
  (:`Pressed`
    (bind _returnvalue (`GameplayStatics.CreateSaveGameObject` "/Game/Savegames/LoadoutSettings.LoadoutSettings_C"))
    (set `self.Savegame` _returnvalue)
    (bind _values (`BlueprintMapLibrary.Map_Values` _techs))
    (for _array_element _values
      (bind (_name _icon _description _button _imagebrush _prerequisites _unlocked _childnames _cost _power _type _id) (break `/Game/Widgets/TechStructure` _array_element))
      (`BlueprintMapLibrary.Map_Add` _techs _name (make `/Game/Widgets/TechStructure` _name _icon _description _button _imagebrush _prerequisites true _childnames _cost _power _type _id)))
    (set `/Game/Savegames/LoadoutSettings.Unlocked Levels` 100 _savegame)
    (`GameplayStatics.SaveGameToSlot` _savegame "Loadout")
    (`KismetSystemLibrary.PrintString` "Unlocked Everything")))

(event `Switch Camera to Main`
  (params (Blur :type "BackgroundBlur Object Reference"))
  (set `self.Blur` Blur)
  (goto _label :!via `Reverse`))

(event `Key|R`
  (params (Key :type "Key Structure"))
  (:`Pressed`
    (bind _returnvalue (`GameplayStatics.CreateSaveGameObject` "/Game/Savegames/LoadoutSettings.LoadoutSettings_C"))
    (`GameplayStatics.SaveGameToSlot` _returnvalue "Loadout")
    (`KismetSystemLibrary.PrintString` "Reset Progress")))

(event `self.ReceiveBeginPlay`
  (bind _returnvalue (`GameplayStatics.GetPlayerController` 0))
  (bind _shield (`self.Shield`))
  (bind _returnvalue_2 (`KismetMaterialLibrary.CreateDynamicMaterialInstance` "/Game/Materials/SpecialEffects/MI_Railgun_Glow.MI_Railgun_Glow"))
  (set `self.Glow Material` _returnvalue_2)
  (`MaterialInstanceDynamic.SetVectorParameterValue` (`self.Glow Material`) "Colour" (struct :`R` 0.027282 :`G` 0.2986 :`B` 1.0 :`A` 1.0))
  (`self.Refresh Base Mat` (struct :`R` 0.027282 :`G` 0.2986 :`B` 1.0 :`A` 1.0))
  (`Controller.Possess` _returnvalue self)
  (bind _returnvalue_3 (`|CreateWidget` "/Game/Widgets/WBP_MainMenu.WBP_MainMenu_C" _returnvalue self))
  (bind _output_get (set `self.Menu` _returnvalue_3))
  (`UserWidget.AddToViewport` _output_get 0)
  (set `PlayerController.bShowMouseCursor` true (`GameplayStatics.GetPlayerController` 0))
  (bind _returnvalue_4 (`KismetMaterialLibrary.CreateDynamicMaterialInstance` "/Game/Materials/SpecialEffects/ShieldType2.ShieldType2"))
  (bind _output_get_2 (set `self.Shield Material` _returnvalue_4))
  (`PrimitiveComponent.SetMaterial` _shield 0 _output_get_2)
  (`MeshComponent.SetScalarParameterValueOnMaterials` _shield "Emissive" 0.05)
  (`KismetSystemLibrary.Delay` 0.2)
  (`self.Refresh Base Mat` (struct :`R` 0.027282 :`G` 0.2986 :`B` 1.0 :`A` 1.0))
  (`self.Refresh Weapon Mat`))

(fn `UserConstructionScript`)
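; AirPad is a short-lived visual pad actor that animates its opacity and scale over its lifetime, then destroys itself.
; The construction script creates a dynamic instance of MI_AirPad2, tints it with the Colour variable and applies it to the static mesh.
; On BeginPlay a timeline, rate-scaled so it lasts Life seconds, drives the material's Opacity and the mesh's relative scale until it finishes.
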(event `self.ReceiveBeginPlay`
  (`TimelineComponent.SetPlayRate` (`self.Lifetime`) (/ 1.0 (`self.Life`)))
  (bind (_direction _newtrack_0 _newtrack_1) (`Timeline|Lifetime` :!via `PlayFromStart`)
    (:`Update`
      (`MaterialInstanceDynamic.SetScalarParameterValue` (`self.Material`) "Opacity" _newtrack_0)
      (`SceneComponent.SetRelativeScale3D` (`self.StaticMesh`) (`KismetMathLibrary.Conv_DoubleToVector` _newtrack_1))
      (`SceneComponent.SetRelativeScale3D` (`self.StaticMesh`) (`KismetMathLibrary.Conv_DoubleToVector` _newtrack_1)))
    (:`Finished`
      (`self.K2_DestroyActor`))))

(fn `UserConstructionScript`
  (bind _returnvalue (`KismetMaterialLibrary.CreateDynamicMaterialInstance` "/Game/Materials/SpecialEffects/MI_AirPad2.MI_AirPad2"))
  (set `self.Material` _returnvalue)
  (`MaterialInstanceDynamic.SetVectorParameterValue` _returnvalue "Colour" (`self.Colour`))
  (`PrimitiveComponent.SetMaterial` (`self.StaticMesh`) 0 _returnvalue))
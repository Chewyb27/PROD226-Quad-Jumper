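; Player plasma projectile, tinted with the player's glow colour, whose upgraded version flies faster, enables bouncing and deals more damage.
; Collider overlap always triggers an explosion, except that Enemy damage and its explosion fire only once, and a BP_Missile gets a delayed Impact call.
; Explode halts movement and reveals the explosion component, which Tick scales up while a timeline animates its dynamic material, then destroys the actor.
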(event `self.Collider.OnComponentBeginOverlap`
  (params (OverlappedComponent :type "PrimitiveComponent Object Reference") (OtherActor :type "Actor Object Reference") (OtherComp :type "PrimitiveComponent Object Reference") (OtherBodyIndex :type Integer) (bFromSweep :type Boolean) (SweepResult :type "HitResult Structure (by ref)"))
  (bind _asenemy (cast `/Game/Blueprints/Enemies/Enemy` OtherActor)
    (:`then`
      (`/Engine/EditorBlueprintResources/StandardMacros.DoOnce` false
        (:`Completed`
          (`/Game/Blueprints/Enemies/Enemy.Take Damage` _asenemy (`KismetMathLibrary.SelectFloat` 65.0 45.0 (`self.Upgraded`)))
          (`self.Explode`))))
    (:`CastFailed`
      (if (== (`GameplayStatics.GetObjectClass` OtherActor) "/Game/Blueprints/Enemies/Weapons/BP_Missile.BP_Missile_C")
        (`self.Explode`)
        (`KismetSystemLibrary.Delay` 1.0)
        (bind _asbp_missile (cast `/Game/Blueprints/Enemies/Weapons/BP_Missile` OtherActor))
        (`/Game/Blueprints/Enemies/Weapons/BP_Missile.Impact` _asbp_missile)
        (else
          (`ActorComponent.SetActive` (`self.FXS_PlayerPlasma`) false false)
          (`self.Explode`))))))

(event `self.ReceiveBeginPlay`
  (bind _upgraded (`self.Upgraded`))
  (bind _projectilemovement (`self.ProjectileMovement`))
  (bind _glowcolour (`/Game/Blueprints/Player/BP_Player.GlowColour` (`self.Player`)))
  (if _upgraded
    _
    (else
      _))
  (set `ProjectileMovementComponent.bShouldBounce` _upgraded _projectilemovement)
  (set `ProjectileMovementComponent.MaxSpeed` (`KismetMathLibrary.SelectFloat` 25000.0 12000.0 _upgraded) _projectilemovement)
  (set `ProjectileMovementComponent.InitialSpeed` (`KismetMathLibrary.SelectFloat` 25000.0 12000.0 _upgraded) _projectilemovement)
  (bind _returnvalue (`PrimitiveComponent.CreateDynamicMaterialInstance` (`self.Explosion`) 0 "/Game/Materials/SpecialEffects/M_PlasmaInstance.M_PlasmaInstance" "None"))
  (bind _output_get (set `self.ExplosionMat` _returnvalue))
  (`MaterialInstanceDynamic.SetVectorParameterValue` _output_get "Colour" _glowcolour)
  (`FXSystemComponent.SetColorParameter` (`self.FXS_PlayerPlasma`) "Color" (* _glowcolour 30.0))
  (`SceneComponent.K2_SetRelativeRotation` (`self.Explosion`) (`KismetMathLibrary.RandomRotator` true) false false))

(event `self.ReceiveTick`
  (params (DeltaSeconds :type "Float (single-precision)"))
  (if (`self.Timeline Started`)
    (`self.Exploding`)))

(event `Exploding`
  (`SceneComponent.SetRelativeScale3D` (`self.Explosion`) (`KismetMathLibrary.ClampVectorSize` (+ (`SceneComponent.RelativeScale3D` (`self.Explosion`)) 0.1) 1.0 2.0)))

(event `Explode`
  (bind _ringparticle (`self.RingParticle`))
  (bind _projectilemovement (`self.ProjectileMovement`))
  (`ActorComponent.SetActive` (`self.FXS_PlayerPlasma`) false false)
  (set `MovementComponent.Velocity` (0.0 0.0 0.0) _projectilemovement)
  (set `ProjectileMovementComponent.ProjectileGravityScale` 0.0 _projectilemovement)
  (`/Engine/EditorBlueprintResources/StandardMacros.IsValid` _ringparticle
    (:`Is Valid`
      (`ActorComponent.K2_DestroyComponent` _ringparticle))
    (:`Is Not Valid`
      _))
  (`SceneComponent.SetVisibility` (`self.Explosion`) true false)
  (bind (_direction _newtrack_0) (`Timeline|Timeline_0`)
    (:`Update`
      (`MaterialInstanceDynamic.SetScalarParameterValue` (`self.ExplosionMat`) "Amount" _newtrack_0)
      (set `self.Timeline Started` true))
    (:`Finished`
      (set `self.Explosion Complete` true)
      (`self.K2_DestroyActor`))))

(fn `UserConstructionScript`)
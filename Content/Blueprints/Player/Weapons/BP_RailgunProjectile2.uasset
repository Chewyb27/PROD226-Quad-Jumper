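; Railgun projectile that deals heavy damage to an enemy it overlaps and shows effects tinted by the player's glow colour.
; Tick feeds its location and right/up axes into a spiral effect.
; On overlap it spawns a hit effect, deactivates the spiral, disables collision and destroys itself after a delay.
; BeginPlay also gives the Explosion component a dynamic plasma material and random rotation.
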(event `self.ReceiveBeginPlay`
  (bind _returnvalue (`PrimitiveComponent.CreateDynamicMaterialInstance` (`self.Explosion`) 0 "/Game/Materials/SpecialEffects/M_PlasmaInstance.M_PlasmaInstance" "None"))
  (set `self.ExplosionMat` _returnvalue)
  (`SceneComponent.K2_SetRelativeRotation` (`self.Explosion`) (`KismetMathLibrary.RandomRotator` true) false false)
  (`NiagaraComponent.SetVariableLinearColor` (`self.FXS_Spiral`) "Color" (* (`/Game/Blueprints/Player/BP_Player.GlowColour` (`self.player`)) (struct :`R` 30.0 :`G` 30.0 :`B` 30.0 :`A` 1.0))))

(event `self.ReceiveTick`
  (params (DeltaSeconds :type "Float (single-precision)"))
  (bind _fxs_spiral (`self.FXS_Spiral`))
  (`NiagaraComponent.SetVariableVec3` _fxs_spiral "Rotation Center" (`self.K2_GetActorLocation`))
  (`NiagaraComponent.SetVariableVec3` _fxs_spiral "B_X Axis" (`self.GetActorRightVector`))
  (`NiagaraComponent.SetVariableVec3` _fxs_spiral "B_Y Axis" (`self.GetActorUpVector`)))

(event `self.Collider.OnComponentBeginOverlap`
  (params (OverlappedComponent :type "PrimitiveComponent Object Reference") (OtherActor :type "Actor Object Reference") (OtherComp :type "PrimitiveComponent Object Reference") (OtherBodyIndex :type Integer) (bFromSweep :type Boolean) (SweepResult :type "HitResult Structure (by ref)"))
  (bind _asenemy (cast `/Game/Blueprints/Enemies/Enemy` OtherActor)
    (:`then`
      (`/Engine/EditorBlueprintResources/StandardMacros.DoOnce` false
        (:`Completed`
          (`/Game/Blueprints/Enemies/Enemy.Take Damage` _asenemy 800.0 false (`self.player`)))))
    (:`CastFailed`
      (`/Engine/EditorBlueprintResources/StandardMacros.DoOnce` false
        (:`Completed`
          _))))
  (bind _returnvalue (`NiagaraFunctionLibrary.SpawnSystemAtLocation` "/Game/Particles/RailgunHit.RailgunHit" (`.Location` (`GameplayStatics.BreakHitResult` SweepResult)) (struct) (3.0 3.0 3.0)))
  (`NiagaraComponent.SetVariableLinearColor` _returnvalue "Color" (* (`/Game/Blueprints/Player/BP_Player.GlowColour` (`self.player`)) (struct :`R` 10.0 :`G` 10.0 :`B` 10.0 :`A` 1.0)))
  (`NiagaraComponent.SetVariableFloat` _returnvalue "Scale" 3.0)
  (`ActorComponent.Deactivate` (`self.FXS_Spiral`))
  (`PrimitiveComponent.SetCollisionEnabled` (`self.Collider`) "NoCollision")
  (`KismetSystemLibrary.Delay` 5.0)
  (`self.K2_DestroyActor`))

(fn `UserConstructionScript`)
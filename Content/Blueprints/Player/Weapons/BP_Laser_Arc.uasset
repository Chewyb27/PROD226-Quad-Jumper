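; Short-lived electric arc actor that links a start actor to an end actor with a Niagara beam and damages the enemy at its end.
; On spawn it attaches to the start actor; for enemy sources it bends the beam upward if grounded, otherwise randomly, using the player's glow colour.
; Tick tracks the end actor and applies damage over time.
; It decrements the player's arc count and destroys itself after half a second or when the target enemy dies.
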(event `self.ReceiveBeginPlay`
  (bind _niagara (`self.Niagara`))
  (bind _start_actor (`self.Start Actor`))
  (bind (_asenemy _bsuccess) (cast `/Game/Blueprints/Enemies/Enemy` _start_actor :!pure true))
  (`SceneComponent.K2_SetWorldLocation` (`self.Niagara`) (`self.Start Location`) false false)
  (`self.K2_AttachToActor` (`self.Start Actor`) "None" "KeepWorld" "KeepWorld" "KeepWorld")
  (`/Engine/EditorBlueprintResources/StandardMacros.IsValid` _start_actor
    (:`Is Valid`
      (`/Engine/EditorBlueprintResources/StandardMacros.IsValid` _niagara
        (:`Is Valid`
          (if _bsuccess
            (`FXSystemComponent.SetVectorParameter` _niagara "Curve Tangent" (`KismetMathLibrary.SelectVector` (`self.GetActorUpVector` _start_actor) (`KismetMathLibrary.RandomUnitVector`) (`/Game/Blueprints/Enemies/Enemy.Grounded` _asenemy)))
            (`FXSystemComponent.SetColorParameter` _niagara "Color" (`/Game/Blueprints/Player/BP_Player.GlowColour` (`self.Player`)))))))))

(event `self.ReceiveTick`
  (params (DeltaSeconds :type "Float (single-precision)"))
  (bind _niagara (`self.Niagara`))
  (bind _end_actor (`self.End Actor`))
  (bind _lifetime (`self.Lifetime`))
  (bind _player (`self.Player`))
  (`/Engine/EditorBlueprintResources/StandardMacros.IsValid` _end_actor
    (:`Is Valid`
      (`/Engine/EditorBlueprintResources/StandardMacros.IsValid` _niagara
        (:`Is Valid`
          (`FXSystemComponent.SetVectorParameter` _niagara "Beam End" (`KismetMathLibrary.SelectVector` (0.0 0.0 0.0) (`self.K2_GetActorLocation` _end_actor))))
        (:`Is Not Valid`
          _))
      (set `self.Lifetime` (+ _lifetime DeltaSeconds)))
    (:`Is Not Valid`
      _))
  (`|ExecutionSequence`
    (:`then_0`
      (if (>= _lifetime 0.5)
        (set `/Game/Blueprints/Player/BP_Player.Arc Ammount` (- (`/Game/Blueprints/Player/BP_Player.Arc Ammount` _player) 1.0) _player :!label _label)
        (`self.K2_DestroyActor`)))
    (:`then_1`
      (bind _asenemy (cast `/Game/Blueprints/Enemies/Enemy` (`self.End Actor`)))
      (`/Engine/EditorBlueprintResources/StandardMacros.IsValid` _asenemy
        (:`Is Valid`
          (if (`/Game/Blueprints/Enemies/Enemy.EnemyAlive` _asenemy)
            (`/Game/Blueprints/Enemies/Enemy.Take Damage` _asenemy (* DeltaSeconds 200.0) false)
            (else
              (goto _label))))
        (:`Is Not Valid`
          (goto _label))))))

(fn `UserConstructionScript`)
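; BP_Grapple is the player's grapple weapon projectile, a hook that latches onto the first actor it overlaps other than its owner.
; On overlap it deactivates its ProjectileMovement and snaps to the hit actor's location once, without attaching or pulling the player.
; Every tick it draws a debug line to the owning BP_Player's MainBody to show the rope.
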(event `self.ReceiveActorBeginOverlap`
  (params (OtherActor :type "Actor Object Reference"))
  (if (!= OtherActor (`self.GetOwner`))
    (`ActorComponent.Deactivate` (`self.ProjectileMovement`))
    (`self.K2_SetActorLocation` (`self.K2_GetActorLocation` OtherActor))))

(event `self.ReceiveTick`
  (params (DeltaSeconds :type "Float (single-precision)"))
  (`KismetSystemLibrary.DrawDebugLine` (`self.K2_GetActorLocation`) (`SceneComponent.K2_GetComponentLocation` (`/Game/Blueprints/Player/BP_Player.Main Body` (cast `/Game/Blueprints/Player/BP_Player` (`self.GetOwner`) :!pure true))) (struct) 0.0 2.0))

(fn `UserConstructionScript`)
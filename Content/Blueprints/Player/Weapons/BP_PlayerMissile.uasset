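; Player homing missile that rides its loaded object until a launch delay elapses, then flies at the target enemy's body.
; Overlaps ignore the player and bounce/plasma projectiles, and detonate on enemies, BP_Missiles or static world.
; Enemy hits deal damage, boosted when upgraded, which also triggers the player's arc laser setup.
; Detonation stops movement, then a timeline fades a dynamic plasma material while Tick grows the explosion, destroying the actor afterwards.
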(event `self.Collider.OnComponentBeginOverlap`
  (params (OverlappedComponent :type "PrimitiveComponent Object Reference") (OtherActor :type "Actor Object Reference") (OtherComp :type "PrimitiveComponent Object Reference") (OtherBodyIndex :type Integer) (bFromSweep :type Boolean) (SweepResult :type "HitResult Structure (by ref)"))
  (bind _returnvalue (`GameplayStatics.GetObjectClass` OtherActor))
  (if (!= _returnvalue "/Game/Blueprints/Player/Weapons/BP_BounceProjectile.BP_BounceProjectile_C")
    (if (== _returnvalue "/Game/Blueprints/Player/Weapons/BP_PlasmaProjectile.BP_PlasmaProjectile_C")
      _
      (elif (== _returnvalue "/Game/Blueprints/Player/BP_Player.BP_Player_C")
        _
        (elif (== _returnvalue "/Game/Blueprints/Enemies/Weapons/BP_Missile.BP_Missile_C")
          (`self.Explode`)
          (`KismetSystemLibrary.Delay` 1.0)
          (`/Engine/EditorBlueprintResources/StandardMacros.IsValid` OtherActor
            (:`Is Not Valid`
              (bind _asbp_missile (cast `/Game/Blueprints/Enemies/Weapons/BP_Missile` OtherActor))
              (`/Game/Blueprints/Enemies/Weapons/BP_Missile.Impact` _asbp_missile)))
          (else
            (bind _asenemy (cast `/Game/Blueprints/Enemies/Enemy` OtherActor)
              (:`then`
                (`/Game/Blueprints/Enemies/Enemy.Take Damage` _asenemy (`KismetMathLibrary.SelectFloat` 1500.0 750.0 (`self.Upgraded`)))
                (`self.Explode`)
                (if (`self.Upgraded`)
                  (`/Game/Blueprints/Player/BP_Player.Setup Arc Laser` (`self.Player`) OtherActor)))
              (:`CastFailed`
                (if (`|EnumEquality` (`PrimitiveComponent.GetCollisionObjectType` OtherComp) "ECC_WorldStatic")
                  (`self.Explode`))))))))))

(event `self.ReceiveBeginPlay`
  (set `ProjectileMovementComponent.HomingTargetComponent` (`/Game/Blueprints/Enemies/Enemy.Enemy Body` (`self.Target`)) (`self.ProjectileMovement`))
  (`ActorComponent.SetActive` (`self.FXS_Spiral`) false false)
  (`ActorComponent.SetActive` (`self.FXS_RailgunTrail`) false false)
  (bind _returnvalue (`PrimitiveComponent.CreateDynamicMaterialInstance` (`self.Explosion`) 0 "/Game/Materials/SpecialEffects/M_PlasmaInstance.M_PlasmaInstance" "None"))
  (set `self.ExplosionMat` _returnvalue)
  (`SceneComponent.K2_SetRelativeRotation` (`self.Explosion`) (`KismetMathLibrary.RandomRotator` true) false false))

(event `Exploding`
  (`SceneComponent.SetRelativeScale3D` (`self.Explosion`) (`KismetMathLibrary.ClampVectorSize` (+ (`SceneComponent.RelativeScale3D` (`self.Explosion`)) (* (stale `self.ReceiveTick` DeltaSeconds) 200.0)) 1.0 100.0))
  (`ActorComponent.SetActive` (`self.FXS_RailgunTrail`) false false)
  (`ActorComponent.SetActive` (`self.FXS_Spiral`) false false))

(event `self.ReceiveTick`
  (params (DeltaSeconds :type "Float (single-precision)"))
  (bind _loaded_object (`self.Loaded Object`))
  (bind _current_delay (`self.Current Delay`))
  (bind _fxs_spiral (`self.FXS_Spiral`))
  (`|ExecutionSequence`
    (:`then_0`
      (if (>= _current_delay (`self.Delay`))
        (`/Engine/EditorBlueprintResources/StandardMacros.DoOnce` false
          (:`Completed`
            (`ActorComponent.SetActive` (`self.FXS_Spiral`) false false)
            (`ActorComponent.SetActive` (`self.FXS_RailgunTrail`) true false)
            (`ActorComponent.SetActive` (`self.ProjectileMovement`) true false)))
        (else
          (set `self.Current Delay` (+ _current_delay DeltaSeconds))
          (`self.K2_SetActorLocation` (`SceneComponent.K2_GetComponentLocation` _loaded_object) false true)
          (`self.K2_SetActorRotation` (`SceneComponent.K2_GetComponentRotation` _loaded_object) true))))
    (:`then_1`
      (`NiagaraComponent.SetVariableVec3` _fxs_spiral "Rotation Center" (`self.K2_GetActorLocation`))
      (`NiagaraComponent.SetVariableVec3` _fxs_spiral "B_X Axis" (`self.GetActorRightVector`))
      (`NiagaraComponent.SetVariableVec3` _fxs_spiral "B_Y Axis" (`self.GetActorUpVector`))
      (if (`self.Timeline Started`)
        (`self.Exploding`)))))

(event `Explode`
  (bind _projectilemovement (`self.ProjectileMovement`))
  (bind _ringparticle (`self.RingParticle`))
  (set `ProjectileMovementComponent.bIsHomingProjectile` false _projectilemovement)
  (set `MovementComponent.Velocity` (0.0 0.0 0.0) _projectilemovement)
  (`ActorComponent.SetActive` (`self.FXS_RailgunTrail`) false false)
  (`ActorComponent.SetActive` (`self.FXS_Spiral`) false false)
  (set `ProjectileMovementComponent.ProjectileGravityScale` 0.0 (`self.ProjectileMovement`))
  (`/Engine/EditorBlueprintResources/StandardMacros.IsValid` _ringparticle
    (:`Is Valid`
      (`ActorComponent.K2_DestroyComponent` _ringparticle))
    (:`Is Not Valid`
      _))
  (`SceneComponent.SetVisibility` (`self.Explosion`) true false)
  (bind (_direction _newtrack_0) (`Timeline|Timeline_0`)
    (:`Update`
      (`MaterialInstanceDynamic.SetScalarParameterValue` (`self.ExplosionMat`) "Amount" _newtrack_0)
      (set `self.Timeline Started` true))
    (:`Finished`
      (set `self.Explosion Complete` true)
      (`self.K2_DestroyActor`))))

(fn `UserConstructionScript`)
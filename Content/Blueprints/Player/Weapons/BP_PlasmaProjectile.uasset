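; Plasma projectile tinted by the player's glow colour, with an Upgraded flag that alters speed, gravity, damage and blast size.
; Tick line-traces ahead to drive Collide, as the component hit and overlap events are empty.
; Collide damages enemies, impacts missiles or pushes physics bodies; most paths add a sphere-traced blast that hurts enemies and knocks back players.
; Explode grows the explosion mesh while a timeline animates its material, then destroys the actor.
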(event `self.Sphere.OnComponentHit`
  (params (HitComponent :type "PrimitiveComponent Object Reference") (OtherActor :type "Actor Object Reference") (OtherComp :type "PrimitiveComponent Object Reference") (NormalImpulse :type "Vector Structure") (Hit :type "HitResult Structure (by ref)")))

(event `self.Collider.OnComponentHit`
  (params (HitComponent :type "PrimitiveComponent Object Reference") (OtherActor :type "Actor Object Reference") (OtherComp :type "PrimitiveComponent Object Reference") (NormalImpulse :type "Vector Structure") (Hit :type "HitResult Structure (by ref)")))

(event `self.Collider.OnComponentBeginOverlap`
  (params (OverlappedComponent :type "PrimitiveComponent Object Reference") (OtherActor :type "Actor Object Reference") (OtherComp :type "PrimitiveComponent Object Reference") (OtherBodyIndex :type Integer) (bFromSweep :type Boolean) (SweepResult :type "HitResult Structure (by ref)")))

(event `Collide`
  (params (Actor :type "Actor Object Reference") (Comp :type "PrimitiveComponent Object Reference") (AOE :type Boolean))
  (bind _returnvalue (`GameplayStatics.GetObjectClass` Actor))
  (bind _returnvalue_2 (`PrimitiveComponent.GetCollisionObjectType` Comp))
  (bind _colliding_enemies (`self.Colliding Enemies`))
  (bind _collider (`self.Collider`))
  (bind _returnvalue_3 (`SceneComponent.K2_GetComponentLocation` (`self.Explosion`)))
  (bind _returnvalue_4 (`|EnumEquality` _returnvalue_2 "ECC_PhysicsBody"))
  (if true
    (if (== _returnvalue "BP_PlasmaProjectile_C")
      _
      (elif (not (or (== _returnvalue "/Game/Blueprints/Player/BP_Player.BP_Player_C") (== _returnvalue "/Game/Blueprints/Player/BP_Player.BP_Player_C")))
        (set `MovementComponent.Velocity` (0.0 0.0 0.0) (`self.ProjectileMovement`))
        (if (== _returnvalue "/Game/Blueprints/Enemies/Weapons/BP_Missile.BP_Missile_C")
          (`self.Explode`)
          (`KismetSystemLibrary.Delay` 1.0)
          (`/Engine/EditorBlueprintResources/StandardMacros.IsValid` Actor
            (:`Is Valid`
              (bind _asbp_missile (cast `/Game/Blueprints/Enemies/Weapons/BP_Missile` Actor))
              (`/Game/Blueprints/Enemies/Weapons/BP_Missile.Impact` _asbp_missile)
              (`self.Explode`)
              (if AOE :!label _label
                (`KismetSystemLibrary.Delay` 0.05)
                (bind _outhits (`KismetSystemLibrary.SphereTraceMulti` _returnvalue_3 _returnvalue_3 (`KismetMathLibrary.SelectFloat` 1500.0 750.0 (`self.Upgraded`)) "TraceTypeQuery1"))
                (`KismetArrayLibrary.Array_Clear` (`self.Colliding Enemies`))
                (for _array_element _outhits
                  (bind (_bblockinghit _binitialoverlap _time _distance _location _impactpoint _normal _impactnormal _physmat _hitactor) (`GameplayStatics.BreakHitResult` _array_element))
                  (if (not (`KismetArrayLibrary.Array_Contains` _colliding_enemies _hitactor))
                    (`KismetArrayLibrary.Array_Add` _colliding_enemies _hitactor)
                    (bind _asenemy (cast `/Game/Blueprints/Enemies/Enemy` _hitactor)
                      (:`then`
                        (`/Game/Blueprints/Enemies/Enemy.Take Damage` _asenemy (`KismetMathLibrary.SelectFloat` 500.0 150.0 (`self.Upgraded`)) false (`self.Player`)))
                      (:`CastFailed`
                        (bind _asbp_player (cast `/Game/Blueprints/Player/BP_Player` _hitactor))
                        (bind _main_box_component (`/Game/Blueprints/Player/BP_Player.Main Box Component` _asbp_player))
                        (`PrimitiveComponent.SetPhysicsLinearVelocity` _main_box_component (* (`KismetMathLibrary.Normal` (- (`SceneComponent.K2_GetComponentLocation` (`self.Explosion`)) (`SceneComponent.K2_GetComponentLocation` (`/Game/Blueprints/Player/BP_Player.Main Body` _asbp_player)))) -7000.0) true "None")
                        (`GameplayStatics.PlayWorldCameraShake` "/Game/Widgets/ExplodeShake.ExplodeShake_C" (`SceneComponent.K2_GetComponentLocation` _main_box_component) 0.0 5000.0))))))))
          (else
            (bind _asenemy_2 (cast `/Game/Blueprints/Enemies/Enemy` Actor)
              (:`then`
                (`KismetArrayLibrary.Array_Add` (`self.Colliding Enemies`) _asenemy_2)
                (`/Engine/EditorBlueprintResources/StandardMacros.DoOnce` false :!label _label_2
                  (:`Completed`
                    (`/Game/Blueprints/Enemies/Enemy.Take Damage` _asenemy_2 (`KismetMathLibrary.SelectFloat` 1000.0 750.0 (`self.Upgraded`)) false (`self.Player`))
                    (`self.Explode`)
                    (goto _label))))
              (:`CastFailed`
                (bind _asbp_missile_2 (cast `/Game/Blueprints/Enemies/Weapons/BP_Missile` Actor)
                  (:`then`
                    (`/Game/Blueprints/Enemies/Weapons/BP_Missile.Impact` _asbp_missile_2)
                    (`self.Explode`))
                  (:`CastFailed`
                    (if (or (`|EnumEquality` _returnvalue_2 "ECC_WorldStatic") (`KismetStringLibrary.Contains` (`KismetSystemLibrary.GetDisplayName` Actor) "landscape") (`|EnumEquality` _returnvalue_2 "ECC_WorldDynamic") _returnvalue_4)
                      (`self.Explode`)
                      (`|ExecutionSequence`
                        (:`then_0`
                          (if _returnvalue_4
                            (`PrimitiveComponent.AddImpulseAtLocation` Comp (* (`SceneComponent.GetForwardVector` _collider) 10000.0) (`SceneComponent.K2_GetComponentLocation` _collider) "None")))
                        (:`then_1`
                          (goto _label))))))))))))))

(event `Refresh`
  (goto _label_2 :!via `Reset`))

(event `self.ReceiveBeginPlay`
  (bind _upgraded (`self.Upgraded`))
  (bind _projectilemovement (`self.ProjectileMovement`))
  (bind _returnvalue (`KismetMathLibrary.SelectFloat` 120000.0 50000.0 _upgraded))
  (bind _glowcolour (`/Game/Blueprints/Player/BP_Player.GlowColour` (`self.Player`)))
  (set `ProjectileMovementComponent.MaxSpeed` _returnvalue _projectilemovement)
  (bind _output_get (set `ProjectileMovementComponent.InitialSpeed` _returnvalue _projectilemovement))
  (set `ProjectileMovementComponent.ProjectileGravityScale` (`KismetMathLibrary.SelectFloat` 0.0 3.0 _upgraded) _projectilemovement)
  (`FXSystemComponent.SetColorParameter` (`self.Niagara`) "Color" _glowcolour)
  (bind _returnvalue_2 (`PrimitiveComponent.CreateDynamicMaterialInstance` (`self.Explosion`) 0 "/Game/Materials/SpecialEffects/M_PlasmaInstance.M_PlasmaInstance" "None"))
  (bind _output_get_2 (set `self.ExplosionMat` _returnvalue_2))
  (`MaterialInstanceDynamic.SetVectorParameterValue` _output_get_2 "Colour" (* _glowcolour 0.5))
  (`SceneComponent.K2_SetRelativeRotation` (`self.Explosion`) (`KismetMathLibrary.RandomRotator` true) false false)
  (`PrimitiveComponent.SetMaterial` (`self.Sphere`) 0 _output_get_2))

(event `self.ReceiveTick`
  (params (DeltaSeconds :type "Float (single-precision)"))
  (bind _collider (`self.Collider`))
  (bind _returnvalue (`SceneComponent.K2_GetComponentLocation` _collider))
  (if (not (`self.Timeline Started`))
    (bind (_outhit _returnvalue_2) (`KismetSystemLibrary.LineTraceSingle` _returnvalue (+ (* (`SceneComponent.GetForwardVector` _collider) 1000.0) _returnvalue) "TraceTypeQuery1"))
    (if _returnvalue_2
      (bind (_bblockinghit _binitialoverlap _time _distance _location _impactpoint _normal _impactnormal _physmat _hitactor _hitcomponent) (`GameplayStatics.BreakHitResult` _outhit))
      (`self.Collide` _hitactor _hitcomponent true)))
  (if false
    _
    (elif (`self.Timeline Started`)
      (`self.Exploding` DeltaSeconds))))

(event `Exploding`
  (params (Delta :type "Float (double-precision)"))
  (bind _upgraded (`self.Upgraded`))
  (`SceneComponent.SetRelativeScale3D` (`self.Explosion`) (`KismetMathLibrary.ClampVectorSize` (+ (`SceneComponent.RelativeScale3D` (`self.Explosion`)) (* Delta (`KismetMathLibrary.SelectFloat` 125.0 75.0 _upgraded))) 1.0 (`KismetMathLibrary.SelectFloat` 50.0 25.0 _upgraded))))

(event `Explode`
  (bind _sphere (`self.Sphere`))
  (`GameplayStatics.PlaySoundAtLocation` "/Game/Sounds/Weapons/Bluezone_BC0294_modern_cinematic_impact_percussion_009.Bluezone_BC0294_modern_cinematic_impact_percussion_009" (`SceneComponent.K2_GetComponentLocation` (`self.Explosion`)) (struct) 0.8 0.5 0.0 null null null null)
  (set `ProjectileMovementComponent.ProjectileGravityScale` 0.0 (`self.ProjectileMovement`))
  (`/Engine/EditorBlueprintResources/StandardMacros.IsValid` null
    (:`Is Valid`
      (`ActorComponent.K2_DestroyComponent` (`self.Niagara`)))
    (:`Is Not Valid`
      _))
  (`/Engine/EditorBlueprintResources/StandardMacros.IsValid` _sphere
    (:`Is Valid`
      (`ActorComponent.K2_DestroyComponent` _sphere))
    (:`Is Not Valid`
      _))
  (`SceneComponent.SetVisibility` (`self.Explosion`) true false)
  (bind (_direction _newtrack_0) (`Timeline|Timeline_0`)
    (:`Update`
      (`MaterialInstanceDynamic.SetScalarParameterValue` (`self.ExplosionMat`) "Amount" _newtrack_0)
      (set `self.Timeline Started` true)
      (`ActorComponent.SetActive` (`self.Niagara`) false false)
      (if (> _newtrack_0 0.7)
        (`/Engine/EditorBlueprintResources/StandardMacros.DoOnce` false)))
    (:`Finished`
      (set `self.Explosion Complete` true)
      (`self.K2_DestroyActor`))))

(fn `UserConstructionScript`)
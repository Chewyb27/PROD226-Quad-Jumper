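; Plasma projectile for the player's repeater weapon, tinted with the player's glow colour.
; Overlaps outside gravity zones trigger an explosion, damaging Enemy actors once or calling Impact on missiles after a delay.
; The Upgraded flag raises speed and damage and enables bouncing, so blocking hits no longer detonate it.
; Explode stops movement and collision, then a timeline animates a dynamic explosion material while Tick grows the mesh, and destroys the actor.
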(event `self.Collider.OnComponentHit`
  (params (HitComponent :type "PrimitiveComponent Object Reference") (OtherActor :type "Actor Object Reference") (OtherComp :type "PrimitiveComponent Object Reference") (NormalImpulse :type "Vector Structure") (Hit :type "HitResult Structure (by ref)"))
  (if (not (`self.Upgraded`))
    (`ActorComponent.SetActive` (`self.FXS_PlayerPlasma`) false false)
    (`self.Explode`)))

(event `self.Collider.OnComponentBeginOverlap`
  (params (OverlappedComponent :type "PrimitiveComponent Object Reference") (OtherActor :type "Actor Object Reference") (OtherComp :type "PrimitiveComponent Object Reference") (OtherBodyIndex :type Integer) (bFromSweep :type Boolean) (SweepResult :type "HitResult Structure (by ref)"))
  (bind _returnvalue (`GameplayStatics.GetObjectClass` OtherActor))
  (if (and (!= _returnvalue "/Game/Blueprints/Scene/G_Zone.G_Zone_C") (!= _returnvalue "/Game/Blueprints/Scene/Zero_G_Zone.Zero_G_Zone_C"))
    (bind _asenemy (cast `/Game/Blueprints/Enemies/Enemy` OtherActor)
      (:`then`
        (`/Engine/EditorBlueprintResources/StandardMacros.DoOnce` false
          (:`Completed`
            (`/Game/Blueprints/Enemies/Enemy.Take Damage` _asenemy (`KismetMathLibrary.SelectFloat` 75.0 55.0 (`self.Upgraded`)) false)
            (`self.Explode`))))
      (:`CastFailed`
        (if (== _returnvalue "/Game/Blueprints/Enemies/Weapons/BP_Missile.BP_Missile_C")
          (`self.Explode`)
          (`KismetSystemLibrary.Delay` 1.0)
          (bind _asbp_missile (cast `/Game/Blueprints/Enemies/Weapons/BP_Missile` OtherActor))
          (`/Game/Blueprints/Enemies/Weapons/BP_Missile.Impact` _asbp_missile)
          (else
            (`ActorComponent.SetActive` (`self.FXS_PlayerPlasma`) false false)
            (`self.Explode`)))))))

(event `self.ReceiveBeginPlay`
  (bind _upgraded (`self.Upgraded`))
  (bind _projectilemovement (`self.ProjectileMovement`))
  (bind _returnvalue (`KismetMathLibrary.SelectFloat` 100000.0 32000.0 _upgraded))
  (bind _glowcolour (`/Game/Blueprints/Player/BP_Player.GlowColour` (`self.Player`)))
  (if _upgraded
    _
    (else
      _))
  (set `ProjectileMovementComponent.bShouldBounce` _upgraded _projectilemovement)
  (set `ProjectileMovementComponent.MaxSpeed` _returnvalue _projectilemovement)
  (set `ProjectileMovementComponent.InitialSpeed` _returnvalue _projectilemovement)
  (bind _returnvalue_2 (`PrimitiveComponent.CreateDynamicMaterialInstance` (`self.Explosion`) 0 "/Game/Materials/SpecialEffects/M_PlasmaInstance.M_PlasmaInstance" "None"))
  (bind _output_get (set `self.ExplosionMat` _returnvalue_2))
  (`MaterialInstanceDynamic.SetVectorParameterValue` _output_get "Colour" _glowcolour)
  (`FXSystemComponent.SetColorParameter` (`self.FXS_PlayerPlasma`) "Color" (* _glowcolour 100.0))
  (`SceneComponent.K2_SetRelativeRotation` (`self.Explosion`) (`KismetMathLibrary.RandomRotator` true) false false))

(event `self.ReceiveTick`
  (params (DeltaSeconds :type "Float (single-precision)"))
  (if (`self.Timeline Started`)
    (`self.Exploding`)))

(event `Exploding`
  (`SceneComponent.SetRelativeScale3D` (`self.Explosion`) (`KismetMathLibrary.ClampVectorSize` (+ (`SceneComponent.RelativeScale3D` (`self.Explosion`)) 0.1) 1.0 2.0)))

(event `Explode`
  (bind _ringparticle (`self.RingParticle`))
  (bind _ringparticle_2 (`self.RingParticle`))
  (bind _fxs_playerplasma (`self.FXS_PlayerPlasma`))
  (bind _projectilemovement (`self.ProjectileMovement`))
  (`PrimitiveComponent.SetCollisionEnabled` (`self.Collider`) "NoCollision")
  (`/Engine/EditorBlueprintResources/StandardMacros.IsValid` _ringparticle
    (:`Is Valid`
      (`ActorComponent.SetActive` _ringparticle false false))
    (:`Is Not Valid`
      _))
  (`ActorComponent.SetActive` _fxs_playerplasma false false)
  (`SceneComponent.SetVisibility` _fxs_playerplasma false false)
  (set `MovementComponent.Velocity` (0.0 0.0 0.0) _projectilemovement)
  (set `ProjectileMovementComponent.ProjectileGravityScale` 0.0 _projectilemovement)
  (`/Engine/EditorBlueprintResources/StandardMacros.IsValid` _ringparticle_2
    (:`Is Valid`
      (`ActorComponent.K2_DestroyComponent` _ringparticle_2))
    (:`Is Not Valid`
      _))
  (`SceneComponent.SetVisibility` (`self.Explosion`) true false)
  (bind (_direction _newtrack_0) (`Timeline|Timeline_0`)
    (:`Update`
      (`MaterialInstanceDynamic.SetScalarParameterValue` (`self.ExplosionMat`) "Amount" _newtrack_0)
      (set `self.Timeline Started` true))
    (:`Finished`
      (set `self.Explosion Complete` true)
      (`self.K2_DestroyActor`))))

(fn `UserConstructionScript`)
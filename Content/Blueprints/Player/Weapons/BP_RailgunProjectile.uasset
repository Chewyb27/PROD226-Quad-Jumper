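; Player railgun projectile that resolves its hit with a line trace on spawn and draws a Niagara beam in the player's glow colour.
; Tick races the actor to the impact point, while trace and overlap hits feed Collide, which damages enemies, triggers missiles and stops on static world.
; Upgraded shots add a spiral effect and start an arc laser from struck enemies.
; Explode grows a timeline-animated material burst, then destroys the actor.
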(event `Collide`
  (params (NewParam :type "Actor Object Reference") (NewParam2 :type "PrimitiveComponent Object Reference") (NewParam3 :type "Vector Structure"))
  (bind _returnvalue (`GameplayStatics.GetObjectClass` NewParam))
  (set `self.Impact` NewParam3)
  (if (!= _returnvalue "/Game/Blueprints/Player/Weapons/BP_BounceProjectile.BP_BounceProjectile_C")
    (if (== _returnvalue "/Game/Blueprints/Player/Weapons/BP_PlasmaProjectile.BP_PlasmaProjectile_C")
      _
      (elif (not (== _returnvalue "/Game/Blueprints/Player/BP_Player.BP_Player_C"))
        (set `MovementComponent.Velocity` (0.0 0.0 0.0) (`self.ProjectileMovement`))
        (if (== _returnvalue "/Game/Blueprints/Enemies/Weapons/BP_Missile.BP_Missile_C")
          (`self.Explode`)
          (`KismetSystemLibrary.Delay` 1.0)
          (`/Engine/EditorBlueprintResources/StandardMacros.IsValid` NewParam
            (:`Is Not Valid`
              (bind _asbp_missile (cast `/Game/Blueprints/Enemies/Weapons/BP_Missile` NewParam))
              (`/Game/Blueprints/Enemies/Weapons/BP_Missile.Impact` _asbp_missile)))
          (else
            (`/Engine/EditorBlueprintResources/StandardMacros.DoOnce` false
              (:`Completed`
                (bind _asenemy (cast `/Game/Blueprints/Enemies/Enemy` NewParam)
                  (:`then`
                    (`/Game/Blueprints/Enemies/Enemy.Take Damage` _asenemy 2000.0 false)
                    (`self.Explode`)
                    (if (`self.Upgraded`)
                      (`/Game/Blueprints/Player/BP_Player.Setup Arc Laser` (`self.Player`) NewParam)))
                  (:`CastFailed`
                    (if (== _returnvalue "/Game/Blueprints/Player/BP_Player.BP_Player_C")
                      _
                      (elif (`|EnumEquality` (`PrimitiveComponent.GetCollisionObjectType` NewParam2) "ECC_WorldStatic")
                        (`self.Explode`)))))))))))))

(event `self.Collider.OnComponentBeginOverlap`
  (params (OverlappedComponent :type "PrimitiveComponent Object Reference") (OtherActor :type "Actor Object Reference") (OtherComp :type "PrimitiveComponent Object Reference") (OtherBodyIndex :type Integer) (bFromSweep :type Boolean) (SweepResult :type "HitResult Structure (by ref)"))
  (`self.Collide` OtherActor OtherComp (`SceneComponent.K2_GetComponentLocation` (`self.Collider`))))

(event `self.ReceiveBeginPlay`
  (bind _returnvalue (`self.K2_GetActorLocation`))
  (bind _glowcolour (`/Game/Blueprints/Player/BP_Player.GlowColour` (`self.Player`)))
  (bind _returnvalue_2 (+ (* (`self.GetActorForwardVector`) 500000.0) _returnvalue))
  (set `self.Impact` _returnvalue)
  (set `self.ringlocation` _returnvalue)
  (`SceneComponent.SetVisibility` (`self.FXS_Spiral`) (`self.Upgraded`) false)
  (bind _returnvalue_3 (`PrimitiveComponent.CreateDynamicMaterialInstance` (`self.Explosion`) 0 "/Game/Materials/SpecialEffects/M_PlasmaInstance.M_PlasmaInstance" "None"))
  (bind _output_get (set `self.ExplosionMat` _returnvalue_3))
  (`MaterialInstanceDynamic.SetVectorParameterValue` _output_get "Colour" (* _glowcolour 0.5))
  (`FXSystemComponent.SetColorParameter` (`self.FXS_Spiral`) "Color" _glowcolour)
  (`SceneComponent.K2_SetRelativeRotation` (`self.Explosion`) (`KismetMathLibrary.RandomRotator` true) false false)
  (bind (_outhit _returnvalue_4) (`KismetSystemLibrary.LineTraceSingle` _returnvalue _returnvalue_2 "TraceTypeQuery1"))
  (bind (_bblockinghit _binitialoverlap _time _distance _location _impactpoint _normal _impactnormal _physmat _hitactor _hitcomponent) (`GameplayStatics.BreakHitResult` _outhit))
  (bind _returnvalue_5 (`NiagaraFunctionLibrary.SpawnSystemAtLocation` "/Game/Particles/FXS_Railgun2.FXS_Railgun2" (`self.ringlocation`) (`self.K2_GetActorRotation`) (`KismetMathLibrary.MakeVector` (`KismetMathLibrary.SelectFloat` (* _distance 0.01) 800.0 (> _distance 0.0)) 0.5 0.5)))
  (`FXSystemComponent.SetColorParameter` _returnvalue_5 "Color" (* (`/Game/Blueprints/Player/BP_Player.GlowColour` (`self.Player`)) (`KismetMathLibrary.SelectColor` (struct :`R` 1.0 :`G` 1.0 :`B` 1.0 :`A` 1.0) (struct :`R` 1.0 :`G` 1.0 :`B` 1.0 :`A` 1.0) (`self.Upgraded`))))
  (set `self.Trail` _returnvalue_5)
  (if _returnvalue_4
    (`self.Collide` _hitactor _hitcomponent _impactpoint)
    (else
      (set `self.Impact` _returnvalue_2))))

(event `self.ReceiveTick`
  (params (DeltaSeconds :type "Float (single-precision)"))
  (bind _returnvalue (`self.K2_GetActorLocation`))
  (bind _fxs_spiral (`self.FXS_Spiral`))
  (set `self.alivetime` (+ (`self.alivetime`) DeltaSeconds))
  (if (not (`self.Explosion Complete`))
    (set `self.ringlocation` _returnvalue)
    (`self.K2_SetActorLocation` (`KismetMathLibrary.VInterpTo_Constant` _returnvalue (`self.Impact`) DeltaSeconds 500000.0))
    (`NiagaraComponent.SetVariableVec3` _fxs_spiral "Rotation Center" _returnvalue)
    (`NiagaraComponent.SetVariableVec3` _fxs_spiral "B_X Axis" (`self.GetActorRightVector`))
    (`NiagaraComponent.SetVariableVec3` _fxs_spiral "B_Y Axis" (`self.GetActorUpVector`))
    (if (`self.Timeline Started`)
      (`self.Exploding` DeltaSeconds))))

(event `Exploding`
  (params (delta :type "Float (double-precision)"))
  (`SceneComponent.SetRelativeScale3D` (`self.Explosion`) (`KismetMathLibrary.ClampVectorSize` (+ (`SceneComponent.RelativeScale3D` (`self.Explosion`)) (* delta 200.0)) 1.0 100.0)))

(event `Explode`
  (bind _ringparticle (`self.RingParticle`))
  (`ActorComponent.SetActive` (`self.FXS_Spiral`) true false)
  (set `ProjectileMovementComponent.ProjectileGravityScale` 0.0 (`self.ProjectileMovement`))
  (`/Engine/EditorBlueprintResources/StandardMacros.IsValid` _ringparticle
    (:`Is Valid`
      (`ActorComponent.K2_DestroyComponent` _ringparticle))
    (:`Is Not Valid`
      _))
  (`SceneComponent.SetVisibility` (`self.Explosion`) true false)
  (`KismetSystemLibrary.Delay` 0.01)
  (bind (_direction _newtrack_0) (`Timeline|Timeline_0`)
    (:`Update`
      (`MaterialInstanceDynamic.SetScalarParameterValue` (`self.ExplosionMat`) "Amount" _newtrack_0)
      (set `self.Timeline Started` true))
    (:`Finished`
      (set `self.Explosion Complete` true)
      (`KismetSystemLibrary.Delay` 1.0)
      (`ActorComponent.K2_DestroyComponent` (`self.Trail`))
      (`ActorComponent.SetActive` (`self.FXS_Spiral`) false false)
      (`self.K2_DestroyActor`))))

(fn `UserConstructionScript`)
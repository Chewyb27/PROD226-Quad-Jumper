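; Friendly laser projectile that damages Enemy actors, with a tinted particle effect.
; On spawn it sets its homing target to the MainBoxComponent of the BP_Player nearest the world origin, despite being friendly fire.
; Sphere overlaps trigger Impact on missiles without ending the blast, while enemies and WorldStatic hits end it.
; Its Impact spawns an explosion, strips its components and destroys the actor after a delay.
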(event `self.ReceiveBeginPlay`
  (`FXSystemComponent.SetColorParameter` (`self.FXS_Enemy_Blast`) "Color" (* (`self.Colour`) 50.0))
  (bind _outactors (`GameplayStatics.GetAllActorsOfClass` "/Game/Blueprints/Player/BP_Player.BP_Player_C"))
  (bind _asbp_player (cast `/Game/Blueprints/Player/BP_Player` (`.ReturnValue` (`GameplayStatics.FindNearestActor` (0.0 0.0 0.0) _outactors))))
  (set `ProjectileMovementComponent.HomingTargetComponent` (`/Game/Blueprints/Player/BP_Player.Main Box Component` _asbp_player) (`self.ProjectileMovement`))
  (`KismetSystemLibrary.Delay` 2.0)
  (set `self.Spawn Expired` true))

(event `self.ReceiveTick`
  (params (DeltaSeconds :type "Float (single-precision)"))
  (set `self.Time since launch` (+ (`self.Time since launch`) DeltaSeconds)))

(event `Impact`
  (`GameplayStatics.SpawnEmitterAtLocation` "/Game/Particles/PS_Explosion.PS_Explosion" (`SceneComponent.K2_GetComponentLocation` (`self.Sphere`)))
  (`ActorComponent.K2_DestroyComponent` (`self.Sphere`))
  (`ActorComponent.K2_DestroyComponent` (`self.FXS_Enemy_Blast`))
  (`ActorComponent.K2_DestroyComponent` (`self.ProjectileMovement`))
  (`KismetSystemLibrary.Delay` 10.0)
  (`self.K2_DestroyActor`))

(event `self.Sphere.OnComponentBeginOverlap`
  (params (OverlappedComponent :type "PrimitiveComponent Object Reference") (OtherActor :type "Actor Object Reference") (OtherComp :type "PrimitiveComponent Object Reference") (OtherBodyIndex :type Integer) (bFromSweep :type Boolean) (SweepResult :type "HitResult Structure (by ref)"))
  (if (>= (`self.Time since launch`) 0.001)
    (if (== (`GameplayStatics.GetObjectClass` OtherActor) "/Game/Blueprints/Enemies/Weapons/BP_Missile.BP_Missile_C")
      (bind _asbp_missile (cast `/Game/Blueprints/Enemies/Weapons/BP_Missile` OtherActor))
      (`/Game/Blueprints/Enemies/Weapons/BP_Missile.Impact` _asbp_missile)
      (else
        (bind _asenemy (cast `/Game/Blueprints/Enemies/Enemy` OtherActor)
          (:`then`
            (`/Game/Blueprints/Enemies/Enemy.Take Damage` _asenemy 3.0)
            (`self.Impact`))
          (:`CastFailed`
            (if (`|EnumEquality` (`PrimitiveComponent.GetCollisionObjectType` OtherComp) "ECC_WorldStatic")
              (`self.Impact`))))))))

(fn `UserConstructionScript`)
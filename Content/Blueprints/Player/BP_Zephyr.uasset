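; BP_Zephyr is a cloaking dropship that delivers players into non-multiplayer levels.
; As level ship, it is possessed by player 0, follows a spline on a timeline, decloaks, spawns and possesses a BP_P08X per saved player near the drop point, recloaks and destroys itself.
; Cloaking drives dynamic hull materials and location-tracked post-process distortion through a FlipFlop that ignores its CloakingEnabled input.
; Other ships toggle cloak periodically on Tick.
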(event `Drop Sequence`
  (bind _spline (`/Game/LevelStart/BP_ShipSpline.Spline` (`self.Track Reference`)))
  (bind _returnvalue (`KismetMathLibrary.Lerp` 0.0 (`SplineComponent.GetSplineLength` _spline) (`self.Alpha`)))
  (bind _returnvalue_2 (`SplineComponent.GetLocationAtDistanceAlongSpline` _spline _returnvalue "World"))
  (`/Engine/EditorBlueprintResources/StandardMacros.DoOnce` false
    (:`Completed`
      (`Controller.Possess` (`GameplayStatics.GetPlayerController` 0) self)
      (`TimelineComponent.SetPlayRate` (`self.ShipMovement`) (/ 1.0 (`self.StartDuration`)))
      (`TimelineComponent.SetNewTime` (`self.ShipMovement`) (`self.StartOffset`))
      (bind (_direction _alpha) (`Timeline|ShipMovement`)
        (:`Update`
          (bind _output_get (set `self.Alpha` _alpha))
          (if (and (not (`self.Decloaked`)) (>= _output_get 0.1))
            (`self.Switch Cloaking` false)
            (set `self.Decloaked` true))
          (`self.K2_SetActorLocationAndRotation` _returnvalue_2 (`SplineComponent.GetRotationAtDistanceAlongSpline` _spline _returnvalue "World"))
          (if (<= (`KismetMathLibrary.Vector_Distance` _returnvalue_2 (`self.Closest Point`)) 1000.0)
            (`/Engine/EditorBlueprintResources/StandardMacros.DoOnce` false
              (:`Completed`
                (for _index (range (`self.Player Num`))
                  (bind _returnvalue_3 (`GameplayStatics.GetPlayerController` _index))
                  (`/Engine/EditorBlueprintResources/StandardMacros.IsValid` _returnvalue_3
                    (:`Is Valid`
                      _)
                    (:`Is Not Valid`
                      (`GameplayStatics.CreatePlayer` -1)))
                  (bind _returnvalue_4 (`|SpawnActorFromClass` "/Game/Blueprints/Player/BP_P-08X.BP_P-08X_C" (`self.GetTransform` (`self.Spawn Location`)) "AdjustIfPossibleButAlwaysSpawn" "OverrideRootScale" null 1.0 (struct) _index self))
                  (`Controller.Possess` _returnvalue_3 _returnvalue_4))
                (`KismetSystemLibrary.Delay` 1.0)
                (`self.Switch Cloaking` true)
                (`KismetSystemLibrary.Delay` 10.0)
                (`self.K2_DestroyActor`)))))))))

(event `self.ReceiveBeginPlay`)

(event `Start Level`
  (bind _main_body (`self.Main Body`))
  (if (not (`self.multiplayer`))
    (bind _returnvalue (`GameplayStatics.LoadGameFromSlot` "Loadout"))
    (bind _asloadout_settings (cast `/Game/Savegames/LoadoutSettings` _returnvalue))
    (bind _output_get (set `self.Player Num` (`/Game/Savegames/LoadoutSettings.playernum` _asloadout_settings)))
    (`|ExecutionSequence`
      (:`then_0`
        (bind _returnvalue_2 (`PrimitiveComponent.CreateDynamicMaterialInstance` _main_body 0 "/Game/Materials/StealthMaterials/StealthShipBody.StealthShipBody" "None"))
        (set `self.Body Material` _returnvalue_2)
        (bind _returnvalue_3 (`PrimitiveComponent.CreateDynamicMaterialInstance` _main_body 1 "/Game/Materials/StealthMaterials/StealthshipEngine.StealthshipEngine" "None"))
        (set `self.Engine Material` _returnvalue_3)
        (bind _returnvalue_4 (`PrimitiveComponent.CreateDynamicMaterialInstance` _main_body 2 "/Game/Materials/StealthMaterials/StealthshipWindowInst.StealthshipWindowInst" "None"))
        (set `self.Window Material` _returnvalue_4)
        (bind _returnvalue_5 (`KismetMaterialLibrary.CreateDynamicMaterialInstance` "/Game/Materials/StealthMaterials/M_Distortion.M_Distortion"))
        (bind _output_get_2 (set `self.Post Process Material` _returnvalue_5))
        (bind _outactors (`GameplayStatics.GetAllActorsOfClass` "/Script/Engine.PostProcessVolume"))
        (for _array_element _outactors
          (`KismetArrayLibrary.Array_Add` (`.Array` (break `WeightedBlendables` (`.WeightedBlendables` (break `PostProcessSettings` (`PostProcessVolume.Settings` _array_element))))) (make `WeightedBlendable` 1.0 _output_get_2)))
        (if (`self.LevelShip`)
          (bind _closestpoint (`self.Closest Point in Spline` (`SceneComponent.K2_GetComponentLocation` (`Actor.RootComponent` (`self.Spawn Location`))) (`/Game/LevelStart/BP_ShipSpline.Spline` (`self.Track Reference`))))
          (set `self.Closest Point` _closestpoint)
          (`self.Drop Sequence`)))
      (:`then_1`
        (`MaterialInstanceDynamic.SetScalarParameterValue` (`self.Body Material`) "Amount" 1.0)
        (`MaterialInstanceDynamic.SetScalarParameterValue` (`self.Engine Material`) "Amount" 1.0)
        (`MaterialInstanceDynamic.SetScalarParameterValue` (`self.Window Material`) "Amount" 1.0)
        (`MaterialInstanceDynamic.SetScalarParameterValue` (`self.Post Process Material`) "Amount" 1.0)))))

(event `Switch Cloaking`
  (params (`Cloaking Enabled` :type Boolean))
  (`/Engine/EditorBlueprintResources/StandardMacros.FlipFlop` :!label _label
    (:`A`
      (bind (_direction _cloaking_amount _distortion) (`Timeline|Timeline_0` :!via `ReverseFromEnd` :!label _label_2)
        (:`Update`
          (`MaterialInstanceDynamic.SetScalarParameterValue` (`self.Body Material`) "Amount" _cloaking_amount)
          (`MaterialInstanceDynamic.SetScalarParameterValue` (`self.Engine Material`) "Amount" _cloaking_amount)
          (`MaterialInstanceDynamic.SetScalarParameterValue` (`self.Window Material`) "Amount" _cloaking_amount)
          (`MaterialInstanceDynamic.SetScalarParameterValue` (`self.Post Process Material`) "Amount" _distortion))))
    (:`B`
      (goto _label_2))))

(event `self.ReceiveTick`
  (params (DeltaSeconds :type "Float (single-precision)"))
  (bind _post_process_material (`self.Post Process Material`))
  (bind _cloak_delay (`self.Cloak Delay`))
  (`/Engine/EditorBlueprintResources/StandardMacros.IsValid` _post_process_material
    (:`Is Valid`
      (`MaterialInstanceDynamic.SetVectorParameterValue` _post_process_material "Location" (`KismetMathLibrary.Conv_VectorToLinearColor` (`self.K2_GetActorLocation`)))
      (if (not (`self.LevelShip`))
        (if (>= _cloak_delay 10.0)
          (set `self.Cloak Delay` 0.0)
          (goto _label)
          (else
            (set `self.Cloak Delay` (+ _cloak_delay DeltaSeconds))))))))

(fn `Closest Point in Spline`
  (params (`Location To Check` :type "Vector Structure") (Spline :type "SplineComponent Object Reference"))
  (returns (ClosestPoint :type "Vector Structure") (`Spline Point` :type Integer))
  (bind _returnvalue (`SplineComponent.FindInputKeyClosestToWorldLocation` Spline `Location To Check`))
  (bind _returnvalue_2 (`KismetMathLibrary.FFloor` _returnvalue))
  (bind _returnvalue_3 (+ _returnvalue_2 1))
  (bind _returnvalue_4 (`SplineComponent.GetDistanceAlongSplineAtSplinePoint` Spline _returnvalue_3))
  (return (`SplineComponent.GetLocationAtDistanceAlongSpline` Spline (- _returnvalue_4 (* (- (`SplineComponent.GetDistanceAlongSplineAtSplinePoint` Spline _returnvalue_2) _returnvalue_4) (- _returnvalue (`KismetMathLibrary.Conv_IntToDouble` _returnvalue_3)))) "World") _returnvalue_2))

(fn `UserConstructionScript`)